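; Moon boss enemy Blueprint that hands off to a cinematic and level change when it dies.
; The OnDeathEvent override runs the parent death logic, then creates and auto-plays the MoonBossSequence level sequence, pausing at its end.
; After a fixed delay, it messages the player pawn to open the gs_moonstruck level by name at its first entrance.
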(event `LoadLevelSequence`
  (bind (_outactor _returnvalue) (`LevelSequencePlayer.CreateLevelSequencePlayer` "/Game/EmPath/Movies/MoonBossSequence.MoonBossSequence" (make `MovieSceneSequencePlaybackSettings` true (struct) (struct :`bAllowRounding` true) 1.0 0.0 false false false false false false "None" true)))
  (`MovieSceneSequencePlayer.Play` _returnvalue)
  (`KismetSystemLibrary.Delay` 45.0)
  (message `/Game/EmPath/Interfaces/BI_GameActions.OpenLevel` (`GameplayStatics.GetPlayerPawn` 0) "gs_moonstruck" "0" false false))

(fn `OnDeathEvent`
  (`parent.OnDeathEvent`)
  (`self.LoadLevelSequence`))

(fn `UserConstructionScript`
  (`parent.UserConstructionScript`))