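; BP_TPoseDecoy is a decoy enemy that damages the player as soon as it spawns and dies to almost any hit.
; On BeginPlay it sets an AI state, drops its health to a token value and sends a damage message to the player pawn.
; Its TakeDamage override subtracts health without calling the parent, then runs a custom death that hides the mesh, spawns a Niagara blood explosion and destroys the actor after a short delay.
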(event `self.ReceiveBeginPlay`
  (`parent.ReceiveBeginPlay`)
  (`self.SetAiState` "NewEnumerator1")
  (set `/Game/EmPath/Blueprints/DamageSystem/BPC_DamageSystem.Health` 1.0 (`self.BPC_DamageSystem`))
  (message `/Game/EmPath/Interfaces/BPI_Damagable.TakeDamage` (`GameplayStatics.GetPlayerPawn` 0) (make `/Game/EmPath/Structures/S_DamageInfo` 8.0) null))

(event `CustomDeathSequence`
  (`SceneComponent.SetVisibility` (`self.Mesh`) false false)
  (`NiagaraFunctionLibrary.SpawnSystemAtLocation` "/Game/MegaMagicVFXBundle/VFX/MagicalExplosionsVFX/VFX/BloodExplosion/Systems/N_BloodExplosion.N_BloodExplosion" (`self.K2_GetActorLocation`) (`self.K2_GetActorRotation`))
  (`KismetSystemLibrary.Delay` 0.6)
  (`self.K2_DestroyActor`))

(fn `PlayDeathSequence`
  (`parent.PlayDeathSequence`))

(fn `TakeDamage`
  (params (DamageInfo :type "/Game/EmPath/Structures/S_DamageInfo Structure") (`Damage Causer` :type "Actor Object Reference"))
  (returns (WasDamaged :type Boolean))
  (bind _bpc_damagesystem (`self.BPC_DamageSystem`))
  (bind _output_get (set `/Game/EmPath/Blueprints/DamageSystem/BPC_DamageSystem.Health` (- (`/Game/EmPath/Blueprints/DamageSystem/BPC_DamageSystem.Health` _bpc_damagesystem) (`.Amount_2_64864A0D4320D27C3EA14D8019B5EC9D` (break `/Game/EmPath/Structures/S_DamageInfo` DamageInfo))) _bpc_damagesystem))
  (if (<= _output_get 0.0)
    (`self.CustomDeathSequence`))
  (return false))

(fn `UserConstructionScript`
  (`parent.UserConstructionScript`))