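; BP_BrainSystem is an enemy that chases the player while its mesh is off-screen and freezes, animation paused, while recently rendered.
; Tick switches between stopping and moving toward the player using that render check.
; While the player overlaps its sphere, it makes their MP regen negative, plays audio, shows a spotlight and heals itself on a looping timer, updating its health bar.
; On death it plays a jump-scare sound and destroys itself.
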(event `self.ReceiveTick`
  (params (DeltaSeconds :type "Float (single-precision)"))
  (bind _returnvalue (`self.GetController`))
  (bind _returnvalue_2 (`GameplayStatics.GetPlayerCharacter` 0))
  (if (`PrimitiveComponent.WasRecentlyRendered` (`self.Mesh`) 0.2)
    (if (`self.IsMoving`)
      (`Controller.StopMovement` (`self.GetController`))
      (set `self.IsMoving` false)
      (set `SkeletalMeshComponent.GlobalAnimRateScale` 0.0 (`self.Mesh`))
      (set `MovementComponent.Velocity` (0.0 0.0 0.0) (`self.CharacterMovement`)))
    (else
      (`/Engine/EditorBlueprintResources/StandardMacros.IsValid` _returnvalue_2
        (:`Is Valid`
          (`/Engine/EditorBlueprintResources/StandardMacros.IsValid` _returnvalue
            (:`Is Valid`
              (`AIBlueprintHelperLibrary.SimpleMoveToLocation` _returnvalue (`self.K2_GetActorLocation` _returnvalue_2))
              (set `self.IsMoving` true)
              (set `SkeletalMeshComponent.GlobalAnimRateScale` 1.0 (`self.Mesh`)))))))))

(event `self.ReceiveBeginPlay`
  (`parent.ReceiveBeginPlay`)
  (`AudioComponent.Stop` (`self.Audio1`))
  (`SkeletalMeshComponent.PlayAnimation` (`self.CharacterMesh1`) "/Game/MonsterForSurvivalGame/Animation/PBR/Beholder/Beholder_Attack02RPT_ANIM.Beholder_Attack02RPT_ANIM" true))

(event `self.Sphere.OnComponentBeginOverlap`
  (params (OverlappedComponent :type "PrimitiveComponent Object Reference") (OtherActor :type "Actor Object Reference") (OtherComp :type "PrimitiveComponent Object Reference") (OtherBodyIndex :type Integer) (bFromSweep :type Boolean) (SweepResult :type "HitResult Structure (by ref)"))
  (bind _returnvalue (`GameplayStatics.GetPlayerPawn` 0))
  (if (== OtherActor _returnvalue)
    (message `/Game/EmPath/Interfaces/BI_GameActions.SetMPRegenRate` _returnvalue -3.0)
    (`AudioComponent.Play` (`self.Audio1`) 0.0)
    (bind _returnvalue_2 (`KismetSystemLibrary.K2_SetTimerDelegate` (delegate `Regen`) 0.3 true))
    (set `self.RegenHandler` _returnvalue_2)
    (`SceneComponent.SetVisibility` (`self.SpotLight`) true false)))

(event `Regen`
  (bind _bpc_damagesystem (`self.BPC_DamageSystem`))
  (`/Game/EmPath/Blueprints/DamageSystem/BPC_DamageSystem.Heal` (`self.BPC_DamageSystem`) 10.0)
  (bind _asw_health_bar (cast `/Game/EmPath/Blueprints/DamageSystem/W_HealthBar` (`WidgetComponent.GetWidget` (`self.Healthbar`))))
  (`/Game/EmPath/Blueprints/DamageSystem/W_HealthBar.SetPercent` _asw_health_bar (`/Game/EmPath/Blueprints/DamageSystem/BPC_DamageSystem.Health` _bpc_damagesystem) (`/Game/EmPath/Blueprints/DamageSystem/BPC_DamageSystem.MaxHealth` _bpc_damagesystem)))

(event `self.Sphere.OnComponentEndOverlap`
  (params (OverlappedComponent :type "PrimitiveComponent Object Reference") (OtherActor :type "Actor Object Reference") (OtherComp :type "PrimitiveComponent Object Reference") (OtherBodyIndex :type Integer))
  (if (== OtherActor (`GameplayStatics.GetPlayerPawn` 0))
    (message `/Game/EmPath/Interfaces/BI_GameActions.SetMPRegenRate` (`GameplayStatics.GetPlayerPawn` 0) 5.0)
    (`AudioComponent.FadeOut` (`self.Audio1`) 0.0 0.0 "Linear")
    (`KismetSystemLibrary.K2_ClearAndInvalidateTimerHandle` (`self.RegenHandler`))
    (`SceneComponent.SetVisibility` (`self.SpotLight`) false false)))

(fn `PlayDeathSequence`
  (`parent.PlayDeathSequence`)
  (`GameplayStatics.PlaySound2D` "/Game/EmPath/Sounds/SC_JumpScare__18_.SC_JumpScare__18_" 0.4 1.0 0.0 null null)
  (`self.K2_DestroyActor`))

(fn `UserConstructionScript`
  (`parent.UserConstructionScript`))