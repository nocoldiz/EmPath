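; Spawner actor that populates the area around itself with a one-time horde of mixed goblin enemies.
; On BeginPlay it waits for a set delay, then loops up to a configurable maximum, spawning each goblin at a random navigable point within a radius.
; A random-index Select picks sword, mage or brawler goblins, repeating the sword class to weight the mix toward it.
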(event `self.ReceiveBeginPlay`
  (`KismetSystemLibrary.Delay` (`self.Duration`))
  (for _ (range (+ (`self.Max`) 1))
    (bind _output_get (set `self.RandomIndex` (`KismetMathLibrary.RandomIntegerInRange` 0 4)))
    (bind _randomlocation (`NavigationSystemV1.K2_GetRandomLocationInNavigableRadius` (`self.K2_GetActorLocation`) (`self.Radius`) null null))
    (`|SpawnActorFromClass` (select `int` _output_get :`0` "/Game/EmPath/Enemies/BP_GoblinSword.BP_GoblinSword_C" :`1` "/Game/EmPath/Enemies/BP_GoblinMage.BP_GoblinMage_C" :`2` "/Game/EmPath/Enemies/BP_GoblinSword.BP_GoblinSword_C" :`3` "/Game/EmPath/Enemies/BP_GoblinBrawler.BP_GoblinBrawler_C" :`4` "/Game/EmPath/Enemies/BP_GoblinSword.BP_GoblinSword_C" :!type "Actor Class Reference") (`KismetMathLibrary.Conv_VectorToTransform` _randomlocation) "Undefined" "MultiplyWithRoot" null null)))

(fn `UserConstructionScript`)