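; Weeping Angel enemy character that chases the player while unseen and freezes when on screen.
; Each Tick uses the mesh's WasRecentlyRendered, with a short tolerance, as the visibility test instead of line traces.
; When rendered, it stops movement, zeroes velocity and pauses animation; otherwise it reissues SimpleMoveToLocation toward player 0 and resumes animation.
; BeginPlay sets an initial AI state, which the Tick logic never reads.
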(event `self.ReceiveTick`
  (params (DeltaSeconds :type "Float (single-precision)"))
  (if (`PrimitiveComponent.WasRecentlyRendered` (`self.Mesh`) 0.2)
    (if (`self.IsMoving`)
      (`Controller.StopMovement` (`self.GetController`))
      (set `self.IsMoving` false)
      (set `SkeletalMeshComponent.GlobalAnimRateScale` 0.0 (`self.Mesh`))
      (set `MovementComponent.Velocity` (0.0 0.0 0.0) (`self.CharacterMovement`)))
    (else
      (`AIBlueprintHelperLibrary.SimpleMoveToLocation` (`self.GetController`) (`self.K2_GetActorLocation` (`GameplayStatics.GetPlayerCharacter` 0)))
      (set `self.IsMoving` true)
      (set `SkeletalMeshComponent.GlobalAnimRateScale` 1.0 (`self.Mesh`)))))

(event `self.ReceiveBeginPlay`
  (`self.SetAiState` "NewEnumerator2"))

(fn `UserConstructionScript`
  (`parent.UserConstructionScript`))