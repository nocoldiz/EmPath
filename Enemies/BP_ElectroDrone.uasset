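; BP_ElectroDrone is an enemy drone Blueprint that adds an explosive death to its parent class.
; Its OnDeathEvent override runs the parent logic, then spawns a charged blackhole explosion effect and a sci-fi explosion sound at the drone's location.
; It then calls the Explode event, which destroys the actor after a short delay.
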(event `Explode`
  (`KismetSystemLibrary.Delay` 1.0)
  (`self.K2_DestroyActor`))

(fn `OnDeathEvent`
  (bind _returnvalue (`self.K2_GetActorLocation`))
  (`parent.OnDeathEvent`)
  (`NiagaraFunctionLibrary.SpawnSystemAtLocation` "/Game/MegaMagicVFXBundle/VFX/MagicalExplosionsVFX/VFX/BlackholeExplosion/Systems/N_BlackholeExplosionCharged.N_BlackholeExplosionCharged" _returnvalue)
  (`GameplayStatics.PlaySoundAtLocation` "/Game/EmPath/Sounds/sci-fi-explosion.sci-fi-explosion" _returnvalue (struct) 1.0 1.0 0.0 null null null null)
  (`self.Explode`))

(fn `UserConstructionScript`
  (`parent.UserConstructionScript`))