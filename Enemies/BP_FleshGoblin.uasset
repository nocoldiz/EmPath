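; Flesh goblin enemy Blueprint that adds a static mesh to the character's head when play begins.
; After the parent BeginPlay, it creates the component at triple scale and attaches it to the "head" socket of Mesh, snapping location and rotation while keeping relative scale.
; The construction script only calls its parent, and the overlap and Tick events are disabled stubs.
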(event `self.ReceiveBeginPlay`
  (`parent.ReceiveBeginPlay`)
  (bind _returnvalue (`AddComponent|NODE_AddStaticMeshComponent-0` :`RelativeTransform` (`KismetMathLibrary.MakeTransform` (0.0 0.0 0.0) (struct) (3.0 3.0 3.0))))
  (`SceneComponent.K2_AttachToComponent` _returnvalue (`self.Mesh`) "head" "SnapToTarget" "SnapToTarget" "KeepRelative" true))

(fn `UserConstructionScript`
  (`parent.UserConstructionScript`))