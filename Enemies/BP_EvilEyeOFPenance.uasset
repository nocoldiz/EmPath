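; BP_EvilEyeOFPenance is an enemy pawn that pursues other pawns it sees, excluding the player.
; Its PawnSensing component triggers an AI move toward any sighted non-player pawn.
; When its mesh overlaps an actor other than itself or the player, it destroys itself and spawns a fresh copy at a random reachable nav point close to its location.
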(event `self.Mesh.OnComponentBeginOverlap`
  (params (OverlappedComponent :type "PrimitiveComponent Object Reference") (OtherActor :type "Actor Object Reference") (OtherComp :type "PrimitiveComponent Object Reference") (OtherBodyIndex :type Integer) (bFromSweep :type Boolean) (SweepResult :type "HitResult Structure (by ref)"))
  (if (and (!= OtherActor (`GameplayStatics.GetPlayerPawn` 0)) (!= OtherActor self))
    (`self.K2_DestroyActor`)
    (`|SpawnActorFromClass` "BP_EvilEyeOFPenance_C" (`KismetMathLibrary.Conv_VectorToTransform` (`NavigationSystemV1.K2_GetRandomReachablePointInRadius` (`self.K2_GetActorLocation`) 100.0 null null)) "Undefined" "MultiplyWithRoot" null null)))

(event `CustomEvent`)

(event `self.PawnSensing.OnSeePawn`
  (params (Pawn :type "Pawn Object Reference"))
  (if (!= Pawn (`GameplayStatics.GetPlayerPawn` 0))
    (`|AIMoveTo` self (`self.K2_GetActorLocation` Pawn) Pawn)))

(fn `UserConstructionScript`)