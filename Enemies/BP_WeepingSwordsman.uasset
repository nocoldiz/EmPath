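; BP_WeepingSwordsman is an enemy that moves toward the player only while unseen, freezing in place when rendered on screen.
; Tick checks the mesh's WasRecentlyRendered to either halt movement and animation rate, or resume both with SimpleMoveToLocation toward the player.
; BeginPlay sets an AI state, and the death sequence extends the parent's with a 2D scream sound before destroying the actor.
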(event `self.ReceiveTick`
  (params (DeltaSeconds :type "Float (single-precision)"))
  (bind _returnvalue (`self.GetController`))
  (bind _returnvalue_2 (`GameplayStatics.GetPlayerCharacter` 0))
  (if (`PrimitiveComponent.WasRecentlyRendered` (`self.Mesh`) 0.2)
    (if (`self.IsMoving`)
      (`Controller.StopMovement` (`self.GetController`))
      (set `self.IsMoving` false)
      (set `SkeletalMeshComponent.GlobalAnimRateScale` 0.0 (`self.Mesh`))
      (set `MovementComponent.Velocity` (0.0 0.0 0.0) (`self.CharacterMovement`)))
    (else
      (`/Engine/EditorBlueprintResources/StandardMacros.IsValid` _returnvalue_2
        (:`Is Valid`
          (`/Engine/EditorBlueprintResources/StandardMacros.IsValid` _returnvalue
            (:`Is Valid`
              (`AIBlueprintHelperLibrary.SimpleMoveToLocation` _returnvalue (`self.K2_GetActorLocation` _returnvalue_2))
              (set `self.IsMoving` true)
              (set `SkeletalMeshComponent.GlobalAnimRateScale` 1.0 (`self.Mesh`)))))))))

(event `self.ReceiveBeginPlay`
  (`self.SetAiState` "NewEnumerator2"))

(fn `PlayDeathSequence`
  (`parent.PlayDeathSequence`)
  (`GameplayStatics.PlaySound2D` "/Game/EmPath/Sounds/0_ElevenLabs/goblin_screaming_bur_3_.goblin_screaming_bur_3_" 1.0 1.0 0.0 null null)
  (`self.K2_DestroyActor`))

(fn `UserConstructionScript`
  (`parent.UserConstructionScript`))