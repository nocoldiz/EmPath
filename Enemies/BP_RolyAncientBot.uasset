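; BP_RolyAncientBot is an enemy Blueprint for the Roly Ancient Bot, currently a stub with no behavior of its own in its graphs.
; It declares spell functions for compressing, creating, randomizing and retrieving spells, but all are empty, with GetStoredSpell returning only a false IsDominant flag.
; The event graph holds only disabled default nodes, and the construction script just calls its parent.
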(fn `CompressSpell`
  (params (DominantSpell :type "/Game/EmPath/Enum/E_SpellNames Enum" :default "NewEnumerator0") (SecondarySpell :type "/Game/EmPath/Enum/E_SpellNames Enum" :default "NewEnumerator0"))
  (returns (Spell :type "/Game/EmPath/Structures/Spell/S_Spell Structure"))
  (return))

(fn `CreateRandomSpell`
  (params (ChaosFactor :type Integer))
  (returns (Spell :type "/Game/EmPath/Structures/Spell/S_Spell Structure"))
  (return))

(fn `CreateSpell`
  (params (SpellName :type "/Game/EmPath/Enum/E_SpellNames Enum" :default "NewEnumerator0"))
  (returns (Spell :type "/Game/EmPath/Structures/Spell/S_Spell Structure"))
  (return))

(fn `GetStoredSpell`
  (returns (SpellInfo :type "/Game/EmPath/Structures/Spell/S_Spell Structure") (IsDominant :type Boolean))
  (return (struct) false))

(fn `UserConstructionScript`
  (`parent.UserConstructionScript`))