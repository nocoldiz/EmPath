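; Allied phantom goblin enemy variant that, after a short delay from spawning, sends itself a large hit of damage.
; Its TakeDamage override only returns false, applying no damage itself, including for that self-hit.
; While alive, seeing a pawn records its position, optionally alerts others, equips any weapon, then follows, or attacks after a delay if ranged and near.
; A retriggerable delay leads to investigation once sightings pause.
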(event `self.ReceiveBeginPlay`
  (`parent.ReceiveBeginPlay`)
  (`KismetSystemLibrary.Delay` 3.0)
  (`self.TakeDamage` (make `/Game/EmPath/Structures/S_DamageInfo` 1000.0) self))

(event `self.PawnSensing.OnSeePawn`
  (params (Pawn :type "Pawn Object Reference"))
  (if (not (`/Game/EmPath/Blueprints/DamageSystem/BPC_DamageSystem.IsDead` (`self.BPC_DamageSystem`)))
    (set `self.LastKnownPosition` (`self.K2_GetActorLocation` Pawn))
    (if (`self.WeepingAngel`)
      (if (`self.AlertOtherEnemies`)
        (`self.AlertEnemies`)))
    (`|ExecutionSequence`
      (:`then_0`
        (if (`self.HasWeapon`)
          (`self.EquipWeapon`))
        (if (`self.Ranged`)
          (bind _playernear (`self.Is Target Near` 1000.0))
          (if _playernear
            (`KismetSystemLibrary.RetriggerableDelay` 6.0)
            (`self.AttackTarget` false)
            (else
              (`/Game/EmPath/Interfaces/BPI_EnemyAI.FollowActor`)))
          (else
            (`/Game/EmPath/Interfaces/BPI_EnemyAI.FollowActor`))))
      (:`then_1`
        (`KismetSystemLibrary.RetriggerableDelay` 1.0)
        (`self.Investigate`)))))

(fn `TakeDamage`
  (params (DamageInfo :type "/Game/EmPath/Structures/S_DamageInfo Structure") (`Damage Causer` :type "Actor Object Reference") (HitLocation :type "Vector Structure"))
  (returns (WasDamaged :type Boolean))
  (return false))

(fn `UserConstructionScript`
  (`parent.UserConstructionScript`))