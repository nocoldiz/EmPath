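; BP_AlienChaser is an enemy that damages the player on contact and then relocates itself.
; When its Sphere overlaps the player pawn, it plays a low-pitched stab sound and applies one point of damage.
; It then teleports to a random navigable point within a randomly sized radius around itself.
; The graph contains no chase or movement logic, and BeginPlay and Tick are disabled.
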(event `self.Sphere.OnComponentBeginOverlap`
  (params (OverlappedComponent :type "PrimitiveComponent Object Reference") (OtherActor :type "Actor Object Reference") (OtherComp :type "PrimitiveComponent Object Reference") (OtherBodyIndex :type Integer) (bFromSweep :type Boolean) (SweepResult :type "HitResult Structure (by ref)"))
  (if (== OtherActor (`GameplayStatics.GetPlayerPawn` 0))
    (`GameplayStatics.PlaySoundAtLocation` "/Game/EmPath/SoundCues/SC_Stab.SC_Stab" (`self.K2_GetActorLocation`) (struct) 1.0 0.4 0.0 null null null null)
    (`GameplayStatics.ApplyDamage` (`GameplayStatics.GetPlayerPawn` 0) 1.0 null self)
    (bind _randomlocation (`NavigationSystemV1.K2_GetRandomLocationInNavigableRadius` (`self.K2_GetActorLocation`) (`KismetMathLibrary.RandomFloatInRange` 2000.0 10000.0) null null))
    (`self.K2_TeleportTo` _randomlocation)))

(fn `UserConstructionScript`
  (`parent.UserConstructionScript`))