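; BP_TravelMap is an interactable travel map that opens the world map UI when used.
; Use runs the HM interaction check, then creates W_WorldMap, adds it to the viewport and switches to Game-and-UI input with a visible cursor.
; It also sets its Widget component to world space; the logic restoring game-only input and screen space is unconnected.
; The construction script runs the shared HM default setup for horror events.
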(event `self.ReceiveTick`
  (params (DeltaSeconds :type "Float (single-precision)")))

(event `self.Use`
  (params (HorrorEvent :type Boolean))
  ;[1 1 1] Interact Settings
  (`/Game/HorrorEngine/Blueprints/Core/HorrorEngineMacros.HM_CheckInteraction`)
  (bind _returnvalue (`|CreateWidget` "/Game/EmPath/UI/W_WorldMap.W_WorldMap_C" (`GameplayStatics.GetPlayerController` 0)))
  (`UserWidget.AddToViewport` _returnvalue 0)
  (`WidgetBlueprintLibrary.SetInputMode_GameAndUIEx` (`GameplayStatics.GetPlayerController` 0) _returnvalue "DoNotLock" false)
  (`WidgetComponent.SetWidgetSpace` (`self.Widget`) "World")
  (set `PlayerController.bShowMouseCursor` true (`GameplayStatics.GetPlayerController` 0)))

(fn `UserConstructionScript`
  (`/Game/HorrorEngine/Blueprints/Core/HorrorEngineMacros.HM_DefaultConstructions` (`self.CreateNewHorrorEvent`)))