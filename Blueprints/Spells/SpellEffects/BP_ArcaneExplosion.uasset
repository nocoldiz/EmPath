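; Spell effect actor for Arcane Explosion that spawns a dark-magic meteor portal and launches a projectile from its Arrow component.
; BeginPlay plays an energy-burn sound, spawns the Niagara portal, then after a short delay spawns a scaled-down ProjectileBP.
; After a further wait it destroys itself.
; If RepeaterTracker is set, NextArrow first re-enters the portal-and-projectile sequence, with destruction following one second later.
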(event `self.ReceiveBeginPlay`
  (bind (_returnvalue_location _returnvalue_rotation) (`KismetMathLibrary.BreakTransform` (`SceneComponent.K2_GetComponentToWorld` (`self.Arrow`))))
  (`GameplayStatics.PlaySoundAtLocation` "/Game/UltimateMagicUE/wav/Spell_Loops/Loop_-__Blue_Energy_Burn.Loop_-__Blue_Energy_Burn" (`self.K2_GetActorLocation`) (struct) 1.0 1.0 0.0 null null null null)
  (`NiagaraFunctionLibrary.SpawnSystemAtLocation` "/Game/DarkMagicFX/Niagara/Meteor/NS_Portal_Meteor_DarkMagic.NS_Portal_Meteor_DarkMagic" _returnvalue_location _returnvalue_rotation :!label _label)
  (`KismetSystemLibrary.Delay` 1.0)
  (`|SpawnActorFromClass` (`self.ProjectileBP`) (`KismetMathLibrary.MakeTransform` _returnvalue_location _returnvalue_rotation (0.1 0.1 0.1)) "Undefined" "SelectDefaultAtRuntime" null null)
  (`KismetSystemLibrary.Delay` (`KismetMathLibrary.RandomFloatInRange` 3.0 3.0))
  (if (`self.RepeaterTracker`)
    (`self.NextArrow`)
    (`KismetSystemLibrary.Delay` 1.0)
    (`self.K2_DestroyActor`)
    (else
      (`self.K2_DestroyActor`))))

(event `NextArrow`
  (goto _label))

(fn `UserConstructionScript`)