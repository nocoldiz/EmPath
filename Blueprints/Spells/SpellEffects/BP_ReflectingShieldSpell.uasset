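; BP_ReflectingShieldSpell is a spell effect actor, by its name a reflecting shield, with a short fixed lifetime.
; On BeginPlay it waits briefly, starts an audio fade-out and destroys itself immediately, without waiting for the fade to finish.
; Its graphs hold no reflection logic, and the spell create, compress and query functions are empty stubs returning at most a default value.
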(event `self.ReceiveBeginPlay`
  (`KismetSystemLibrary.Delay` 3.0)
  (`AudioComponent.FadeOut` (`self.Audio`) 3.0 0.0 "Linear")
  (`self.K2_DestroyActor`))

(fn `CompressSpell`
  (params (DominantSpell :type "/Game/EmPath/Enum/E_SpellNames Enum" :default "NewEnumerator0") (SecondarySpell :type "/Game/EmPath/Enum/E_SpellNames Enum" :default "NewEnumerator0"))
  (returns (Spell :type "/Game/EmPath/Structures/Spell/S_Spell Structure"))
  (return))

(fn `CreateRandomSpell`
  (params (ChaosFactor :type Integer))
  (returns (Spell :type "/Game/EmPath/Structures/Spell/S_Spell Structure"))
  (return))

(fn `CreateSpell`
  (params (SpellName :type "/Game/EmPath/Enum/E_SpellNames Enum" :default "NewEnumerator0"))
  (returns (Spell :type "/Game/EmPath/Structures/Spell/S_Spell Structure"))
  (return))

(fn `GetStoredSpell`
  (returns (SpellInfo :type "/Game/EmPath/Structures/Spell/S_Spell Structure") (IsDominant :type Boolean))
  (return (struct) false))

(fn `UserConstructionScript`)