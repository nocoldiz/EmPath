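; BP_SpawnCamper is a spell effect that brings the small camper to the effect's location, facing the player pawn's rotation.
; On BeginPlay, outside the level TheRoad, it teleports the first existing BP_CamperSmall there and calls StartDriving on it.
; If no camper exists, it destroys the first BP_Bubba found, then spawns an actor at that transform, adjusting for collision but always spawning.
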(event `self.ReceiveBeginPlay`
  (bind _returnvalue (`self.K2_GetActorRotation` (`GameplayStatics.GetPlayerPawn` 0)))
  (bind _returnvalue_2 (`GameplayStatics.GetCurrentLevelName` true))
  (if (not (`KismetStringLibrary.EqualEqual_StrStr` _returnvalue_2 "TheRoad"))
    (bind _outactors (`GameplayStatics.GetAllActorsOfClass` "/Game/EmPath/Blueprints/Camper/BP_CamperSmall.BP_CamperSmall_C"))
    (bind _output (`|GetArrayItem` _outactors))
    (`/Engine/EditorBlueprintResources/StandardMacros.IsValid` _output
      (:`Is Valid`
        (`self.K2_TeleportTo` _output (`self.K2_GetActorLocation`) _returnvalue)
        (`/Game/EmPath/Interfaces/BI_Drivable.StartDriving` _output))
      (:`Is Not Valid`
        (bind _outactors_2 (`GameplayStatics.GetAllActorsOfClass` "/Game/EmPath/Blueprints/NPC/BP_Bubba.BP_Bubba_C"))
        (bind _output_2 (`|GetArrayItem` _outactors_2))
        (`/Engine/EditorBlueprintResources/StandardMacros.IsValid` _output_2
          (:`Is Valid`
            (`self.K2_DestroyActor` _output_2))
          (:`Is Not Valid`
            _))
        (`|SpawnActorFromClass` "/Game/EmPath/Blueprints/Camper/BP_CamperSmall.BP_CamperSmall_C" (`KismetMathLibrary.MakeTransform` (.location (`self.GetTransform`)) _returnvalue) "AdjustIfPossibleButAlwaysSpawn" "MultiplyWithRoot" null false null)))))

(fn `UserConstructionScript`)