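; Spell effect actor that temporarily summons a random NPC to its own location.
; Shortly after BeginPlay, it picks a random BP_NPC, stores that NPC's location and teleports it to the effect.
; After a timed delay, it spawns a rune Niagara effect and teleport sound, returns the NPC to the saved location, then destroys the effect component.
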(event `self.ReceiveBeginPlay`
  (bind _returnvalue (`self.K2_GetActorLocation`))
  (`KismetSystemLibrary.Delay` 1.2)
  (bind _outactors (`GameplayStatics.GetAllActorsOfClass` "/Game/EmPath/Blueprints/NPC/BP_NPC.BP_NPC_C"))
  (bind _output_get (set `self.Actor` (`KismetArrayLibrary.Array_Random` _outactors)))
  (`/Engine/EditorBlueprintResources/StandardMacros.IsValid` _output_get
    (:`Is Valid`
      (set `self.LastLocation` (`self.K2_GetActorLocation` (`self.Actor`)))
      (`self.K2_TeleportTo` :`self` (`self.Actor`) :`DestLocation` _returnvalue)
      (`KismetSystemLibrary.Delay` 20.0)
      (bind _returnvalue_2 (`NiagaraFunctionLibrary.SpawnSystemAtLocation` "/Game/NiagaraEffectMix5/Effects/NS_Rune_And_RIngs.NS_Rune_And_RIngs" (+ _returnvalue (0.0 0.0 20.0))))
      (`GameplayStatics.PlaySoundAtLocation` "/Game/EmPath/Sounds/teleport-90137.teleport-90137" (0.0 0.0 0.0) (struct) 1.0 1.0 0.0 "/Game/YI_TankCollection/Sounds/Master/SA_Standard.SA_Standard" null null null)
      (`self.K2_TeleportTo` :`self` (`self.Actor`) :`DestLocation` (`self.LastLocation`))
      (`KismetSystemLibrary.Delay` 1.0)
      (`ActorComponent.K2_DestroyComponent` _returnvalue_2))))

(fn `UserConstructionScript`)