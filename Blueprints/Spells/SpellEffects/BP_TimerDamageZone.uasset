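; Spell effect zone that periodically damages overlapping BPI_Damagable actors and can apply a status effect.
; Sphere or box overlaps, chosen by UseBoxCollider, feed AffectedActors; box end overlap adds instead of removing.
; A looping timer runs Damage over that list through interface messages.
; BeginPlay either randomizes yaw or optionally snaps to ground, damages immediately and self-destructs after MaxDuration; random rotation skips those latter steps.
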(event `self.ReceiveBeginPlay`
  (bind _returnvalue (`self.K2_GetActorLocation`))
  (bind _maxduration (`self.MaxDuration`))
  (`KismetSystemLibrary.K2_SetTimer` null "Damage" (`self.DamageTick`) true)
  (if (`self.RandomRotation`)
    (`self.K2_SetActorRotation` (`KismetMathLibrary.MakeRotator` 0.0 0.0 (`KismetMathLibrary.RandomFloatInRange` 0.0 360.0)))
    (else
      (if (`self.TeleportOnGround`)
        (bind (_outhit _returnvalue_2) (`KismetSystemLibrary.LineTraceSingle` _returnvalue (- _returnvalue (0.0 0.0 10000.0)) "TraceTypeQuery1"))
        (if _returnvalue_2
          (`self.K2_SetActorLocation` (`.Location` (`GameplayStatics.BreakHitResult` _outhit)))))
      (`self.Damage`)
      (if (> _maxduration 0.0)
        (`KismetSystemLibrary.Delay` _maxduration)
        (`self.K2_DestroyActor`)))))

(event `self.Sphere.OnComponentBeginOverlap`
  (params (OverlappedComponent :type "PrimitiveComponent Object Reference") (OtherActor :type "Actor Object Reference") (OtherComp :type "PrimitiveComponent Object Reference") (OtherBodyIndex :type Integer) (bFromSweep :type Boolean) (SweepResult :type "HitResult Structure (by ref)"))
  (if (not (`self.UseBoxCollider`))
    (`self.AddDamage` OtherActor OtherActor)))

(event `self.Sphere.OnComponentEndOverlap`
  (params (OverlappedComponent :type "PrimitiveComponent Object Reference") (OtherActor :type "Actor Object Reference") (OtherComp :type "PrimitiveComponent Object Reference") (OtherBodyIndex :type Integer))
  (if (not (`self.UseBoxCollider`))
    (`self.RemoveDamage` OtherActor OtherActor)))

(event `self.Box.OnComponentBeginOverlap`
  (params (OverlappedComponent :type "PrimitiveComponent Object Reference") (OtherActor :type "Actor Object Reference") (OtherComp :type "PrimitiveComponent Object Reference") (OtherBodyIndex :type Integer) (bFromSweep :type Boolean) (SweepResult :type "HitResult Structure (by ref)"))
  (if (`self.UseBoxCollider`)
    (`self.AddDamage` OtherActor OtherActor)))

(event `self.Box.OnComponentEndOverlap`
  (params (OverlappedComponent :type "PrimitiveComponent Object Reference") (OtherActor :type "Actor Object Reference") (OtherComp :type "PrimitiveComponent Object Reference") (OtherBodyIndex :type Integer))
  (if (`self.UseBoxCollider`)
    (`self.AddDamage` OtherActor OtherActor)))

(fn `AddDamage`
  (params (NewItem :type "Actor Object Reference (by ref)") (TestObject :type "Object Object Reference"))
  (if (`KismetSystemLibrary.DoesImplementInterface` TestObject "/Game/EmPath/Interfaces/BPI_Damagable.BPI_Damagable_C")
    (`KismetArrayLibrary.Array_AddUnique` (`self.AffectedActors`) NewItem)))

(fn `Damage`
  (bind _status (`self.Status`))
  (for _array_element (`self.AffectedActors`)
    (`/Engine/EditorBlueprintResources/StandardMacros.IsValid` _array_element
      (:`Is Valid`
        (message `/Game/EmPath/Interfaces/BPI_Damagable.TakeDamage` _array_element (make `/Game/EmPath/Structures/S_DamageInfo` (`self.Damage Info Amount`) "NewEnumerator4" (`self.Damage Info Damage Response`)) null (`self.K2_GetActorLocation`))
        (if (not (`|EnumEquality` _status "NewEnumerator12"))
          (message `/Game/EmPath/Interfaces/BPI_Damagable.ApplyStatus` _array_element _status (`self.StatusDuration`) (`self.StatusMagnitude`) false (`self.StatusSuccessRate`) "None"))))))

(fn `RemoveDamage`
  (params (Item :type "Actor Object Reference (by ref)") (TestObject :type "Object Object Reference"))
  (if (`KismetSystemLibrary.DoesImplementInterface` TestObject "/Game/EmPath/Interfaces/BPI_Damagable.BPI_Damagable_C")
    (`KismetArrayLibrary.Array_RemoveItem` (`self.AffectedActors`) Item)))

(fn `UserConstructionScript`)