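; BP_PartySpawner is a short-lived actor that gathers team 0 characters at its location by teleporting existing actors rather than spawning new ones.
; On BeginPlay it zeroes its root rotation, then filters all BP_EnemyBase actors by team number.
; An incrementing index assigns matches to four scene component markers, with overflow sharing the last.
; Each teleported character has its AI state set, and the spawner destroys itself after a brief delay.
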(event `self.ReceiveBeginPlay`
  (`SceneComponent.K2_SetWorldRotation` :`self` (`self.DefaultSceneRoot`))
  (`KismetSystemLibrary.PrintString` "Spaw ")
  (bind _outactors (`GameplayStatics.GetAllActorsOfClass` "/Game/EmPath/Enemies/BP_EnemyBase.BP_EnemyBase_C"))
  (for _array_element _outactors
    (bind _teamnumber (`/Game/EmPath/Interfaces/BPI_Damagable.GetTeamNumber` _array_element))
    (if (== _teamnumber 0)
      (bind _result (`/Engine/EditorBlueprintResources/StandardMacros.IncrementInt` (`self.TeamIndex`))
        (:`  `
          (switch `int` _result
            (:`Default`
              (`self.K2_TeleportTo` :`self` _array_element :`DestLocation` (`SceneComponent.K2_GetComponentLocation` (`self.Scene3`)) :!label _label))
            (:`0`
              (`self.K2_TeleportTo` :`self` _array_element :`DestLocation` (`SceneComponent.K2_GetComponentLocation` (`self.Scene`))))
            (:`1`
              (`self.K2_TeleportTo` :`self` _array_element :`DestLocation` (`SceneComponent.K2_GetComponentLocation` (`self.Scene1`))))
            (:`2`
              (`self.K2_TeleportTo` :`self` _array_element :`DestLocation` (`SceneComponent.K2_GetComponentLocation` (`self.Scene2`))))
            (:`3`
              (goto _label)))
          (`/Game/EmPath/Enemies/BP_EnemyBase.SetAiState` _array_element "NewEnumerator0")))))
  (`KismetSystemLibrary.Delay` 1.0)
  (`self.K2_DestroyActor`))

(fn `UserConstructionScript`)