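; BP_ElementalReaction is a spell actor representing an elemental reaction, with a text label, a Niagara effect and a hitbox.
; Its construction script labels it with the reaction enum name and applies the particle and hitbox scale from GetElementalReactionData.
; GetCombination maps two schools to a reaction, but both lookups are stubs covering only Electrify Water, with no particle assigned.
; The event graph holds no active logic.
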(fn `GetCombination`
  (params (SchoolA :type "/Game/EmPath/Enum/E_MagicSchools Enum" :default "NewEnumerator0") (SchoolB :type "/Game/EmPath/Enum/E_MagicSchools Enum" :default "NewEnumerator0"))
  (returns (NewParam :type "/Game/EmPath/Enum/E_ElementalReactions Enum"))
  (switch `/Game/EmPath/Enum/E_MagicSchools` SchoolA
    (:`NewEnumerator0`
      (return "NewEnumerator0"))))

(fn `GetElementalReactionData`
  (params (NewParam :type "/Game/EmPath/Enum/E_ElementalReactions Enum" :default "NewEnumerator0"))
  (returns (Particle :type "NiagaraSystem Object Reference") (Scale :type "Vector Structure"))
  (switch `/Game/EmPath/Enum/E_ElementalReactions` NewParam
    (:`NewEnumerator0`
      (return null (1.0 1.0 1.0)))))

(fn `UserConstructionScript`
  (bind _elementalreaction (`self.ElementalReaction`))
  (bind (_particle _scale) (`self.GetElementalReactionData` _elementalreaction))
  ;[1 1 1] Text Render
  (`TextRenderComponent.K2_SetText` (`self.TextRender`) (`KismetTextLibrary.Conv_StringToText` (`|GetEnumeratorNameAsString` _elementalreaction)))
  (bind _returnvalue (`PrimitiveComponent.CreateDynamicMaterialInstance` (`self.TextRender`) 0 "/Game/EmPath/Materials/M_TextMaterial.M_TextMaterial" "None"))
  (`MaterialInstanceDynamic.SetScalarParameterValue` _returnvalue "Opacity" -80.0)
  (`NiagaraComponent.SetAsset` (`self.Niagara`) _particle true)
  (`SceneComponent.SetRelativeScale3D` (`self.Hitbox`) _scale))