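; BP_EnemySpell is an enemy spell projectile driven by its Spell data, which sets movement, effects, sounds, damage and lifetime.
; BeginPlay branches on spell type into a line trace, brief homing on the player, plain flight or an empty self-target stub.
; Collisions damage the player or damageable actors; hit and destroy events spawn BP_SpellHit, optional objects and, on hit, type-specific AOE.
; The Play*Sequence functions are empty hooks.
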(event `self.ReceiveBeginPlay`
  (bind _particle (`self.Particle`))
  (bind (_castsound _travelanimation _travelsound _hitanimation _hitsound _damage _spawnobject _speed _spelltype _despawnafterhit _bouncetype _bouncetimes) (break `/Game/EmPath/Structures/S_EnemySpell` (`self.Spell`)))
  (bind (_castsound_2 _travelanimation_2 _travelsound_2 _hitanimation_2 _hitsound_2 _damage_2 _spawnobject_2 _speed_2 _spelltype_2) (break `/Game/EmPath/Structures/S_EnemySpell` (`self.Spell`)))
  (bind _returnvalue (`|EnumEquality` _spelltype "NewEnumerator1"))
  ;[1 1 1] Initialize particle FX
  (if (`|EnumEquality` _spelltype_2 "NewEnumerator5")
    (`self.TargetSelfPlayer`)
    (else
      (`/Engine/EditorBlueprintResources/StandardMacros.IsValid` _travelanimation_2
        (:`Is Valid`
          (`NiagaraComponent.SetAsset` _particle _travelanimation_2 false))
        (:`Is Not Valid`
          _))
      ;[0 1 0.3242] Spell Flowchart
      ;;[1 1 1 1 28] Set rotation
      (`SceneComponent.SetWorldScale3D` _particle (1.0 1.0 1.0))
      (`SceneComponent.K2_SetRelativeRotation` (`self.ImpactRadius`) (`KismetMathLibrary.Conv_VectorToRotator` (`self.GetActorForwardVector` (`self.GetOwner`))) false false)
      (if (`|EnumEquality` _spelltype_2 "NewEnumerator2")
        (bind (_outhit _returnvalue_2) (`KismetSystemLibrary.LineTraceSingle` :`Start` (`self.K2_GetActorLocation`) :`End` (`self.GetActorForwardVector`) :`TraceChannel` "TraceTypeQuery1" :`DrawDebugType` "Persistent"))
        (if _returnvalue_2
          (bind _output_get (set `self.Hit` _outhit))
          (if (`KismetSystemLibrary.DoesImplementInterface` (`.HitComponent` (`GameplayStatics.BreakHitResult` _output_get)) "/Game/EmPath/Interfaces/BPI_Damagable.BPI_Damagable_C")
            (`self.TriggerSpellHit` "NewEnumerator1")
            (else
              (`self.TriggerSpellHit` "NewEnumerator3"))))
        (else
          (if _returnvalue
            (`self.Set Homing Projectile` false))
          (set `self.BounceTimes` _bouncetimes)
          ;;[1 1 1] Async load particle
          (`/Engine/EditorBlueprintResources/StandardMacros.IsValid` _travelsound
            (:`Is Valid`
              (bind _returnvalue_3 (`GameplayStatics.SpawnSoundAttached` _travelsound (`self.Particle`) "None" (0.0 0.0 0.0) (struct) "KeepRelativeOffset" true (`self.Volume Multiplier`) (`self.Pitch Multiplier`) 0.0 "/Game/HorrorEngine/Audio/_ATT_Profiles/ATT_Teleport.ATT_Teleport" null))
              (bind _output_get_2 (set `self.TravelSound` _returnvalue_3))
              (if _returnvalue
                (`KismetSystemLibrary.Delay` 0.4)
                (set `ProjectileMovementComponent.bIsHomingProjectile` false (`self.ProjectileMovement`))))
            (:`Is Not Valid`
              _))
          (`self.PlayTravelSequence`)
          (`KismetSystemLibrary.Delay` (`.MaxDuration_50_38CB0B964F25558489D3ED9870D2E37B` (break `/Game/EmPath/Structures/S_EnemySpell` (`self.Spell`))))
          (`/Engine/EditorBlueprintResources/StandardMacros.IsValid` _output_get_2
            (:`Is Valid`
              ;;[1 1 1] Destroy sequence
              (`AudioComponent.FadeOut` _output_get_2 1.0 0.0 "Linear"))
            (:`Is Not Valid`
              _))
          (`self.Destroy`))))))

(event `StopMovement`
  (bind _travelsound (`self.TravelSound`))
  ;[0 1 0.3242] Spell Flowchart
  ;;[1 1 1] Stop movement
  (`/Engine/EditorBlueprintResources/StandardMacros.IsValid` _travelsound
    (:`Is Valid`
      (`AudioComponent.FadeOut` _travelsound 0.6 0.0 "Linear"))
    (:`Is Not Valid`
      _))
  (`MovementComponent.StopMovementImmediately` (`self.ProjectileMovement`))
  (if (`.DespawnAfterHit_51_22338A7B4955C0ADDB1F4FB1A0C00A6F` (break `/Game/EmPath/Structures/S_EnemySpell` (`self.Spell`)))
    (`self.Destroy`)))

(event `Destroy`
  (bind _returnvalue (`self.K2_GetActorLocation`))
  (bind (_castsound _travelanimation _travelsound _hitanimation _hitsound _damage _spawnobject) (break `/Game/EmPath/Structures/S_EnemySpell` (`self.Spell`)))
  ;[0 1 0.3242] Spell Flowchart
  ;;[1 1 1] Destroy
  (`self.PlayDestroySequence`)
  (`/Engine/EditorBlueprintResources/StandardMacros.DoOnce` false
    (:`Completed`
      (`|SpawnActorFromClass` "/Game/EmPath/Blueprints/Spells/BP_SpellHit.BP_SpellHit_C" (`KismetMathLibrary.MakeTransform` (`.Location` (`GameplayStatics.BreakHitResult` (`self.Hit`)))) "Undefined" "MultiplyWithRoot" null _hitanimation _hitsound 1.0 (`self.SpellCharge`) null)
      (if (`KismetSystemLibrary.IsValidSoftClassReference` _spawnobject)
        (bind _outhit (`KismetSystemLibrary.LineTraceSingle` _returnvalue (* _returnvalue (0.0 0.0 -1000.0)) "TraceTypeQuery1" true))
        (bind _returnvalue_location (`KismetMathLibrary.BreakTransform` (`KismetMathLibrary.Conv_VectorToTransform` (`.Location` (`GameplayStatics.BreakHitResult` _outhit)))))
        ;;[1 1 1] SpawnActorOnHit
        (`|SpawnActorFromClass` (`|ConvertAsset` _spawnobject) (`KismetMathLibrary.MakeTransform` _returnvalue_location (`KismetMathLibrary.Conv_VectorToRotator` (`self.GetActorForwardVector` (`GameplayStatics.GetPlayerCameraManager` 0)))) "AdjustIfPossibleButAlwaysSpawn" "MultiplyWithRoot" null null))
      (if true
        _
        (else
          _))
      (`self.K2_DestroyActor`))))

(event `TriggerSpellHit`
  (params (Type :type "/Game/EmPath/Enum/E_SpellImpactTarget Enum" :default "NewEnumerator0"))
  (bind _bouncetimes (`self.BounceTimes`))
  (bind (_castsound _travelanimation _travelsound _hitanimation _hitsound _damage _spawnobject _speed _spelltype) (break `/Game/EmPath/Structures/S_EnemySpell` (`self.Spell`)))
  (bind (_castsound_2 _travelanimation_2 _travelsound_2 _hitanimation_2 _hitsound_2 _damage_2 _spawnobject_2) (break `/Game/EmPath/Structures/S_EnemySpell` (`self.Spell`)))
  ;[0.9815 0.1329 1] Spell Hit sequence
  ;;[1 1 1] Spell hit events
  (`self.PlayHitSequence`)
  (`|SpawnActorFromClass` "/Game/EmPath/Blueprints/Spells/BP_SpellHit.BP_SpellHit_C" (`KismetMathLibrary.MakeTransform` (`.Location` (`GameplayStatics.BreakHitResult` (`self.Hit`)))) "Undefined" "MultiplyWithRoot" null _hitanimation _hitsound 1.0 (`self.SpellCharge`) null)
  (`|ExecutionSequence`
    (:`then_0`
      (if (`|EnumEquality` (`.BounceType_47_524D10FA4C9267DFD142D68E17BE0481` (break `/Game/EmPath/Structures/S_EnemySpell` (`self.Spell`))) "NewEnumerator0")
        ;;[1 1 1] Decrease Max Bounce
        (`/Engine/EditorBlueprintResources/StandardMacros.DecrementInt` _bouncetimes
          (:`  `
            (if (== _bouncetimes 0)
              (`self.StopMovement`))))
        (else
          (`self.StopMovement`))))
    (:`then_1`
      ;;[1 1 1] SpawnActorOnHit
      (`|LoadAssetClass` _spawnobject_2
        (:`then`
          (`|SpawnActorFromClass` (`|ConvertAsset` _spawnobject_2) (`KismetMathLibrary.Conv_VectorToTransform` (`.ImpactPoint` (`GameplayStatics.BreakHitResult` (`self.Hit`)))) "AdjustIfPossibleButAlwaysSpawn" "MultiplyWithRoot" null null))))
    (:`then_2`
      (if (`|EnumEquality` _spelltype "NewEnumerator3")
        (`self.AOEDamage` 200.0 (make `/Game/EmPath/Structures/S_DamageInfo` _damage_2 "NewEnumerator3" "NewEnumerator4" false false false false true))))
    (:`then_4`
      (switch `/Game/EmPath/Enum/E_SpellImpactTarget` Type))))

(event `self.ImpactRadius.OnComponentBeginOverlap`
  (params (OverlappedComponent :type "PrimitiveComponent Object Reference") (OtherActor :type "Actor Object Reference") (OtherComp :type "PrimitiveComponent Object Reference") (OtherBodyIndex :type Integer) (bFromSweep :type Boolean) (SweepResult :type "HitResult Structure (by ref)"))
  ;[1 0.5177 0.03873 1 24] Spell impact
)

(event `TargetSelfPlayer`
  ;[1 0.5177 0.03873 1 24] Spell impact
  ;;[1 1 1] Impact with player
)

(event `self.ImpactRadius.OnComponentHit`
  (params (HitComponent :type "PrimitiveComponent Object Reference") (OtherActor :type "Actor Object Reference") (OtherComp :type "PrimitiveComponent Object Reference") (NormalImpulse :type "Vector Structure") (Hit :type "HitResult Structure (by ref)"))
  (bind _travelsound (`self.TravelSound`))
  ;[1 0.5177 0.03873 1 24] Spell impact
  (`/Engine/EditorBlueprintResources/StandardMacros.IsValid` _travelsound
    (:`Is Valid`
      (`AudioComponent.FadeOut` _travelsound 1.0 0.0 "Linear"))
    (:`Is Not Valid`
      _))
  (set `self.Hit` Hit)
  ;;[1 1 1] Check if hit another spell
  (if (not (`KismetMathLibrary.ClassIsChildOf` (`GameplayStatics.GetObjectClass` OtherActor) "/Game/EmPath/Blueprints/Spells/BP_BaseSpell.BP_BaseSpell_C"))
    ;;[1 1 1] Impact with player
    (if (`self.ActorHasTag` OtherActor "Player")
      (bind _iscolliding (message `/Game/EmPath/Interfaces/BI_GameActions.GetSpellCollision` (`GameplayStatics.GetPlayerPawn` 0)))
      (if (not _iscolliding)
        (message `/Game/EmPath/Interfaces/BPI_Damagable.TakeDamage` (`GameplayStatics.GetPlayerPawn` 0) (make `/Game/EmPath/Structures/S_DamageInfo` (`.Damage_14_EA09ED90438671D85D0772832F4A02AC` (break `/Game/EmPath/Structures/S_EnemySpell` (`self.Spell`))) "NewEnumerator1") null)
        (if (`.DespawnAfterHit_51_22338A7B4955C0ADDB1F4FB1A0C00A6F` (break `/Game/EmPath/Structures/S_EnemySpell` (`self.Spell`)))
          (`self.K2_DestroyActor`)))
      (else
        ;;[1 1 1] Take Damage
        (if (`KismetSystemLibrary.DoesImplementInterface` OtherActor "/Game/EmPath/Interfaces/BPI_Damagable.BPI_Damagable_C")
          (message `/Game/EmPath/Interfaces/BPI_Damagable.TakeDamage` OtherActor (make `/Game/EmPath/Structures/S_DamageInfo` (`.Damage_14_EA09ED90438671D85D0772832F4A02AC` (break `/Game/EmPath/Structures/S_EnemySpell` (`self.Spell`))) "NewEnumerator1") null)
          (`self.TriggerSpellHit` "NewEnumerator1")
          (else
            ;;[1 1 1] Set Spell compressor
            (if (`KismetSystemLibrary.DoesImplementInterface` OtherActor "/Game/EmPath/Interfaces/BI_Spellcrafting.BI_Spellcrafting_C")
              (set `ProjectileMovementComponent.ProjectileGravityScale` -10.0 (`self.ProjectileMovement`))
              (else
                ;;[1 1 1] Object
                (if (`KismetSystemLibrary.DoesImplementInterface` OtherActor "/Game/EmPath/Interfaces/BI_Object.BI_Object_C")
                  _)))))))))

(event `AOEDamage`
  (params (Radius :type "Float (single-precision)") (DamageInfo :type "/Game/EmPath/Structures/S_DamageInfo Structure"))
  ;[1 1 1] AOE Damage
  (bind _returnvalue (`|SpawnActorFromClass` "/Game/EmPath/Enemies/LegacySystem/AOE/BP_SpellAOE.BP_SpellAOE_C" (`KismetMathLibrary.MakeTransform` (`self.K2_GetActorLocation`)) "Undefined" "MultiplyWithRoot" null true false false (`GameplayStatics.GetPlayerPawn` 0)))
  (set `/Game/EmPath/Enemies/LegacySystem/AOE/BP_SpellAOE.Radius` Radius _returnvalue)
  (set `/Game/EmPath/Enemies/LegacySystem/AOE/BP_SpellAOE.DamageInfo` DamageInfo _returnvalue)
  (set `/Game/EmPath/Enemies/LegacySystem/AOE/BP_SpellAOE.Delay` 2.0 _returnvalue)
  (`/Game/EmPath/Enemies/LegacySystem/AOE/BP_SpellAOE.SpawnAOESphere` _returnvalue))

(event `self.ProjectileMovement.OnProjectileBounce`
  (params (ImpactResult :type "HitResult Structure (by ref)") (ImpactVelocity :type "Vector Structure (by ref)"))
  ;[1 0.5177 0.03873 1 24] Spell impact
)

(event `AOEDamageActor`
  (params (Actor :type "Actor Object Reference"))
  ;[1 1 1] AOE Damage
  (message `/Game/EmPath/Interfaces/BPI_Damagable.TakeDamage` Actor (stale `AOEDamage` DamageInfo) (`self.GetOwner`)))

(fn `PlayCastSequence`)

(fn `PlayDestroySequence`)

(fn `PlayHitSequence`)

(fn `PlaySpawnSequence`)

(fn `PlayTravelSequence`)

(fn `Set Homing Projectile`
  (params (TargetEnemy :type Boolean))
  (bind _projectilemovement (`self.ProjectileMovement`))
  ;[1 1 1] SetHomingProjectile
  (if TargetEnemy
    (bind _asmaster (`/Game/HorrorEngine/Blueprints/Core/HorrorEngineFunctions.GetPlayer`))
    (bind _lasttarget (`/Game/HorrorEngine/Blueprints/HorrorEngine.LastTarget` _asmaster))
    (`/Engine/EditorBlueprintResources/StandardMacros.IsValid` (`|ConvertAsset` _lasttarget)
      (:`Is Valid`
        (bind _output (`|ConvertAsset` _lasttarget))
        (if (`KismetSystemLibrary.DoesImplementInterface` _output "/Game/EmPath/Interfaces/BPI_Damagable.BPI_Damagable_C")
          (bind _health (message `/Game/EmPath/Interfaces/BPI_Damagable.GetCurrentHealth` _output))
          (if (> _health 0.0)
            (bind _returnvalue (`AddComponent|NODE_AddSceneComponent-3`))
            (set `self.Homing Target Component` _returnvalue)
            (set `ProjectileMovementComponent.HomingTargetComponent` (`self.Homing Target Component`) _projectilemovement :!label _label)
            (set `ProjectileMovementComponent.bIsHomingProjectile` true _projectilemovement)
            (set `ProjectileMovementComponent.HomingAccelerationMagnitude` 15000.0 _projectilemovement)))))
    (else
      (bind _asem_path_player (cast `/Game/EmPath/Blueprints/EmPathPlayer` (`GameplayStatics.GetPlayerCharacter` 0)))
      (bind _returnvalue_2 (`AddComponent|NODE_AddSceneComponent-1` :`self` _asem_path_player))
      (set `self.Homing Target Component` _returnvalue_2)
      (goto _label))))

(fn `SetProjectileMovement`
  (bind _projectilemovement (`self.ProjectileMovement`))
  (bind _projectilemovement_2 (`self.ProjectileMovement`))
  (bind (_castsound _travelanimation _travelsound _hitanimation _hitsound _damage _spawnobject _speed _spelltype _despawnafterhit _bouncetype _bouncetimes _gravityscale) (break `/Game/EmPath/Structures/S_EnemySpell` (`self.Spell`)))
  ;[1 1 1] Set projectile movement
  (set `ProjectileMovementComponent.InitialSpeed` _speed _projectilemovement)
  (set `ProjectileMovementComponent.MaxSpeed` _speed _projectilemovement)
  (set `ProjectileMovementComponent.ProjectileGravityScale` _gravityscale _projectilemovement)
  (switch `/Game/EmPath/Enum/E_BounceType` _bouncetype
    (:`NewEnumerator0`
      (set `ProjectileMovementComponent.Bounciness` 0.0 _projectilemovement_2))
    (:`NewEnumerator1`
      (set `ProjectileMovementComponent.Bounciness` 1.0 _projectilemovement_2))
    (:`NewEnumerator2`
      (set `ProjectileMovementComponent.Bounciness` -6.0 _projectilemovement_2))
    (:`NewEnumerator3`
      (set `ProjectileMovementComponent.Bounciness` 0.5 _projectilemovement_2))))

(fn `UserConstructionScript`
  ;[1 1 1] Get Magic school
  (`self.SetProjectileMovement`))