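; Fog boundary controller that thickens fog as the player strays from CenterLocation and teleports them back to this actor's location beyond MaxFogDistance.
; Each Tick, UpdateFogDensity lerps the referenced fog actor's density by player distance past StartFogDistance, clamped between min and max.
; A teleport sets ExitFog, which schedules ExitFromFog on a delayed timer to set density once from CurrentAlpha.
; The construction script destroys the actor without a valid FogActorRef.
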(event `self.ReceiveTick`
  (params (DeltaSeconds :type "Float (single-precision)"))
  (`self.UpdateFogDensity`))

(fn `ExitFromFog`
  (bind _minfogdensity (`self.MinFogDensity`))
  (bind _fogactorref (`self.FogActorRef`))
  (if (`KismetSystemLibrary.IsValid` _fogactorref)
    (`ExponentialHeightFogComponent.SetFogDensity` (`ExponentialHeightFog.Component` _fogactorref) (`KismetMathLibrary.FClamp` (`KismetMathLibrary.Lerp` _minfogdensity (`self.MaxFogDensity`) (`self.CurrentAlpha`)) _minfogdensity))))

(fn `UpdateFogDensity`
  (bind _returnvalue (`GameplayStatics.GetPlayerCharacter` 0))
  (bind _returnvalue_2 (`KismetMathLibrary.Vector_Distance` (`self.CenterLocation`) (`self.K2_GetActorLocation` _returnvalue)))
  (if (`KismetSystemLibrary.IsValid` _returnvalue)
    (if (`self.ExitFog`)
      (`KismetSystemLibrary.K2_SetTimer` null "ExitFromFog" 4.0)
      (set `self.ExitFog` false)
      (elif (>= _returnvalue_2 (`self.StartFogDistance`))
        (if (`KismetSystemLibrary.IsValid` (`self.FogActorRef`))
          (`ExponentialHeightFogComponent.SetFogDensity` (`ExponentialHeightFog.Component` (`self.FogActorRef`)) (`KismetMathLibrary.FClamp` (`KismetMathLibrary.Lerp` (`self.MinFogDensity`) (`self.MaxFogDensity`) (/ (- _returnvalue_2 (`self.StartFogDistance`)) (* (- (`self.MaxFogDistance`) (`self.StartFogDistance`)) 3.0))) (`self.MinFogDensity`) (`self.MaxFogDensity`))))
        (if (> _returnvalue_2 (`self.MaxFogDistance`))
          (`KismetSystemLibrary.PrintString` "Teleport")
          (`self.K2_TeleportTo` :`self` (`GameplayStatics.GetPlayerCharacter` 0) :`DestLocation` (`self.K2_GetActorLocation` self))
          (set `self.ExitFog` true))))))

(fn `UserConstructionScript`
  (if (not (`KismetSystemLibrary.IsValid` (`self.FogActorRef`)))
    (`self.K2_DestroyActor`)))