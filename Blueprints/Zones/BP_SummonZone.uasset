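; BP_SummonZone is a one-shot trigger zone that summons an actor when the player walks into it.
; Its sphere's begin-overlap checks for player pawn 0, then spawns a configurable class at the Arrow component's location.
; A particle system and sound play at the same spot, and the zone then destroys itself.
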(event `self.Sphere.OnComponentBeginOverlap`
  (params (OverlappedComponent :type "PrimitiveComponent Object Reference") (OtherActor :type "Actor Object Reference") (OtherComp :type "PrimitiveComponent Object Reference") (OtherBodyIndex :type Integer) (bFromSweep :type Boolean) (SweepResult :type "HitResult Structure (by ref)"))
  (bind _returnvalue (`SceneComponent.K2_GetComponentLocation` (`self.Arrow`)))
  (if (== OtherActor (`GameplayStatics.GetPlayerPawn` 0))
    (`|SpawnActorFromClass` (`self.Class`) (`KismetMathLibrary.Conv_VectorToTransform` _returnvalue) "Undefined" "MultiplyWithRoot" null null)
    (`NiagaraFunctionLibrary.SpawnSystemAtLocation` (`self.System Template`) _returnvalue)
    (`GameplayStatics.PlaySoundAtLocation` (`self.Sound`) _returnvalue (struct) 1.0 1.0 0.0 null null null null)
    (`self.K2_DestroyActor`)))

(fn `UserConstructionScript`)