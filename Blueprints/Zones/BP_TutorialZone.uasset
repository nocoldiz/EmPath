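; BP_TutorialZone is a trigger volume that shows tutorial text to the player while they stand inside it.
; When the player pawn enters or leaves the box, it finds the first CharacterStatusWidget via GetAllWidgetsOfClass and sets its tutorial text to InText or clears it.
; A static mesh rotates every tick by the Rotation variable.
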(event `self.Box.OnComponentBeginOverlap`
  (params (OverlappedComponent :type "PrimitiveComponent Object Reference") (OtherActor :type "Actor Object Reference") (OtherComp :type "PrimitiveComponent Object Reference") (OtherBodyIndex :type Integer) (bFromSweep :type Boolean) (SweepResult :type "HitResult Structure (by ref)"))
  (if (== OtherActor (`GameplayStatics.GetPlayerPawn` 0))
    (bind _foundwidgets (`WidgetBlueprintLibrary.GetAllWidgetsOfClass` "/Game/MRPGT/UserInterface/WidgetBlueprints/CharacterStatusWidget.CharacterStatusWidget_C" false))
    (`/Game/MRPGT/UserInterface/WidgetBlueprints/CharacterStatusWidget.SetTutorialText` (`|GetArrayItem` _foundwidgets) (`self.In Text`))))

(event `self.Box.OnComponentEndOverlap`
  (params (OverlappedComponent :type "PrimitiveComponent Object Reference") (OtherActor :type "Actor Object Reference") (OtherComp :type "PrimitiveComponent Object Reference") (OtherBodyIndex :type Integer))
  (if (== OtherActor (`GameplayStatics.GetPlayerPawn` 0))
    (bind _foundwidgets (`WidgetBlueprintLibrary.GetAllWidgetsOfClass` "/Game/MRPGT/UserInterface/WidgetBlueprints/CharacterStatusWidget.CharacterStatusWidget_C" false))
    (`/Game/MRPGT/UserInterface/WidgetBlueprints/CharacterStatusWidget.SetTutorialText` (`|GetArrayItem` _foundwidgets) "")))

(event `self.ReceiveTick`
  (params (DeltaSeconds :type "Float (single-precision)"))
  (`SceneComponent.K2_AddLocalRotation` (`self.StaticMesh`) (`self.Rotation`) false false))

(fn `UserConstructionScript`)