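; BP_SoundTriggerZone is a box trigger volume that plays a configured sound when the player pawn enters it.
; The sound plays either as 2D UI audio or at the SoundOrigin location with configurable volume, pitch, start time and attenuation.
; A Triggered flag blocks retriggering until the player exits and a cooldown delay elapses, while non-repeatable zones destroy themselves after the first play.
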(event `self.Box.OnComponentBeginOverlap`
  (params (OverlappedComponent :type "PrimitiveComponent Object Reference") (OtherActor :type "Actor Object Reference") (OtherComp :type "PrimitiveComponent Object Reference") (OtherBodyIndex :type Integer) (bFromSweep :type Boolean) (SweepResult :type "HitResult Structure (by ref)"))
  (bind _sound (`self.Sound`))
  (if (== OtherActor (`GameplayStatics.GetPlayerPawn` 0))
    (if (not (`self.Triggered`))
      (set `self.Triggered` true)
      (if (`self.UiSound`)
        (`GameplayStatics.PlaySound2D` _sound 1.0 1.0 0.0 null null)
        (else
          (`GameplayStatics.PlaySoundAtLocation` _sound (`SceneComponent.K2_GetComponentLocation` (`self.SoundOrigin`)) (struct) (`self.Volume Multiplier`) (`self.Pitch Multiplier`) (`self.Start Time`) (`self.Attenuation Settings`) null null null)))
      (if (not (`self.Repeatable`))
        (`self.K2_DestroyActor`)))))

(event `self.Box.OnComponentEndOverlap`
  (params (OverlappedComponent :type "PrimitiveComponent Object Reference") (OtherActor :type "Actor Object Reference") (OtherComp :type "PrimitiveComponent Object Reference") (OtherBodyIndex :type Integer))
  (if (== OtherActor (`GameplayStatics.GetPlayerPawn` 0))
    (`KismetSystemLibrary.Delay` (`self.CoolDown`))
    (set `self.Triggered` false)))

(fn `UserConstructionScript`)