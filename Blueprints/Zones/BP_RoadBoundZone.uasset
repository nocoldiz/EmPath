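; Road boundary zone that returns the player to the map through a save and reload.
; On BeginPlay it caches the game instance and small camper, then starts a looping timer that passes the player's, then the camper's location to IsInLevelBounds.
; A true result shows the loading widget, then after a short delay saves a new game with level, transform and coordinates and auto-loads it.
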(event Custom|ReturnToMap
  (bind _gameinstance (Variables|Default|GetGameInstance))
  (bind _levelname (Variables|Default|GetLevelName))
  (bind _mapcoordinates (Default|GetCoordinates (Variables|Default|GetGameInstance)))
  (bind _returnvalue (UserInterface|CreateWidget "/Game/EmPath/UI/W_Loading.W_Loading_C"))
  (UserInterface|Viewport|AddtoViewport _returnvalue 0)
  (Utilities|FlowControl|Delay 0.4)
  (Default|SaveNewGame _gameinstance "NewEnumerator0" _levelname "None" (Variables|Default|GetTransform) _mapcoordinates)
  (Default|LoadSavedGame _gameinstance "0" true (Variables|Default|GetEntrance) (Utilities|String|ToString(Name) _levelname)))

(event Custom|CheckCoordinates
  (if (Utilities|IsinLevelBounds (Transformation|GetActorLocation (Game|Player|GetPlayerPawn 0)))
    (CallFunction|ReturntoMap)
    (elif (Utilities|IsinLevelBounds (Transformation|GetActorLocation (Variables|Default|GetCamper)))
      (CallFunction|ReturntoMap))))

(event EventBeginPlay
  (bind _asbp_em_path_game_instance (Utilities|Casting|CastToBP_EmPathGameInstance (Game|GetGameInstance)))
  (Variables|Default|SetGameInstance _asbp_em_path_game_instance)
  (bind _returnvalue (Actor|GetActorOfClass "/Game/EmPath/Blueprints/Camper/BP_CamperSmall.BP_CamperSmall_C"))
  (Variables|Default|SetCamper _returnvalue)
  (Utilities|Time|SetTimerbyEvent (delegate Custom|CheckCoordinates) 2.0 true))

(event Collision|EventActorBeginOverlap
  (params (OtherActor :type Actor%20Object%20Reference)))

(event EventTick
  (params (DeltaSeconds :type Float%20%28single-precision%29)))

(event Input|KeyboardEvents|DebugKeyZ
  (params (Key :type Key%20Structure) (ActionValue :type Input%20Action%20Value%20Structure))
  (:Pressed
    (Development|PrintString (Utilities|String|ToString(Vector) (Transformation|GetActorLocation (Game|Player|GetPlayerPawn 0))))))

(fn ConstructionScript)