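; BP_WaypointZone is a trigger sphere with a configurable radius that announces a named waypoint when the player enters it.
; After a one-second startup delay, it caches the player controller and disables the popup if that waypoint was already visited.
; The first valid overlap plays a chanting sound and shows WB_WaypointPopup.
; VisitedWaypoints is reassigned to itself because the Add node is unwired, and the cached MusicPlayer goes unused.
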(event `self.ReceiveBeginPlay`
  (`KismetSystemLibrary.Delay` 1.0)
  (`|ExecutionSequence`
    (:`then_0`
      ;[1 1 1] Get a reference to PlayerController
      (bind _asbp_em_path_game_player_controller (cast `/Game/MRPGT/Blueprints/Controllers/BP_EmPathGamePlayerController` (`GameplayStatics.GetPlayerController` 0)))
      (set `self.PlayerController` _asbp_em_path_game_player_controller))
    (:`then_1`
      (if (`/Game/MRPGT/Blueprints/Controllers/BP_EmPathGamePlayerController.HasVisitedWaypoint` (`self.PlayerController`) (`self.WaypointName`))
        (set `self.DisablePopup` true)))
    (:`then_2`
      (bind _outactors (`GameplayStatics.GetAllActorsOfClass` "/Game/EmPath/Blueprints/BP_MusicPlayer.BP_MusicPlayer_C"))
      (set `self.MusicPlayer` (`|GetArrayItem` _outactors)))))

(event `self.Sphere.OnComponentBeginOverlap`
  (params (OverlappedComponent :type "PrimitiveComponent Object Reference") (OtherActor :type "Actor Object Reference") (OtherComp :type "PrimitiveComponent Object Reference") (OtherBodyIndex :type Integer) (bFromSweep :type Boolean) (SweepResult :type "HitResult Structure (by ref)"))
  (bind _playercontroller (`self.PlayerController`))
  (if (== OtherActor (`GameplayStatics.GetPlayerPawn` 0))
    (if (not (`self.DisablePopup`))
      (`/Engine/EditorBlueprintResources/StandardMacros.DoOnce` false
        (:`Completed`
          (`GameplayStatics.PlaySound2D` "/Game/EmPath/Sounds/0_ElevenLabs/arcane_dark_chanting_1_.arcane_dark_chanting_1_" 1.0 1.0 0.0 null null)
          (bind _returnvalue (`|CreateWidget` "/Game/EmPath/UI/WB_WaypointPopup.WB_WaypointPopup_C" null (`self.WaypointName`)))
          (`UserWidget.AddToViewport` _returnvalue 10)
          (`/Engine/EditorBlueprintResources/StandardMacros.IsValid` _playercontroller
            (:`Is Valid`
              (set `/Game/MRPGT/Blueprints/Controllers/BP_EmPathGamePlayerController.VisitedWaypoints` (`/Game/MRPGT/Blueprints/Controllers/BP_EmPathGamePlayerController.VisitedWaypoints` _playercontroller) _playercontroller))))))))

(fn `UserConstructionScript`
  (`SphereComponent.SetSphereRadius` (`self.Sphere`) (`self.In Sphere Radius`) true))