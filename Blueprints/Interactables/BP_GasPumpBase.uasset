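; Base gas pump interactable that refuels the player's small camper when it is within the pump's sphere.
; Interact plays pumping audio and starts a looping timer that adds fuel through the player controller's needs, or reports the camper is too far.
; Each tick messages progress; near full, it reports completion, stops audio and invalidates the timer handle.
; The construction script shows gas station components when beam lights are enabled.
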(event `self.ReceiveBeginPlay`
  (bind _asbp_em_path_game_player_controller (cast `/Game/MRPGT/Blueprints/Controllers/BP_EmPathGamePlayerController` (`GameplayStatics.GetPlayerController` 0)))
  (set `self.InGamePlayerController` _asbp_em_path_game_player_controller))

(event `self.Sphere.OnComponentBeginOverlap`
  (params (OverlappedComponent :type "PrimitiveComponent Object Reference") (OtherActor :type "Actor Object Reference") (OtherComp :type "PrimitiveComponent Object Reference") (OtherBodyIndex :type Integer) (bFromSweep :type Boolean) (SweepResult :type "HitResult Structure (by ref)"))
  (if (== OtherActor "/Game/EmPath/Blueprints/Camper/BP_CamperSmall.BP_CamperSmall")
    (set `self.CamperCanRefuel` true)))

(event `self.Sphere.OnComponentEndOverlap`
  (params (OverlappedComponent :type "PrimitiveComponent Object Reference") (OtherActor :type "Actor Object Reference") (OtherComp :type "PrimitiveComponent Object Reference") (OtherBodyIndex :type Integer))
  (if (== OtherActor "/Game/EmPath/Blueprints/Camper/BP_CamperSmall.BP_CamperSmall")
    (set `self.CamperCanRefuel` false)))

(event `/Game/MRPGT/Blueprints/Interfaces/Interface_Interactable.Interact`
  (params (HitComponent :type "ActorComponent Object Reference") (InteractingActor :type "Actor Object Reference") (AlternativeInteract :type Boolean))
  (bind _audio (`self.Audio`))
  (`/Engine/EditorBlueprintResources/StandardMacros.IsValid` (`|GetArrayItem` (`PrimitiveComponent.GetOverlappingActors` (`self.Sphere`) "/Game/EmPath/Blueprints/Camper/BP_CamperSmall.BP_CamperSmall_C"))
    (:`Is Valid`
      (set `self.CamperCanRefuel` true))
    (:`Is Not Valid`
      _))
  (if (`self.CamperCanRefuel`)
    (`AudioComponent.SetSound` _audio "/Game/EmPath/Sounds/Matt_Script_-_Sputter__Glug__Sutter__Chug_/Coolspring_Power_Museum_4_hp_Fairbanks_Morse_Model_T_vertical_circa_1910_running_rhythmic_gears_mechanical_pumping_pressure_release.Coolspring_Power_Museum_4_hp_Fairbanks_Morse_Model_T_vertical_circa_1910_running_rhythmic_gears_mechanical_pumping_pressure_release")
    (`AudioComponent.Play` _audio 0.0)
    (bind _returnvalue (`KismetSystemLibrary.K2_SetTimerDelegate` (delegate `Refuel`) 3.0 true))
    (set `self.RefuelTimerHandle` _returnvalue)
    (`self.Refuel`)
    (else
      (`/Game/MRPGT/Blueprints/Controllers/BP_EmPathGamePlayerController.SendShortMessage` (`self.InGamePlayerController`) "Camper is too far"))))

(event `Refuel`
  (bind _ingameplayercontroller (`self.InGamePlayerController`))
  (bind _needs (`/Game/MRPGT/Blueprints/Controllers/BP_EmPathGamePlayerController.GetNeeds` _ingameplayercontroller))
  (bind (_calories _fun _urine _mood _fuel) (break `/Game/EmPath/Structures/S_Needs` _needs))
  (if (>= _fuel 99.0)
    (`/Game/MRPGT/Blueprints/Controllers/BP_EmPathGamePlayerController.SendShortMessage` _ingameplayercontroller "Refueling complete")
    (`AudioComponent.Stop` (`self.Audio`))
    (`KismetSystemLibrary.K2_InvalidateTimerHandle` (`self.RefuelTimerHandle`))
    (else
      (`/Game/MRPGT/Blueprints/Controllers/BP_EmPathGamePlayerController.UpdateNeeds` _ingameplayercontroller (make `/Game/EmPath/Structures/S_Needs` 0.0 0.0 0.0 0.0 10.0))
      (`/Game/MRPGT/Blueprints/Controllers/BP_EmPathGamePlayerController.SendShortMessage` _ingameplayercontroller (`KismetTextLibrary.Conv_StringToText` (`KismetStringLibrary.Concat_StrStr` "Fuel -" (`KismetStringLibrary.Conv_DoubleToString` (+ _fuel 10.0)) "%"))))))

(fn `UserConstructionScript`
  (`parent.UserConstructionScript`)
  (if (`self.HasBeamLights`)
    (`SceneComponent.SetVisibility` (`self.GasStation9`) true false)
    (`SceneComponent.SetVisibility` (`self.GasStation12`) true false)
    (`SceneComponent.SetVisibility` (`self.GasStation11`) true false)
    (`SceneComponent.SetVisibility` (`self.GasStation10`) true false)
    (`SceneComponent.SetVisibility` (`self.GasStation13`) true false)
    (`SceneComponent.SetVisibility` (`self.GasStation8`) true false)
    (`SceneComponent.SetVisibility` (`self.GasStation7`) true false)
    (`SceneComponent.SetVisibility` (`self.GasStation6`) true false)
    (`SceneComponent.SetVisibility` (`self.GasStation5`) true false)))