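; BP_LightPoint is an interactable point light actor that can be switched on and off.
; The On and Off events toggle the PointLight component's visibility.
; The construction script calls its parent, then applies the exposed intensity, attenuation radius and intensity units to the light.
; Lookingat is empty and GetObjectName returns an empty string, so the light gives no look-at response or name.
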(event `self.Off`
  (`SceneComponent.SetVisibility` (`self.PointLight`) false false))

(event `self.On`
  (`SceneComponent.SetVisibility` (`self.PointLight`) true false))

(event `self.LookingAt`
  (params (HitComponent :type "ActorComponent Object Reference")))

(fn `GetObjectName`
  (returns (NameOut :type String))
  (return ""))

(fn `UserConstructionScript`
  (bind _pointlight (`self.PointLight`))
  (`parent.UserConstructionScript`)
  (`LightComponent.SetIntensity` _pointlight (`self.Intensity`))
  (`LocalLightComponent.SetAttenuationRadius` _pointlight (`self.Radius`))
  (`LocalLightComponent.SetIntensityUnits` _pointlight (`self.Intensity Units`)))