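; BP_Projector is an interactable projector that plays a video playlist on a Media Plate in the level.
; On BeginPlay it waits briefly, casts the first actor tagged "Movie" to a Media Plate, takes its media player and starts the first playlist entry.
; Interact opens the playlist's next entry on that player, with short delays before each play call after opening.
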(event `self.ReceiveBeginPlay`
  (bind _player (`self.Player`))
  (bind _playlist (`self.Playlist`))
  (`KismetSystemLibrary.Delay` 1.0)
  (bind _outactors (`GameplayStatics.GetAllActorsWithTag` "Movie"))
  (bind _asmedia_plate (cast `MediaPlate` (`|GetArrayItem` _outactors)))
  (bind _returnvalue (`MediaPlateComponent.GetMediaPlayer` (`MediaPlate.MediaPlateComponent` _asmedia_plate)))
  (set `self.Player` _returnvalue)
  (`MediaPlayer.OpenPlaylist` _player _playlist)
  (`MediaPlayer.OpenPlaylistIndex` _player _playlist 0)
  (`KismetSystemLibrary.Delay` 1.0)
  (`MediaPlayer.Play` _player))

(event `/Game/MRPGT/Blueprints/Interfaces/Interface_Interactable.Interact`
  (params (HitComponent :type "ActorComponent Object Reference") (InteractingActor :type "Actor Object Reference") (AlternativeInteract :type Boolean))
  (bind _playlist (`self.Playlist`))
  (bind _inoutindex (`MediaPlaylist.GetNext` _playlist))
  (`MediaPlayer.OpenPlaylistIndex` (`self.Player`) _playlist _inoutindex)
  (`KismetSystemLibrary.Delay` 0.2)
  (`MediaPlayer.Play` (`self.Player`)))

(fn `UserConstructionScript`
  (`parent.UserConstructionScript`))