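; Interactable that teleports the first player's pawn to an arrow marker when used.
; Interact plays a 2D teleport sound, then calls TeleportToArrow on the Target reference if valid, otherwise on itself, so it can send the player to another teleporter's arrow or its own.
; TeleportToArrow moves the pawn to the arrow's world location and rotation, and also sets the controller's control rotation to match.
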(event `TeleportToArrow`
  (bind _arrow (`self.Arrow`))
  (bind _returnvalue (`SceneComponent.K2_GetComponentRotation` _arrow))
  (`self.K2_TeleportTo` (`GameplayStatics.GetPlayerPawn` 0) (`SceneComponent.K2_GetComponentLocation` _arrow) _returnvalue)
  (`Controller.SetControlRotation` (`GameplayStatics.GetPlayerController` 0) _returnvalue))

(event `/Game/MRPGT/Blueprints/Interfaces/Interface_Interactable.Interact`
  (params (HitComponent :type "ActorComponent Object Reference") (InteractingActor :type "Actor Object Reference") (AlternativeInteract :type Boolean))
  (bind _target (`self.Target`))
  (`GameplayStatics.PlaySound2D` (`self.TeleportSound`) 1.0 1.0 0.0 null null)
  (`/Engine/EditorBlueprintResources/StandardMacros.IsValid` _target
    (:`Is Valid`
      (`self.TeleportToArrow` _target))
    (:`Is Not Valid`
      (`self.TeleportToArrow` self))))

(fn `UserConstructionScript`
  (`parent.UserConstructionScript`))