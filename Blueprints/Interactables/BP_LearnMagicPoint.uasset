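; BP_LearnMagicPoint is an interactable point that teaches the player a spell.
; On Interact it sends its SpellName to the player pawn through LearnSpellsMessage, then a DoOnce plays a sound at its location and activates the Niagara effect only on the first use.
; The construction script assigns the SummoningCircle asset to the Niagara component.
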(event `/Game/MRPGT/Blueprints/Interfaces/Interface_Interactable.Interact`
  (params (HitComponent :type "ActorComponent Object Reference") (InteractingActor :type "Actor Object Reference") (AlternativeInteract :type Boolean))
  (message `/Game/EmPath/Interfaces/BI_GameActions.LearnSpells` (`GameplayStatics.GetPlayerPawn` 0) (`self.SpellName`) (struct))
  (`/Engine/EditorBlueprintResources/StandardMacros.DoOnce` false
    (:`Completed`
      (`GameplayStatics.PlaySoundAtLocation` (`self.Sound`) (`self.K2_GetActorLocation`) (struct) 1.0 1.0 0.0 null null null null)
      (`ActorComponent.Activate` (`self.Niagara`) true))))

(fn `UserConstructionScript`
  (`parent.UserConstructionScript`)
  (`NiagaraComponent.SetAsset` (`self.Niagara`) (`self.SummoningCircle`) true))