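; Interactable umbrella prop that toggles between open and closed by swapping its static mesh.
; Both interact events share one path that flips IsOpen, plays a drawer sound with randomized pitch and sets the matching mesh.
; The player pawn overlapping the Sphere also triggers the toggle through ForceInteract.
; The construction script applies the mesh for the initial IsOpen value, so placed instances show their starting state.
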(event `self.ReceiveBeginPlay`)

(event `ForceInteract`
  (bind _object (`self.Object`))
  (if true :!label _label
    (`GameplayStatics.PlaySoundAtLocation` "/Game/EmPath/Sounds/SoundFxwizard_-_Closets_Small_Doors/CST_Cutlery_Drawer_Open_Medium_SFXWiz.CST_Cutlery_Drawer_Open_Medium_SFXWiz" (`SceneComponent.K2_GetComponentLocation` (`self.Object`)) (struct) 1.0 (`KismetMathLibrary.RandomFloatInRange` 0.5 0.1) 0.0 "/Game/YI_TankCollection/Sounds/Master/SA_Standard.SA_Standard" null null null)
    (bind _output_get (set `self.IsOpen` (not (`self.IsOpen`))))
    (if _output_get
      (`StaticMeshComponent.SetStaticMesh` _object "/Game/CityPark/Meshes/Props/SM_Umbrella01.SM_Umbrella01")
      (else
        (`StaticMeshComponent.SetStaticMesh` _object "/Game/CityPark/Meshes/Props/SM_Umbrella02.SM_Umbrella02")))))

(event `/Game/MRPGT/Blueprints/Interfaces/Interface_Interactable.Interact`
  (params (HitComponent :type "ActorComponent Object Reference") (InteractingActor :type "Actor Object Reference") (AlternativeInteract :type Boolean))
  (goto _label))

(event `self.Sphere.OnComponentBeginOverlap`
  (params (OverlappedComponent :type "PrimitiveComponent Object Reference") (OtherActor :type "Actor Object Reference") (OtherComp :type "PrimitiveComponent Object Reference") (OtherBodyIndex :type Integer) (bFromSweep :type Boolean) (SweepResult :type "HitResult Structure (by ref)"))
  (if (== OtherActor (`GameplayStatics.GetPlayerPawn` 0))
    (`self.ForceInteract`)))

(fn `UserConstructionScript`
  (bind _object (`self.Object`))
  (`parent.UserConstructionScript`)
  (if (`self.IsOpen`)
    (`StaticMeshComponent.SetStaticMesh` _object "/Game/CityPark/Meshes/Props/SM_Umbrella01.SM_Umbrella01")
    (else
      (`StaticMeshComponent.SetStaticMesh` _object "/Game/CityPark/Meshes/Props/SM_Umbrella02.SM_Umbrella02"))))