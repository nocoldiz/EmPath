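; BP_SitPoint is an interactable that lets the player sit at its location and stand up again.
; Use toggles the Sitting state, rotating the pawn to face the Arrow on sitting or moving it to ReleasePoint on standing, then calls the parent Use.
; While seated, Tick pins player 0's pawn to the actor's location every frame, without attachment or any change to movement input.
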(event `self.ReceiveTick`
  (params (DeltaSeconds :type "Float (single-precision)"))
  (if (`self.Sitting`)
    (`self.K2_SetActorLocation` (`GameplayStatics.GetPlayerPawn` 0) (`self.K2_GetActorLocation`) false false)))

(fn `Use`
  (params (HorrorEvent :type Boolean))
  (locals (NewLocalVar :type "Pawn Object Reference"))
  (bind _returnvalue (`GameplayStatics.GetPlayerPawn` 0))
  (set `self.Sitting` (not (`self.Sitting`)))
  (if (`self.Sitting`)
    (`self.K2_SetActorRotation` _returnvalue (`KismetMathLibrary.Conv_VectorToRotator` (`SceneComponent.GetForwardVector` (`self.Arrow`))) false)
    (else
      (`self.K2_SetActorLocation` _returnvalue (`SceneComponent.K2_GetComponentLocation` (`self.ReleasePoint`)) false false)))
  (`parent.Use` HorrorEvent))

(fn `UserConstructionScript`
  (`parent.UserConstructionScript`))