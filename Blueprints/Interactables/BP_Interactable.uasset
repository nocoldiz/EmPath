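; BP_Interactable is an interactable object with a configurable mesh, name and action, apparently serving as a base for more specific interactables.
; The construction script applies the Mesh variable to the Object component.
; GetObjectName joins Action and Name into a label, while GetInfo reports the name as non-buyable and free.
; Lookingat is empty, and the ID, launcher and projectile queries return empty or false defaults.
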(event `self.LookingAt`
  (params (HitComponent :type "ActorComponent Object Reference")))

(fn `GetID`
  (returns (ID :type String))
  (return ""))

(fn `GetInfo`
  (returns (Name :type Text) (Buyable :type Boolean) (Price :type "Float (double-precision)") (Mesh :type "StaticMesh Object Reference"))
  (return (`KismetTextLibrary.Conv_StringToText` (`self.Name`)) false 0.0 null))

(fn `GetLauncherActor`
  (returns (LauncherActor :type "Actor Object Reference"))
  (return null))

(fn `GetObjectName`
  (returns (NameOut :type String))
  (return (`KismetStringLibrary.Concat_StrStr` (`self.Action`) " " (`self.Name`))))

(fn `IsProjectile`
  (returns (Result :type Boolean))
  (return false))

(fn `UserConstructionScript`
  (`StaticMeshComponent.SetStaticMesh` (`self.Object`) (`self.Mesh`)))