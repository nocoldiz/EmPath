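; Interactable radio that cycles through Off, FM, AM and EM bands, with alternate interact stepping the frequency.
; FM picks songs by station genre from data tables and chains them with retriggerable delays, starting the first mid-track.
; AM plays random excerpts at intervals, while EM plays one random track, gating one author behind RespectsGiven.
; It updates a HUD widget, passes song names to chat and notifies BP_MusicPlayer on power changes.
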(event `self.ReceiveBeginPlay`
  (bind _returnvalue (`|CreateWidget` "/Game/EmPath/UI/WB_RadioHUD.WB_RadioHUD_C" null 0.0 "NewEnumerator3" "NewEnumerator0" "None" "None" "" "None"))
  ;[1 1 1] Begin play
  (bind _output_get (set `self.RadioHUD` _returnvalue))
  (`UserWidget.AddToViewport` _output_get 0)
  (`/Game/EmPath/UI/WB_RadioHUD.SetHidden` _output_get)
  (bind _outrownames (`DataTableFunctionLibrary.GetDataTableRowNames` "/Game/EmPath/DataTables/DT_RadioStations.DT_RadioStations"))
  (for _array_element _outrownames
    (bind _returnvalue_2 (`|GetDataTableRow` "/Game/EmPath/DataTables/DT_RadioStations.DT_RadioStations" _array_element)
      (:`then`
        (`KismetArrayLibrary.Array_Add` (`self.FMRadio`) _returnvalue_2))))
  (set `self.MaxFMStation` (`KismetArrayLibrary.Array_Length` (`self.FMRadio`)))
  (`self.IntializeBestOf`))

(event `self.LookingAt`
  (params (HitComponent :type "ActorComponent Object Reference"))
  ;[1 1 1] E key will toggle light
)

(event `self.Interact`
  (params (HitComponent :type "ActorComponent Object Reference") (InteractingActor :type "Actor Object Reference") (AlternativeInteract :type Boolean))
  ;[1 1 1] E key will toggle light
  (if AlternativeInteract
    (if (not (`|EnumEquality` (`self.RadioType`) "NewEnumerator3"))
      (`self.SetFrequency` false))
    (else
      (`/Game/EmPath/Interfaces/BI_Radio.CycleBand`))))

(event `/Game/EmPath/Interfaces/BI_Radio.CycleBand`
  (bind _radiohud (`self.RadioHUD`))
  (bind _radiohud_2 (`self.RadioHUD`))
  (bind _radiohud_3 (`self.RadioHUD`))
  (bind _radiohud_4 (`self.RadioHUD`))
  ;[1 1 1] CycleBand
  (switch `/Game/EmPath/Enum/E_Radio` (`self.RadioType`)
    (:`NewEnumerator3`
      (set `self.RadioType` "NewEnumerator1")
      (set `self.Frequency` (`self.LastFM`))
      (`TextRenderComponent.K2_SetText` (`self.TextRender1`) (`self.FMValue`))
      (`/Game/EmPath/UI/WB_RadioHUD.SetBand` _radiohud "NewEnumerator1")
      (`/Game/EmPath/UI/WB_RadioHUD.SetVisible` _radiohud_3)
      (`/Game/EmPath/UI/WB_RadioHUD.SetFrequencyText` _radiohud_3 (`self.Frequency`))
      (`self.GetRandomSongOfCurrentGender`)
      (bind _outactors (`GameplayStatics.GetAllActorsOfClass` "/Game/EmPath/Blueprints/BP_MusicPlayer.BP_MusicPlayer_C"))
      (bind _output (`|GetArrayItem` _outactors))
      (`/Engine/EditorBlueprintResources/StandardMacros.IsValid` _output
        (:`Is Valid`
          (message `/Game/EmPath/Interfaces/BI_MusicPlayer.SetMusic` _output true))))
    (:`NewEnumerator0`
      (set `self.RadioType` "NewEnumerator2")
      (set `self.Frequency` (`self.LastEM`))
      (`TextRenderComponent.K2_SetText` (`self.TextRender1`) (`self.EmValue`))
      (`/Game/EmPath/UI/WB_RadioHUD.SetBand` _radiohud "NewEnumerator2")
      (`/Game/EmPath/UI/WB_RadioHUD.SetVisible` _radiohud_2)
      (`self.PlayNoise`)
      (set `/Game/EmPath/UI/WB_RadioHUD.RadioNameText` "em.Path" _radiohud_2)
      (set `/Game/EmPath/UI/WB_RadioHUD.MusicGenre` "NewEnumerator93" _radiohud_2)
      (`/Game/EmPath/UI/WB_RadioHUD.SetFrequencyText` _radiohud_2 (`self.Frequency`))
      (`self.GetEMStation`))
    (:`NewEnumerator1`
      (set `self.RadioType` "NewEnumerator0")
      (set `self.Frequency` (`self.LastAM`))
      (set `self.Volume` 1.0)
      (`TextRenderComponent.K2_SetText` (`self.TextRender1`) (`self.AMValue`))
      (`/Game/EmPath/UI/WB_RadioHUD.SetBand` _radiohud "NewEnumerator0")
      (`/Game/EmPath/UI/WB_RadioHUD.SetVisible` _radiohud_4)
      (`self.PlayNoise`)
      (`/Game/EmPath/UI/WB_RadioHUD.SetFrequencyText` _radiohud_4 (`self.Frequency`))
      (set `/Game/EmPath/UI/WB_RadioHUD.MusicGenre` "NewEnumerator95" _radiohud_4)
      (set `/Game/EmPath/UI/WB_RadioHUD.RadioNameText` "???" _radiohud_4)
      (`self.GetAMRadioStation`))
    (:`NewEnumerator2`
      (set `self.RadioType` "NewEnumerator3")
      (set `self.Volume` 0.0)
      (`AudioComponent.Stop` (`self.Audio`))
      (`TextRenderComponent.K2_SetText` (`self.TextRender1`) (`self.OffValue`))
      (set `self.RadioStationIndex` 0)
      (bind _outactors_2 (`GameplayStatics.GetAllActorsOfClass` "/Game/EmPath/Blueprints/BP_MusicPlayer.BP_MusicPlayer_C"))
      (bind _output_2 (`|GetArrayItem` _outactors_2))
      (`/Engine/EditorBlueprintResources/StandardMacros.IsValid` _output_2
        (:`Is Valid`
          (message `/Game/EmPath/Interfaces/BI_MusicPlayer.SetMusic` _output_2 false))
        (:`Is Not Valid`
          _))
      (set `/Game/EmPath/UI/WB_RadioHUD.RadioStation` "NewEnumerator3" (`self.RadioHUD`)))))

(event `GetAMRadioStation`
  (bind _audio (`self.Audio`))
  ;[1 1 1] GetAMRadioStation
  (bind _outrownames (`DataTableFunctionLibrary.GetDataTableRowNames` "/Game/EmPath/DataTables/DT_AutoradioAM.DT_AutoradioAM"))
  (bind _returnvalue (`|GetDataTableRow` "/Game/EmPath/DataTables/DT_AutoradioAM.DT_AutoradioAM" (`KismetArrayLibrary.Array_Random` _outrownames))
    (:`then`
      (bind (_name _author _lyrics _music) (break `/Game/EmPath/Structures/S_Music` _returnvalue))
      ;[1 1 1] CycleBand
      (`|LoadAsset` _music
        (:`Completed`
          (`KismetSystemLibrary.Delay` 0.2)
          (if (`AudioComponent.IsPlaying` _audio)
            (`AudioComponent.Stop` _audio))
          (bind _output (`|ConvertAsset` _music))
          (`AudioComponent.SetSound` _audio _output)
          (`/Engine/EditorBlueprintResources/StandardMacros.IsValid` _audio
            (:`Is Valid`
              (`AudioComponent.Play` _audio (`KismetMathLibrary.RandomFloatInRange` 0.0 (- (`SoundBase.Duration` _output) 10.0)))
              (`KismetSystemLibrary.RetriggerableDelay` 30.0)
              (if (`|EnumEquality` (`self.RadioType`) "NewEnumerator0")
                (`self.GetAMRadioStation`)))))))))

(event `GetCurrentFMRadioStation`
  (bind _radiohud (`self.RadioHUD`))
  (bind (_name _genre) (break `/Game/EmPath/Structures/S_RadioStation` (`self.CurrentRadio`)))
  ;[1 1 1] Get current radio station
  (switch `/Game/EmPath/Enum/E_Radio` (`self.RadioType`)
    (:`NewEnumerator0`
      (`self.PlayNoise`))
    (:`NewEnumerator1`
      (set `self.CurrentRadio` (`|GetArrayItem` (`self.FMRadio`) (`self.RadioStationIndex`)))
      (set `self.CurrentGenre` _genre)
      (set `/Game/EmPath/UI/WB_RadioHUD.MusicGenre` _genre _radiohud)
      (set `/Game/EmPath/UI/WB_RadioHUD.RadioNameText` _name _radiohud)
      (if (`|EnumEquality` _genre "NewEnumerator103")
        _
        (elif (`|EnumEquality` _genre "NewEnumerator95")
          (`self.GetRandomFMSong`)
          (else
            (`self.GetRandomSongOfCurrentGender`)))))
    (:`NewEnumerator2`
      (`self.PlayNoise`))))

(event `GetEMStation`
  (bind _audio (`self.Audio`))
  ;[1 1 1] GetEMRadioStation
  (`KismetSystemLibrary.RetriggerableDelay` 1.0)
  (bind _outrownames (`DataTableFunctionLibrary.GetDataTableRowNames` "/Game/EmPath/DataTables/DT_Music.DT_Music"))
  (bind _returnvalue (`|GetDataTableRow` "/Game/EmPath/DataTables/DT_Music.DT_Music" (`KismetArrayLibrary.Array_Random` _outrownames))
    (:`then`
      (bind (_name _author _lyrics _music) (break `/Game/EmPath/Structures/S_Music` _returnvalue))
      (bind _returnvalue_2 (`|EnumEquality` _author "NewEnumerator1"))
      (if (and _returnvalue_2 (`self.RespectsGiven`))
        (`KismetSystemLibrary.LoadAsset_Blocking` _music :!label _label)
        (`KismetSystemLibrary.Delay` 0.2)
        (bind _output (`|ConvertAsset` _music))
        (bind _duration (`SoundBase.Duration` _output))
        (if (> _duration 0.0)
          (if (`AudioComponent.IsPlaying` _audio)
            (`AudioComponent.Stop` _audio))
          (`AudioComponent.SetSound` _audio _output)
          (`AudioComponent.Play` _audio 0.0)
          (`self.Update Song HUD` _name _lyrics (`KismetTextLibrary.Conv_StringToText` (`|GetEnumeratorNameAsString` _author)) "NewEnumerator93")
          (`KismetSystemLibrary.RetriggerableDelay` _duration)
          (if (`|EnumEquality` (`self.RadioType`) "NewEnumerator2")
            _))
        (elif _returnvalue_2
          (`self.GetEMStation`)
          (else
            (goto _label)))))))

(event `GetRandomFMSong`
  (bind _radiohud (`self.RadioHUD`))
  (bind (_name _genre) (break `/Game/EmPath/Structures/S_RadioStation` (`self.CurrentRadio`)))
  ;[1 1 1] Get current radio station
  (switch `/Game/EmPath/Enum/E_Radio` (`self.RadioType`)
    (:`NewEnumerator0`
      (`self.PlayNoise`))
    (:`NewEnumerator1`
      (set `self.CurrentRadio` (`|GetArrayItem` (`self.FMRadio`) (`self.RadioStationIndex`)))
      (set `self.CurrentGenre` _genre)
      (set `/Game/EmPath/UI/WB_RadioHUD.MusicGenre` _genre _radiohud)
      (set `/Game/EmPath/UI/WB_RadioHUD.RadioNameText` _name _radiohud)
      (if (`|EnumEquality` _genre "NewEnumerator103")
        _
        (elif (`|EnumEquality` _genre "NewEnumerator95")
          (`self.GetRandomFMSong`)
          (else
            (`self.GetRandomSongOfCurrentGender`)))))
    (:`NewEnumerator2`
      (`self.PlayNoise`))))

(event `IntializeBestOf`
  ;[1 1 1] InitializeBestOF
  (bind _outrownames (`DataTableFunctionLibrary.GetDataTableRowNames` "/Game/EmPath/DataTables/DT_AutoRadio.DT_AutoRadio"))
  (for _array_element _outrownames
    (bind _returnvalue (`|GetDataTableRow` "/Game/EmPath/DataTables/DT_AutoRadio.DT_AutoRadio" _array_element)
      (:`then`
        (if (`.WasInTop10_23_382FA930470B2B9C0526DAA0F24F984D` (break `/Game/EmPath/Structures/S_Music` _returnvalue))
          (`KismetArrayLibrary.Array_Add` (`self.BestOI`)))))))

(event `GetBestOfFMSong`
  (bind _audio (`self.Audio`))
  (bind _currentsongs (`self.CurrentSongs`))
  (bind _currentsongs_2 (`self.CurrentSongs`))
  (bind _currentgenre (`self.CurrentGenre`))
  (bind _returnvalue (`KismetArrayLibrary.Array_Length` _currentsongs))
  (bind _returnvalue_2 (== (`self.SongsPlayedSameStation`) 0))
  (bind (_name _author _lyrics _music _loop _album _radiostation) (break `/Game/EmPath/Structures/S_Music` (`|GetArrayItem` _currentsongs (`self.Next`))))
  (bind _output (`|ConvertAsset` _music))
  (bind _duration (`SoundBase.Duration` _output))
  (bind _returnvalue_3 (/ _duration 2.0))
  (bind _returnvalue_4 (`KismetMathLibrary.SelectFloat` _returnvalue_3 0.0 _returnvalue_2))
  (set `self.CurrentGenre` "NewEnumerator103")
  (set `self.Next` 0)
  (`KismetArrayLibrary.Array_Clear` _currentsongs_2)
  (`KismetArrayLibrary.Array_Add` _currentsongs_2 (`KismetArrayLibrary.Array_Random` (`self.BestOI`)))
  (`KismetSystemLibrary.RetriggerableDelay` 1.0 :!label _label_2)
  ;[1 1 1] Start playing FM song
  (if (== _returnvalue 0)
    ;[1 1 1] Noise
    (`self.PlayNoise`)
    (else
      (`|LoadAsset` _music
        (:`Completed`
          (`/Engine/EditorBlueprintResources/StandardMacros.IsValid` _output
            (:`Is Valid`
              (`AudioComponent.SetSound` _audio _output)
              (`AudioComponent.Play` _audio _returnvalue_4)
              (`self.Update Song HUD` _name _lyrics _album _radiostation (`KismetTextLibrary.Conv_StringToText` (`KismetStringLibrary.Concat_StrStr` (`KismetTextLibrary.Conv_TextToString` (`KismetTextLibrary.Conv_IntToText` (`self.Next`))) "/" (`KismetStringLibrary.Conv_IntToString` _returnvalue))))
              (set `self.TrackDuration` _returnvalue_4)
              (if (> _duration 0.0)
                (`KismetSystemLibrary.RetriggerableDelay` (`KismetMathLibrary.SelectFloat` _returnvalue_3 _duration _returnvalue_2))
                (`/Engine/EditorBlueprintResources/StandardMacros.IncrementInt` (`self.SongsPlayedSameStation`)
                  (:`  `
                    (if (`|EnumEquality` (`self.RadioType`) "NewEnumerator1")
                      (if (`|EnumEquality` _currentgenre "NewEnumerator95")
                        (`self.GetRandomFMSong`)
                        (elif (`|EnumEquality` _currentgenre "NewEnumerator103")
                          (`self.GetBestOfFMSong`)
                          (else
                            (`self.GetRandomSongOfCurrentGender` :!label _label_3)))))))
                (else
                  (goto _label_3))))
            (:`Is Not Valid`
              (`self.GetRandomSongOfCurrentGender`))))))))

(event `GetRandomSongOfCurrentGender`
  (bind _currentsongs (`self.CurrentSongs`))
  (`KismetArrayLibrary.Array_Clear` _currentsongs)
  ;[1 1 1] Get song of the current gengre
  (bind _outrownames (`DataTableFunctionLibrary.GetDataTableRowNames` "/Game/EmPath/DataTables/DT_AutoRadio.DT_AutoRadio"))
  (for _array_element _outrownames
    (bind _returnvalue (`|GetDataTableRow` "/Game/EmPath/DataTables/DT_AutoRadio.DT_AutoRadio" _array_element)
      (:`then`
        (if (`|EnumEquality` (`.RadioStation_20_D02C079140A71EF17CB63E9F38124A66` (break `/Game/EmPath/Structures/S_Music` _returnvalue)) (`self.CurrentGenre`))
          (`KismetArrayLibrary.Array_Add` _currentsongs _returnvalue)))))
  (set `self.Next` (`KismetMathLibrary.RandomIntegerInRange` 0 (`KismetArrayLibrary.Array_Length` _currentsongs)))
  (goto _label_2))

(event `CustomEvent`
  (bind _radiohud (`self.RadioHUD`))
  ;[1 1 1] Noise
  (`AudioComponent.SetSound` (`self.Audio`) null)
  (set `/Game/EmPath/UI/WB_RadioHUD.SongNameText` "" _radiohud)
  (set `/Game/EmPath/UI/WB_RadioHUD.AlbumNameText` "" _radiohud)
  (set `/Game/EmPath/UI/WB_RadioHUD.IndexText` "" _radiohud))

(event `ForceFrequency`
  (bind _radiohud (`self.RadioHUD`))
  (bind _frequency (`self.Frequency`))
  (bind _frequency_2 (`self.Frequency`))
  ;[1 1 1] Set frequency
  (`TextRenderComponent.K2_SetText` (`self.TextRender1`) (`KismetTextLibrary.Conv_StringToText` (`KismetStringLibrary.Concat_StrStr` (`KismetStringLibrary.Conv_DoubleToString` _frequency_2) (`|GetEnumeratorNameAsString` (`self.RadioType`)))) :!label _label_4)
  (`/Game/EmPath/UI/WB_RadioHUD.SetVisible` _radiohud)
  (`/Game/EmPath/UI/WB_RadioHUD.SetFrequencyText` _radiohud _frequency_2)
  (switch `/Game/EmPath/Enum/E_Radio` (`self.RadioType`)
    (:`NewEnumerator0`
      (set `self.LastAM` _frequency)
      (`self.GetAMRadioStation`))
    (:`NewEnumerator1`
      (`self.GetCurrentFMRadioStation`))
    (:`NewEnumerator2`
      (set `self.LastEM` _frequency)
      (`self.GetEMStation`))))

(event `/Game/EmPath/Interfaces/BI_Radio.SetFrequency`
  (params (Inverse :type Boolean))
  (bind _frequency (`self.Frequency`))
  (bind _radiostationindex (`self.RadioStationIndex`))
  ;[1 1 1] Set frequency
  (set `self.SongsPlayedSameStation` 0)
  (if (`|EnumInequality` (`self.RadioType`) "NewEnumerator3")
    (if Inverse
      (if (< (`self.Frequency`) (`self.MinRangeFM`))
        (set `self.Frequency` (`self.MaxRangeFm`))
        (set `self.RadioStationIndex` (- (`self.MaxFMStation`) 1))
        (goto _label_4)
        (else
          (set `self.Frequency` (- _frequency 0.8))
          (if (not (<= _radiostationindex 0))
            (`/Engine/EditorBlueprintResources/StandardMacros.DecrementInt` _radiostationindex
              (:`  `
                (goto _label_4))))))
      (elif (> (`self.Frequency`) (`self.MaxRangeFm`))
        ;;[1 1 1] ResetFmFromStart
        (set `self.Frequency` (`self.MinRangeFM`))
        (set `self.RadioStationIndex` 0)
        (goto _label_4)
        (else
          (set `self.Frequency` (+ _frequency 0.8))
          (`/Engine/EditorBlueprintResources/StandardMacros.IncrementInt` _radiostationindex
            (:`  `
              (goto _label_4))))))))

(fn `AlternativeUse`
  (params (InString :type String)))

(fn `GetID`
  (returns (ID :type String))
  (return ""))

(fn `GetInfo`
  (returns (Name :type Text) (Buyable :type Boolean) (Price :type "Float (double-precision)") (Mesh :type "StaticMesh Object Reference"))
  (return (`KismetTextLibrary.Conv_StringToText` "Radio") false 0.0 null))

(fn `GetLauncherActor`
  (returns (LauncherActor :type "Actor Object Reference"))
  (return null))

(fn `GetObjectName`
  (returns (NameOut :type String))
  (bind _returnvalue (`|EnumEquality` (`self.RadioType`) "NewEnumerator3"))
  (bind _returnvalue_2 (`KismetStringLibrary.Concat_StrStr` (`self.RadioButton`) (`KismetMathLibrary.SelectString` "Turn on" (`KismetMathLibrary.SelectString` "Turn off" "Change band" (`|EnumEquality` (`self.RadioType`) "NewEnumerator2")) _returnvalue)))
  (return (`KismetMathLibrary.SelectString` _returnvalue_2 (`KismetStringLibrary.Concat_StrStr` _returnvalue_2 "" "/ " (`self.PreviousStationButton`) " " "Next station" "/" (`self.NextStationButton`) "Previous station") _returnvalue)))

(fn `IsProjectile`
  (returns (Result :type Boolean))
  (return false))

(fn `PlayNoise`
  (bind _radiohud (`self.RadioHUD`))
  (set `/Game/EmPath/UI/WB_RadioHUD.SongNameText` "" _radiohud)
  (set `/Game/EmPath/UI/WB_RadioHUD.AlbumNameText` "" _radiohud)
  (set `/Game/EmPath/UI/WB_RadioHUD.IndexText` "" _radiohud))

(fn `Update Song HUD`
  (params (SongNameText :type Text) (Lyrics :type Text) (AlbumNameText :type Text) (MusicGenre :type "/Game/EmPath/Enum/E_MusicGenres Enum" :default "NewEnumerator0") (IndexText :type Text))
  (bind _radiohud (`self.RadioHUD`))
  (set `/Game/EmPath/UI/WB_RadioHUD.IndexText` IndexText _radiohud)
  (set `/Game/EmPath/UI/WB_RadioHUD.Lyrics` Lyrics _radiohud)
  (set `/Game/EmPath/UI/WB_RadioHUD.SongNameText` SongNameText _radiohud)
  (set `/Game/EmPath/UI/WB_RadioHUD.MusicGenre` MusicGenre _radiohud)
  (set `/Game/EmPath/UI/WB_RadioHUD.AlbumNameText` AlbumNameText _radiohud)
  (bind _foundwidgets (`WidgetBlueprintLibrary.GetAllWidgetsOfClass` "/Game/ChatTimeSystem/Widget/WBP_Chat.WBP_Chat_C"))
  (bind _output (`|GetArrayItem` _foundwidgets))
  (`/Engine/EditorBlueprintResources/StandardMacros.IsValid` _output
    (:`Is Valid`
      (`/Game/ChatTimeSystem/Widget/WBP_Chat.UpdateLyrics` _output SongNameText))))

(fn `UserConstructionScript`)