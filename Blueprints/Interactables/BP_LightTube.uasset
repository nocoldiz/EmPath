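; BP_LightTube is a light tube interactable built around a rect light that can be switched on and off.
; The construction script runs the parent's, then applies exposed-style variables for intensity, units, attenuation radius, source size and color to the RectLight.
; On and Off events only toggle the light's visibility.
; Lookingat is an empty stub and GetObjectName returns an empty string.
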(event `/Game/EmPath/Interfaces/BI_WorldInteraction.Off`
  (`SceneComponent.SetVisibility` (`self.RectLight`) false false))

(event `/Game/EmPath/Interfaces/BI_WorldInteraction.On`
  (`SceneComponent.SetVisibility` (`self.RectLight`) true false))

(event `/Game/MRPGT/MedievalBuildings01/Blueprints/BPI_PlayerInterface.LookingAt`
  (params (HitComponent :type "ActorComponent Object Reference")))

(fn `GetObjectName`
  (returns (NameOut :type String))
  (return ""))

(fn `UserConstructionScript`
  (bind _rectlight (`self.RectLight`))
  (`parent.UserConstructionScript`)
  (`LightComponent.SetIntensity` _rectlight (`self.Intensity`))
  (`LocalLightComponent.SetAttenuationRadius` _rectlight (`self.Radius`))
  (`LocalLightComponent.SetIntensityUnits` _rectlight (`self.Intensity Units`))
  (`RectLightComponent.SetSourceWidth` _rectlight (`self.SourceWidth`))
  (`RectLightComponent.SetSourceHeight` _rectlight (`self.SourceHeight`))
  (`LightComponent.SetLightColor` _rectlight (`self. Light Color`) true))