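; BP_Switch is an interactable two-state switch, labelled as lighting or blowing out a candle, that turns linked actors on or off.
; Both Interact and Lookingat set the on/off mesh from ToggleSwitch, then flip it.
; The new state is sent as OnMessage or OffMessage to ActorsToActivate implementing BI_WorldInteraction.
; The construction script sets the initial mesh, and GetObjectName picks the label from the state.
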(event `self.LookingAt`
  (params (HitComponent :type "ActorComponent Object Reference"))
  ;[1 1 1] E key will toggle light
  (`StaticMeshComponent.SetStaticMesh` (`self.Switch`) (select `bool` (`self.ToggleSwitch`) :`false` (`self.MeshOff`) :`true` (`self.MeshOn`)) :!label _label)
  (set `self.ToggleSwitch` (not (`self.ToggleSwitch`)))
  (for _array_element (`self.ActorsToActivate`)
    (if (`KismetSystemLibrary.DoesImplementInterface` _array_element "/Game/EmPath/Interfaces/BI_WorldInteraction.BI_WorldInteraction_C")
      (if (`self.ToggleSwitch`)
        (message `/Game/EmPath/Interfaces/BI_WorldInteraction.On` _array_element)
        (else
          (message `/Game/EmPath/Interfaces/BI_WorldInteraction.Off` _array_element))))))

(event `self.Interact`
  (params (HitComponent :type "ActorComponent Object Reference") (InteractingActor :type "Actor Object Reference") (AlternativeInteract :type Boolean))
  ;[1 1 1] E key will toggle light
  (goto _label))

(fn `GetID`
  (returns (ID :type String))
  (return ""))

(fn `GetInfo`
  (returns (Name :type Text) (Buyable :type Boolean) (Price :type "Float (double-precision)") (Mesh :type "StaticMesh Object Reference"))
  (return (`KismetTextLibrary.Conv_StringToText` (`self.Name`)) false 0.0 null))

(fn `GetLauncherActor`
  (returns (LauncherActor :type "Actor Object Reference"))
  (return null))

(fn `GetObjectName`
  (returns (NameOut :type String))
  (if (`self.ToggleSwitch`)
    (return "Blow Out Candle")
    (else
      (return "Light Candle"))))

(fn `IsProjectile`
  (returns (Result :type Boolean))
  (return false))

(fn `UserConstructionScript`
  (`StaticMeshComponent.SetStaticMesh` (`self.Switch`) (select `bool` (`self.ToggleSwitch`) :`false` (`self.MeshOff`) :`true` (`self.MeshOn`))))