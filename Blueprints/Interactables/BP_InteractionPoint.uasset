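; BP_InteractionPoint is a configurable interactable, triggered by an Interact event or by player overlap with its sphere when collision interaction is enabled.
; Each use runs a sequence of optional effects: message, particles, sound, damage, player status effect and actor spawning, plus a needs update to the player controller.
; It then starts an optional delay-based cooldown that blocks re-use, or destroys itself if set to single use.
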(event `self.ReceiveBeginPlay`)

(event `/Game/MRPGT/Blueprints/Interfaces/Interface_Interactable.Interact`
  (params (HitComponent :type "ActorComponent Object Reference") (InteractingActor :type "Actor Object Reference") (AlternativeInteract :type Boolean))
  (bind _infomessage (`self.InfoMessage`))
  (bind _audio (`self.Audio`))
  (bind _damage (`self.Damage`))
  (bind _status (`self.Status`))
  (bind _spawnedactor (`self.SpawnedActor`))
  (bind _interactioncooldown (`self.InteractionCooldown`))
  (bind _niagarafx (`self.NiagaraFx`))
  (bind _cascadefx (`self.CascadeFx`))
  (bind _particlefx (`self.ParticleFx`))
  (bind _sound (`self.Sound`))
  (if (not (`self.Cooldown`))
    (`|ExecutionSequence`
      (:`then_0`
        (if (not (`KismetTextLibrary.TextIsEmpty` _infomessage))
          (message `/Game/MRPGT/Blueprints/Interfaces/Interface_Messaging.SendShortMessage` (`GameplayStatics.GetPlayerController` 0) _infomessage)))
      (:`then_1`
        (message `/Game/EmPath/Interfaces/BPI_Damagable.SetNeeds` (`GameplayStatics.GetPlayerController` 0) (`self.Needs`)))
      (:`then_2`
        (`/Engine/EditorBlueprintResources/StandardMacros.IsValid` _niagarafx
          (:`Is Valid`
            (`NiagaraFunctionLibrary.SpawnSystemAtLocation` _niagarafx (`SceneComponent.K2_GetComponentLocation` _particlefx) (`SceneComponent.K2_GetComponentRotation` _particlefx)))))
      (:`then_3`
        (`/Engine/EditorBlueprintResources/StandardMacros.IsValid` _cascadefx
          (:`Is Valid`
            (`GameplayStatics.SpawnEmitterAttached` _cascadefx))))
      (:`then_4`
        (`/Engine/EditorBlueprintResources/StandardMacros.IsValid` _sound
          (:`Is Valid`
            (`AudioComponent.SetSound` _audio _sound)
            (`AudioComponent.Play` _audio 0.0))))
      (:`then_5`
        (if (!= _damage 0.0)
          (`/Game/EmPath/Interfaces/BPI_Damagable.TakeDamage` (make `/Game/EmPath/Structures/S_DamageInfo` _damage (`self.Damage Type`) (`self.Damage Response`)) (`GameplayStatics.GetPlayerPawn` 0) (`self.K2_GetActorLocation`))))
      (:`then_6`
        (if (`|EnumInequality` _status "NewEnumerator12")
          (message `/Game/EmPath/Interfaces/BPI_Damagable.ApplyStatus` (`GameplayStatics.GetPlayerPawn` 0) _status (`self.StatusDuration`) (`self.StatusMagnitude`) false (`self.StatusSuccess Rate`) "None")))
      (:`then_7`
        (`/Engine/EditorBlueprintResources/StandardMacros.IsValid` _spawnedactor
          (:`Is Valid`
            (`|SpawnActorFromClass` (`GameplayStatics.GetObjectClass` _spawnedactor) (`SceneComponent.K2_GetComponentToWorld` (`self.SpawnActor`)) "Undefined" "MultiplyWithRoot" _spawnedactor null))))
      (:`then_11`
        (if (> _interactioncooldown 0.0)
          (set `self.Cooldown` true)
          (`KismetSystemLibrary.Delay` _interactioncooldown)
          (set `self.Cooldown` false)))
      (:`then_12`
        (if (`self.DestroyAfterUse`)
          (`self.K2_DestroyActor`))))))

(event `self.InteractionSphere.OnComponentBeginOverlap`
  (params (OverlappedComponent :type "PrimitiveComponent Object Reference") (OtherActor :type "Actor Object Reference") (OtherComp :type "PrimitiveComponent Object Reference") (OtherBodyIndex :type Integer) (bFromSweep :type Boolean) (SweepResult :type "HitResult Structure (by ref)"))
  (bind _returnvalue (`GameplayStatics.GetPlayerPawn` 0))
  (if (and (== OtherActor _returnvalue) (`self.InteractByCollision`))
    (`/Game/MRPGT/Blueprints/Interfaces/Interface_Interactable.Interact` null _returnvalue)))

(event `self.InteractionSphere.OnComponentEndOverlap`
  (params (OverlappedComponent :type "PrimitiveComponent Object Reference") (OtherActor :type "Actor Object Reference") (OtherComp :type "PrimitiveComponent Object Reference") (OtherBodyIndex :type Integer)))

(fn `UserConstructionScript`
  (`parent.UserConstructionScript`))