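; Interactable bed that lets the player sleep to pass in-game time, except in the in_casalpusterlengo level.
; Sleep shows a HUD map message while chained DayDelay macros step the W_Clock widget forward hour by hour, then hides it and advances BP_TimeManager.
; A debug counter prints each use and, past a threshold, sends the player to in_casalpusterlengo.
; A long run of further DayDelay steps is left disconnected.
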(event `Sleep`
  (bind _returnvalue (`PlayerController.GetHUD` (`GameplayStatics.GetPlayerController` 0)))
  (message `/Game/MRPGT/Blueprints/MapSystem/Interface_Map.ToggleMap` _returnvalue true)
  (`KismetSystemLibrary.Delay` 0.2)
  (bind _foundwidgets (`WidgetBlueprintLibrary.GetAllWidgetsOfClass` "/Game/EmPath/UI/W_Clock.W_Clock_C" false))
  (set `self.Clock` (`|GetArrayItem` _foundwidgets))
  (`self.DayDelay`)
  (`self.DayDelay`)
  (`self.DayDelay`)
  (`KismetSystemLibrary.Delay` 1.0)
  (message `/Game/MRPGT/Blueprints/MapSystem/Interface_Map.ToggleMap` _returnvalue false)
  (bind _outactors (`GameplayStatics.GetAllActorsOfClass` "/Game/EmPath/Blueprints/BP_TimeManager.BP_TimeManager_C"))
  (bind _output (`|GetArrayItem` _outactors))
  (`/Engine/EditorBlueprintResources/StandardMacros.IsValid` _output
    (:`Is Valid`
      (`/Game/EmPath/Blueprints/BP_TimeManager.AdvanceTime` _output))))

(event `/Game/MRPGT/Blueprints/Interfaces/Interface_Interactable.Interact`
  (params (HitComponent :type "ActorComponent Object Reference") (InteractingActor :type "Actor Object Reference") (AlternativeInteract :type Boolean))
  (bind _debuguses (`self.DebugUses`))
  (bind _returnvalue (`GameplayStatics.GetCurrentLevelName` true))
  (if (not (`KismetStringLibrary.EqualEqual_StrStr` _returnvalue "in_casalpusterlengo"))
    (`/Engine/EditorBlueprintResources/StandardMacros.IncrementInt` _debuguses
      (:`  `
        (`self.Sleep`)
        (`KismetSystemLibrary.PrintString` (`KismetStringLibrary.Conv_IntToString` _debuguses))
        (if (> _debuguses 11)
          (message `/Game/EmPath/Interfaces/BI_GameActions.OpenLevel` (`GameplayStatics.GetPlayerPawn` 0) "in_casalpusterlengo" "0" false false))))))

(fn `UserConstructionScript`
  (`parent.UserConstructionScript`))