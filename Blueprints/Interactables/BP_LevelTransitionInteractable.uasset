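; BP_LevelTransitionInteractable is an interactable that moves the game to another named level and entrance.
; BeginPlay caches the EmPath game instance.
; OpenLevel shows a loading widget, waits briefly, saves under the target level name with the game instance's coordinates, then auto-loads that save at the configured entrance.
; Interact is empty here, and nothing in this graph calls OpenLevel.
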(event `self.ReceiveBeginPlay`
  (bind _asbp_em_path_game_instance (cast `/Game/MRPGT/Blueprints/GameInstance/BP_EmPathGameInstance` (`GameplayStatics.GetGameInstance`)))
  (set `self.GameInstance` _asbp_em_path_game_instance))

(event `OpenLevel`
  (bind _gameinstance (`self.GameInstance`))
  (bind _name (`self.Name`))
  (bind _returnvalue (`|CreateWidget` "/Game/EmPath/UI/W_Loading.W_Loading_C"))
  ;[1 1 1] Open level
  (`UserWidget.AddToViewport` _returnvalue 0)
  (`KismetSystemLibrary.Delay` 0.4)
  (bind _mapcoordinates (`/Game/MRPGT/Blueprints/GameInstance/BP_EmPathGameInstance.Get Coordinates` (`self.GameInstance`)))
  (`/Game/MRPGT/Blueprints/GameInstance/BP_EmPathGameInstance.SaveNewGame` :`self` _gameinstance :`LevelName` (`KismetStringLibrary.Conv_StringToName` _name) :`Coordinates` _mapcoordinates)
  (`/Game/MRPGT/Blueprints/GameInstance/BP_EmPathGameInstance.LoadSavedGame` _gameinstance "0" true (`self.Entrance`) _name))

(event `self.Interact`
  (params (HitComponent :type "ActorComponent Object Reference") (InteractingActor :type "Actor Object Reference") (AlternativeInteract :type Boolean)))

(fn `UserConstructionScript`
  (`parent.UserConstructionScript`))