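; BP_RitualCaveTent is an interactable tent for the ritual cave that lets the player sleep and changes the sky lighting.
; Its Interact event calls Sleep, which is not defined in this graph, then finds the first BP_HDRIBackdrop tagged Skybox.
; It swaps that backdrop's Skylight cubemap to a sunset texture, with no check that a backdrop was found.
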(event `/Game/MRPGT/Blueprints/Interfaces/Interface_Interactable.Interact`
  (params (HitComponent :type "ActorComponent Object Reference") (InteractingActor :type "Actor Object Reference") (AlternativeInteract :type Boolean))
  (`self.Sleep`)
  (bind _outactors (`GameplayStatics.GetAllActorsOfClassWithTag` "/Game/AutomotiveBridgeScene/Blueprints/BP_HDRIBackdrop.BP_HDRIBackdrop_C" "Skybox"))
  (`SkyLightComponent.SetCubemap` (`/Game/AutomotiveBridgeScene/Blueprints/BP_HDRIBackdrop.Skylight` (`|GetArrayItem` _outactors)) "/Game/HDRI/T_Indoor_MainHall_Sunset_CubeMap.T_Indoor_MainHall_Sunset_CubeMap"))

(fn `UserConstructionScript`
  (`parent.UserConstructionScript`))