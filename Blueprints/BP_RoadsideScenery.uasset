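; BP_RoadsideScenery is a scenery actor that stands in for roadside objects and slides along the world X axis.
; On BeginPlay it rolls a random float against Urbanization to pick a random static mesh from either the City or Wilderness list.
; Each tick it offsets its X position by Speed, without scaling by delta time.
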(event `self.ReceiveBeginPlay`
  (`StaticMeshComponent.SetStaticMesh` (`self.StaticMesh`) (select `bool` (<= (`KismetMathLibrary.RandomFloatInRange` 0.0 1.0) (`self.Urbanization`)) :`false` (`KismetArrayLibrary.Array_Random` (`self.Wilderness`)) :`true` (`KismetArrayLibrary.Array_Random` (`self.City`)))))

(event `self.ReceiveTick`
  (params (DeltaSeconds :type "Float (single-precision)"))
  (`self.K2_AddActorWorldOffset` (`KismetMathLibrary.MakeVector` (`self.Speed`))))

(fn `UserConstructionScript`)