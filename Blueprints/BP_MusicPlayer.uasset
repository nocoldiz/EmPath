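; BP_MusicPlayer is an interactable music source with a candle flame the player can light or blow out.
; On BeginPlay it looks up MusicName in DT_Music, caches the row, async-loads the track and plays it at the set volume.
; Both Lookingat and Interact toggle the flame and IsVisible, which picks the displayed action name.
; SetMusic pauses or resumes audio and GetMusic returns the cached row, while CycleMusic is empty.
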(event `self.ReceiveBeginPlay`
  (bind _audio (`self.Audio`))
  (bind _returnvalue (`|GetDataTableRow` "/Game/EmPath/DataTables/DT_Music.DT_Music" (`self.MusicName`))
    (:`then`
      (set `self.MusicInfo` _returnvalue)
      (bind (_name _author _lyrics _music) (break `/Game/EmPath/Structures/S_Music` _returnvalue))
      (`|LoadAsset` _music
        (:`Completed`
          (`AudioComponent.SetSound` _audio (`|ConvertAsset` _music))
          (set `AudioComponent.VolumeMultiplier` (`self.Volume`) (`self.Audio`))
          (`AudioComponent.Play` _audio 0.0))))))

(event `self.LookingAt`
  (params (HitComponent :type "ActorComponent Object Reference"))
  ;[1 1 1] E key will toggle light
  (`SceneComponent.ToggleVisibility` (`self.P_CandleFlame1`) false :!label _label)
  (set `self.Is Visible` (not (`self.Is Visible`))))

(event `self.Interact`
  (params (HitComponent :type "ActorComponent Object Reference") (InteractingActor :type "Actor Object Reference") (AlternativeInteract :type Boolean))
  ;[1 1 1] E key will toggle light
  (goto _label))

(event `/Game/EmPath/Interfaces/BI_MusicPlayer.SetMusic`
  (params (Disable :type Boolean))
  (bind _audio (`self.Audio`))
  ;[1 1 1] E key will toggle light
  (if Disable
    (`AudioComponent.SetPaused` _audio true)
    (else
      (`AudioComponent.SetPaused` _audio false))))

(event `/Game/EmPath/Interfaces/BI_MusicPlayer.CycleMusic`)

(fn `Get Music`
  (returns (Music :type "/Game/EmPath/Structures/S_Music Structure"))
  (return (`self.MusicInfo`)))

(fn `GetID`
  (returns (ID :type String))
  (return ""))

(fn `GetLauncherActor`
  (returns (LauncherActor :type "Actor Object Reference"))
  (return null))

(fn `GetObjectName`
  (returns (NameOut :type String))
  (if (`self.Is Visible`)
    (return "Blow Out Candle")
    (else
      (return "Light Candle"))))

(fn `IsProjectile`
  (returns (Result :type Boolean))
  (return false))

(fn `UserConstructionScript`)