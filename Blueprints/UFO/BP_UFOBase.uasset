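; BP_UFOBase is the base UFO actor, which pays the player a one-time Bounty as a photo sold online.
; BeginPlay caches the EmPath gameplay player controller.
; ApplyStatus, guarded by DoOnce, plays a cash sound, shows an Italian short message with the amount and adds the gold through that controller.
; The health, damage, team, attack and activity functions are stubs returning defaults.
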(event `self.ReceiveBeginPlay`
  (bind _asbp_em_path_game_player_controller (cast `/Game/MRPGT/Blueprints/Controllers/BP_EmPathGamePlayerController` (`GameplayStatics.GetPlayerController` 0)))
  (set `self.InGamePlayerController` _asbp_em_path_game_player_controller))

(event `/Game/EmPath/Interfaces/BPI_Damagable.ApplyStatus`
  (params (Status :type "/Game/EmPath/Enum/E_SpellEffect Enum" :default "NewEnumerator12") (Duration :type "Float (double-precision)") (Magnitude :type "Float (double-precision)") (Enable :type Boolean) (SuccessRate :type "Float (double-precision)") (HitBoneName :type Name))
  (bind _bounty (`self.Bounty`))
  (`/Engine/EditorBlueprintResources/StandardMacros.DoOnce` false
    (:`Completed`
      (`GameplayStatics.PlaySound2D` "/Game/EmPath/Sounds/Cash.Cash" 1.0 1.0 0.0 null null)
      (message `/Game/MRPGT/Blueprints/Interfaces/Interface_Messaging.SendShortMessage` (`GameplayStatics.GetPlayerController` 0) (`KismetTextLibrary.Conv_StringToText` (`KismetStringLibrary.Concat_StrStr` "Foto venduta online a " (`KismetStringLibrary.Conv_IntToString` _bounty) " €")))
      (`/Game/MRPGT/Blueprints/Controllers/BP_EmPathGamePlayerController.AddGoldToCharacterInfo` (`self.InGamePlayerController`) _bounty))))

(fn `ActivityTimeUpdate`
  (params (Time :type Integer))
  (returns (Activity :type "/Game/EmPath/Enum/E_NPCActivities Enum"))
  (return "NewEnumerator0"))

(fn `GetCurrentHealth`
  (returns (Health :type "Float (double-precision)"))
  (return 0.0))

(fn `GetMaxHealth`
  (returns (MaxHealth :type "Float (double-precision)"))
  (return 0.0))

(fn `GetNextActivity`
  (returns (Activity :type "/Game/EmPath/Enum/E_NPCActivities Enum") (Time :type Integer))
  (return "NewEnumerator0" 0))

(fn `GetTeamNumber`
  (returns (TeamNumber :type Integer))
  (return 0))

(fn `Heal`
  (params (Amount :type "Float (double-precision)"))
  (returns (NewHealth :type "Float (double-precision)"))
  (return 0.0))

(fn `IsAttacking`
  (returns (Attacking :type Boolean))
  (return false))

(fn `IsDead`
  (returns (Dead :type Boolean))
  (return false))

(fn `ReserveAttackToken`
  (params (Amount :type Integer))
  (returns (Success :type Boolean))
  (return false))

(fn `TakeDamage`
  (params (DamageInfo :type "/Game/EmPath/Structures/S_DamageInfo Structure") (`Damage Causer` :type "Actor Object Reference") (HitLocation :type "Vector Structure"))
  (returns (WasDamaged :type Boolean))
  (return false))

(fn `UserConstructionScript`)