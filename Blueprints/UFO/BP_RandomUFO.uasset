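; BP_RandomUFO is a spawner actor that places a randomly chosen UFO-type actor at its own transform.
; On BeginPlay, a random index selects one of fourteen Blueprint classes, mostly UFO variants, to spawn.
; A valid spawn snaps to the spawner's root and is destroyed after a fixed lifetime.
; The spawner then destroys itself after a short extra delay.
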(event `self.ReceiveBeginPlay`
  (bind _returnvalue (`|SpawnActorFromClass` (select `int` (`KismetMathLibrary.RandomIntegerInRange` 0 13) :`0` "/Game/EmPath/Blueprints/UFO/BP_SkullUfo.BP_SkullUfo_C" :`1` "/Game/EmPath/Blueprints/UFO/BP_PlasmaPUFO.BP_PlasmaPUFO_C" :`2` "/Game/EmPath/Blueprints/UFO/BP_CrossUFO.BP_CrossUFO_C" :`3` "/Game/EmPath/Blueprints/UFO/BP_TentacleUFo.BP_TentacleUFo_C" :`4` "/Game/NiagaraEffectMix5/Blueprints/BP_TentaclesMovementPoint.BP_TentaclesMovementPoint_C" :`5` "/Game/EmPath/Blueprints/UFO/BP_BlackTriangleORb.BP_BlackTriangleORb_C" :`6` "/Game/EmPath/Blueprints/UFO/BP_BrainUFO.BP_BrainUFO_C" :`7` "/Game/EmPath/Blueprints/UFO/BP_SmallTriangleUfo.BP_SmallTriangleUfo_C" :`8` "/Game/EmPath/Blueprints/UFO/BP_GriddlerUFO.BP_GriddlerUFO_C" :`9` "/Game/EmPath/Blueprints/UFO/BP_TicTacUFO.BP_TicTacUFO_C" :`10` "/Game/EmPath/Blueprints/UFO/BP_PyramidUFO.BP_PyramidUFO_C" :`11` "/Game/EmPath/Blueprints/UFO/BP_LensUFo.BP_LensUFo_C" :`12` "/Game/EmPath/Blueprints/UFO/BP_HolyUfo.BP_HolyUfo_C" :`13` "/Game/EmPath/Blueprints/UFO/BP_CubeUFO.BP_CubeUFO_C" :!type "Actor Class Reference") (`self.GetTransform`) "Undefined" "MultiplyWithRoot" null null))
  (`/Engine/EditorBlueprintResources/StandardMacros.IsValid` _returnvalue
    (:`Is Valid`
      (`self.K2_AttachToComponent` _returnvalue (`self.DefaultSceneRoot`) "None" "SnapToTarget" "SnapToTarget" "SnapToTarget" true)
      (`KismetSystemLibrary.Delay` 30.0)
      (`self.K2_DestroyActor` _returnvalue))
    (:`Is Not Valid`
      _))
  (`KismetSystemLibrary.Delay` 0.2)
  (`self.K2_DestroyActor`))

(fn `UserConstructionScript`)