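; Generic door Blueprint that automatically opens for enemy AI and responds to status effects.
; Box overlap opens it for BPI_EnemyAI actors; on exit it closes after a delay and locks if AutoLock is set.
; ApplyEffect maps statuses to opening, closing, or an explode that only hides the door mesh.
; Health, damage, team and activity functions are stubs returning defaults.
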(event `self.Box.OnComponentBeginOverlap`
  (params (OverlappedComponent :type "PrimitiveComponent Object Reference") (OtherActor :type "Actor Object Reference") (OtherComp :type "PrimitiveComponent Object Reference") (OtherBodyIndex :type Integer) (bFromSweep :type Boolean) (SweepResult :type "HitResult Structure (by ref)"))
  (if (and (`KismetSystemLibrary.DoesImplementInterface` OtherActor "/Game/EmPath/Interfaces/BPI_EnemyAI.BPI_EnemyAI_C") (not (`self.Open`)))
    (`self.OpenDoor`)))

(event `/Game/EmPath/Interfaces/BPI_Damagable.Apply Effect`
  (params (Status :type "/Game/EmPath/Enum/E_SpellEffect Enum" :default "NewEnumerator12") (Duration :type "Float (double-precision)") (Magnitude :type "Float (double-precision)") (Enable :type Boolean) (SuccessRate :type "Float (double-precision)") (HitBoneName :type Name))
  (switch `/Game/EmPath/Enum/E_SpellEffect` Status
    (:`NewEnumerator10`
      (`self.CloseDoor` false))
    (:`NewEnumerator27`
      (`SceneComponent.SetVisibility` (`self.Door`) false false))
    (:`NewEnumerator2`
      (`self.OpenDoor`)
      (`KismetSystemLibrary.PrintString` "Door"))))

(event `self.Box.OnComponentEndOverlap`
  (params (OverlappedComponent :type "PrimitiveComponent Object Reference") (OtherActor :type "Actor Object Reference") (OtherComp :type "PrimitiveComponent Object Reference") (OtherBodyIndex :type Integer))
  (if (`KismetSystemLibrary.DoesImplementInterface` OtherActor "/Game/EmPath/Interfaces/BPI_EnemyAI.BPI_EnemyAI_C")
    (`KismetSystemLibrary.Delay` 1.6)
    (`self.CloseDoor` false)
    (if (`self.AutoLock`)
      (`self.LockDoor`))))

(fn `ActivityTimeUpdate`
  (params (Time :type Integer))
  (returns (Activity :type "/Game/EmPath/Enum/E_NPCActivities Enum"))
  (return "NewEnumerator0"))

(fn `GetCurrentHealth`
  (returns (Health :type "Float (double-precision)"))
  (return 0.0))

(fn `GetMaxHealth`
  (returns (MaxHealth :type "Float (double-precision)"))
  (return 0.0))

(fn `GetNextActivity`
  (returns (Activity :type "/Game/EmPath/Enum/E_NPCActivities Enum") (Time :type Integer))
  (return "NewEnumerator0" 0))

(fn `GetTeamNumber`
  (returns (TeamNumber :type Integer))
  (return 0))

(fn `Heal`
  (params (Amount :type "Float (double-precision)"))
  (returns (NewHealth :type "Float (double-precision)"))
  (return 0.0))

(fn `IsAttacking`
  (returns (Attacking :type Boolean))
  (return false))

(fn `IsDead`
  (returns (Dead :type Boolean))
  (return false))

(fn `ReserveAttackToken`
  (params (Amount :type Integer))
  (returns (Success :type Boolean))
  (return false))

(fn `TakeDamage`
  (params (DamageInfo :type "/Game/EmPath/Structures/S_DamageInfo Structure") (`Damage Causer` :type "Actor Object Reference"))
  (returns (WasDamaged :type Boolean))
  (return false))

(fn `UserConstructionScript`
  (`parent.UserConstructionScript`))