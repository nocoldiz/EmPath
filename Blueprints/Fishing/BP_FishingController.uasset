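; Fishing bobber actor that floats after a splash and signals bites at random intervals.
; A Bobbing timeline offsets the mesh vertically, while a looping random delay of a few seconds triggers each bite.
; Each bite starts a Wobble roll timeline, plays a pitch-varied sound, shows the Niagara effect and calls SetCatchInterval on the FishingRod.
; The mesh rotation resets shortly afterwards and the wait restarts.
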(event `BobbingSequence`
  (bind (_direction _newtrack_0) (`Timeline|Bobbing`)
    (:`Update`
      (`SceneComponent.K2_AddLocalOffset` (`self.StaticMesh`) (`KismetMathLibrary.MakeVector` 0.0 0.0 (* _newtrack_0 0.2)) false false))))

(event `self.ReceiveBeginPlay`
  (`self.BobbingSequence`)
  (`GameplayStatics.PlaySoundAtLocation` "/Game/EmPath/Sounds/splash-by-blaukreuz-6261.splash-by-blaukreuz-6261" (`self.K2_GetActorLocation`) (struct) 1.0 1.0 0.0 null null null null)
  (`KismetSystemLibrary.Delay` 0.5)
  (`SceneComponent.SetVisibility` (`self.Niagara`) false false)
  (`KismetSystemLibrary.Delay` (`KismetMathLibrary.RandomFloatInRange` 1.5 6.0) :!label _label)
  (`|ExecutionSequence`
    (:`then_0`
      (bind _output_get (set `self.RandomRotator` (`KismetMathLibrary.RandomFloatInRange` 0.0 4.0)))
      (bind (_direction _newtrack_0) (`Timeline|Wobble`)
        (:`Update`
          (`SceneComponent.K2_AddLocalRotation` (`self.StaticMesh`) (`KismetMathLibrary.MakeRotator` (* _newtrack_0 2.0)) false false))))
    (:`then_1`
      (`GameplayStatics.PlaySound2D` "/Game/UltimateMagicUE/cues/Target_Hits/Target_Hit_-_Water__1__Cue.Target_Hit_-_Water__1__Cue" 0.4 (`KismetMathLibrary.RandomFloatInRange` 0.7 1.1) 0.0 null null)
      (`SceneComponent.SetVisibility` (`self.Niagara`) true false)
      (`/Game/EmPath/Blueprints/Weapons/BP_FishingRod.SetCatchInterval` (`self.FishingRod`))
      (`KismetSystemLibrary.Delay` 0.3)
      (`SceneComponent.K2_SetWorldRotation` :`self` (`self.StaticMesh`))
      (`SceneComponent.SetVisibility` (`self.Niagara`) true false)
      (goto _label))))

(fn `UserConstructionScript`)