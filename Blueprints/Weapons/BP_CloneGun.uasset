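; BP_CloneGun is a weapon Blueprint that overrides its parent's start and stop aiming events to give the player aim-down-sights behavior.
; Starting aim calls the parent, then sends messages to player pawn 0 to enable FPS aiming, set a zoomed FOV and lower mouse sensitivity; stopping reverses all three.
; StartAimingEvent calls its parent twice and holds an unconnected SetActive node.
; No cloning logic appears here.
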(fn `StartAimingEvent`
  (bind _returnvalue (`GameplayStatics.GetPlayerPawn` 0))
  (`parent.StartAimingEvent`)
  (`parent.StartAimingEvent`)
  (message `/Game/EmPath/Interfaces/BI_GameActions.SetFPSAiming` _returnvalue true)
  (message `/Game/EmPath/Interfaces/BI_GameActions.SetFOV` _returnvalue 40.0)
  (message `/Game/MRPGT/Blueprints/Interfaces/Interface_GeneralCharacter.LowerMouseSensitivity` _returnvalue 10.0))

(fn `StopAimingEvent`
  (bind _returnvalue (`GameplayStatics.GetPlayerPawn` 0))
  (`parent.StopAimingEvent`)
  (message `/Game/EmPath/Interfaces/BI_GameActions.SetFPSAiming` _returnvalue false)
  (message `/Game/EmPath/Interfaces/BI_GameActions.ResetFOV` _returnvalue)
  (message `/Game/MRPGT/Blueprints/Interfaces/Interface_GeneralCharacter.ResetMouseSensitivity` _returnvalue))

(fn `UserConstructionScript`
  (`parent.UserConstructionScript`))