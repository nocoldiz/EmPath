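; Sniper rifle weapon Blueprint that provides scoped aiming with stepped zoom.
; Starting aim shows WB_SniperHUD and hides the arms and status widget; stopping restores them and resets pawn FOV and mouse sensitivity.
; Zoom events step a clamped FOV, print it, and lower mouse sensitivity in tiers, all through messages to player pawn 0.
; The status widget is found during construction, and a RemoveWidget macro clears existing scope HUDs on each aim change.
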(event `/Game/EmPath/Interfaces/BI_Weapon.ZoomIn`
  (bind _fov (`self.FOV`))
  (set `self.FOV` (`KismetMathLibrary.FClamp` (+ (`self.FOV`) -5.0) (`self.MinZoom`) (`self.MaxZoom`)))
  (message `/Game/EmPath/Interfaces/BI_GameActions.SetFOV` (`GameplayStatics.GetPlayerPawn` 0) (`self.FOV`) :!label _label)
  (`KismetSystemLibrary.PrintString` (`KismetStringLibrary.Conv_DoubleToString` _fov))
  (if (<= _fov 15.0)
    (if (<= (`self.FOV`) 5.0)
      (`self.UpdateMouseSensitivity` 50.0)
      (else
        (`self.UpdateMouseSensitivity` 14.0)))
    (else
      (`self.UpdateMouseSensitivity` 7.0))))

(event `/Game/EmPath/Interfaces/BI_Weapon.ZoomOut`
  (set `self.FOV` (`KismetMathLibrary.FClamp` (- (`self.FOV`) -5.0) (`self.MinZoom`) (`self.MaxZoom`)))
  (goto _label))

(fn `StartAimingEvent`
  (`self.RemoveWidget`
    (:`Completed`
      (bind _returnvalue (`|CreateWidget` "/Game/EmPath/UI/WB_SniperHUD.WB_SniperHUD_C"))
      (`UserWidget.AddToViewport` _returnvalue 0)
      (set `self.CameraHUDWidget` _returnvalue)
      (`SceneComponent.SetVisibility` (`self.Arms`) false true)
      (message `/Game/EmPath/Interfaces/BI_GameActions.SetFPSAiming` (`GameplayStatics.GetPlayerPawn` 0) true)
      (set `self.IsAiming` true)
      (`Widget.SetVisibility` (`self.StatusWidget`) "Hidden")
      (`self.UpdateMouseSensitivity` 5.0))))

(fn `StopAimingEvent`
  (bind _returnvalue (`GameplayStatics.GetPlayerPawn` 0))
  (`self.RemoveWidget`
    (:`Completed`
      (`SceneComponent.SetVisibility` (`self.Arms`) true true)
      (`Widget.SetVisibility` (`self.StatusWidget`) "Visible")
      (message `/Game/EmPath/Interfaces/BI_GameActions.ResetFOV` _returnvalue)
      (message `/Game/MRPGT/Blueprints/Interfaces/Interface_GeneralCharacter.ResetMouseSensitivity` (`GameplayStatics.GetPlayerPawn` 0))
      (message `/Game/EmPath/Interfaces/BI_GameActions.SetFPSAiming` _returnvalue false)
      (set `self.IsAiming` false))))

(fn `UpdateMouseSensitivity`
  (params (B :type "Float (double-precision)"))
  (bind _returnvalue (`GameplayStatics.GetPlayerPawn` 0))
  (message `/Game/EmPath/Interfaces/BI_GameActions.SetFOV` _returnvalue (`self.FOV`))
  (message `/Game/MRPGT/Blueprints/Interfaces/Interface_GeneralCharacter.LowerMouseSensitivity` _returnvalue B))

(fn `UserConstructionScript`
  (`parent.UserConstructionScript`)
  (bind _foundwidgets (`WidgetBlueprintLibrary.GetAllWidgetsOfClass` "/Game/MRPGT/UserInterface/WidgetBlueprints/CharacterStatusWidget.CharacterStatusWidget_C" false))
  (set `self.StatusWidget` (`|GetArrayItem` _foundwidgets)))