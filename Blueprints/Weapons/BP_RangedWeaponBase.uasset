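; Base Blueprint for ranged weapons, providing shared shoot and reload behavior plus empty hooks for aiming, shooting, reloading and showing the HUD.
; Shoot and Reload animate the weapon mesh and call their hooks; Shoot also attaches the GunInfo muzzle effect at MuzzleFlash.
; That soft-referenced effect is loaded synchronously in construction and on every shot.
; HideHUD removes the widget; other input events are empty, and the arm-montage logic is disconnected.
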(event `/Game/EmPath/Interfaces/BI_Weapon.Sheathe`)

(event `self.ReceiveBeginPlay`)

(event `/Game/EmPath/Interfaces/BI_Weapon.Unsheathe`)

(event `Move_1`)

(event `/Game/EmPath/Interfaces/BI_Weapon.ChangeMode`)

(event `/Game/EmPath/Interfaces/BI_Weapon.Jump`)

(event `/Game/EmPath/Interfaces/BI_Weapon.Shoot`
  (bind (_name _weaponclass _comboname _automatic _damage _totalammo _clipammo _firerate _reloadspeed _spread _range _firesound _changemodesound _reloadsound _muzzlefx) (break `/Game/EmPath/Structures/S_RangedWeapon` (`self.GunInfo`)))
  (`|ExecutionSequence`
    (:`then_0`
      (`SkeletalMeshComponent.PlayAnimation` (`self.Weapon`) (`self.ShootMontageWeapon`) false)
      (`self.ShootEvent`)
      (`KismetSystemLibrary.LoadAsset_Blocking` _muzzlefx)
      (`NiagaraFunctionLibrary.SpawnSystemAttached` (`|ConvertAsset` _muzzlefx) (`self.MuzzleFlash`) "None" (0.0 0.0 0.0) (struct) "KeepRelativeOffset"))))

(event `/Game/EmPath/Interfaces/BI_Weapon.Reload`
  (`SkeletalMeshComponent.PlayAnimation` (`self.Weapon`) (`self.ReloadMontageWeapon`) false)
  (`self.ReloadEvent`))

(fn `HideHUD`
  (bind _hudwidget (`self.HudWidget`))
  (`/Engine/EditorBlueprintResources/StandardMacros.IsValid` _hudwidget
    (:`Is Valid`
      (`Widget.RemoveFromParent` _hudwidget))))

(fn `ReloadEvent`)

(fn `ShootEvent`)

(fn `ShowHUD`)

(fn `StartAimingEvent`)

(fn `StopAimingEvent`)

(fn `UserConstructionScript`
  (bind (_name _weaponclass _comboname _automatic _damage _totalammo _clipammo _firerate _reloadspeed _spread _range _firesound _changemodesound _reloadsound _muzzlefx) (break `/Game/EmPath/Structures/S_RangedWeapon` (`self.GunInfo`)))
  (`KismetSystemLibrary.LoadAsset_Blocking` _muzzlefx)
  (set `self.MuzzleFash` (`|ConvertAsset` _muzzlefx)))