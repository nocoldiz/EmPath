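; BP_FPSWeapon is a first-person weapon Blueprint that plays the weapon mesh's shoot and reload animations.
; Shoot and Reload play non-looping animations directly on the Weapon component, while sheathe, unsheathe, movement, jump and mode events are empty.
; The construction script synchronously loads the muzzle effect into a variable that the graph never uses.
; Disconnected nodes retain arm montage logic for shooting and idle, including an EndAttack notify.
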(event `/Game/EmPath/Interfaces/BI_Weapon.Sheathe`)

(event `self.ReceiveBeginPlay`)

(event `/Game/EmPath/Interfaces/BI_Weapon.Unsheathe`)

(event `Move_1`)

(event `/Game/EmPath/Interfaces/BI_Weapon.ChangeMode`)

(event `/Game/EmPath/Interfaces/BI_Weapon.Jump`)

(event `/Game/EmPath/Interfaces/BI_Weapon.Shoot`
  (`|ExecutionSequence`
    (:`then_0`
      (`SkeletalMeshComponent.PlayAnimation` (`self.Weapon`) (`self.ShootMontageWeapon`) false))))

(event `/Game/EmPath/Interfaces/BI_Weapon.Reload`
  (`SkeletalMeshComponent.PlayAnimation` (`self.Weapon`) (`self.ReloadMontageWeapon`) false))

(fn `UserConstructionScript`
  (bind _muzzlefx (break ``))
  (`KismetSystemLibrary.LoadAsset_Blocking` _muzzlefx)
  (set `self.MuzzleFash` (`|ConvertAsset` _muzzlefx)))