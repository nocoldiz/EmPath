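; BP_FishingRod is a fishing rod weapon whose Shoot event toggles fishing on and off.
; Casting runs a line trace from the player pawn's active camera and accepts a water PhysicsVolume or a non-volume actor tagged "Water".
; A water hit spawns a BP_FishingController at the hit point, with debug trace drawing and a location printout.
; Shooting again while fishing destroys that controller.
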(event `/Game/EmPath/Interfaces/BI_Weapon.Shoot`
  (if (`self.IsFishing`)
    (`self.K2_DestroyActor` (`self.FishingController`))
    (set `self.FishingController` null)
    (set `self.IsFishing` false)
    (else
      (bind _hitresult (message `/Game/EmPath/Interfaces/BI_GameActions.LineTraceFromActiveCamera` (`GameplayStatics.GetPlayerPawn` 0) 8000.0 "ForDuration"))
      (bind (_bblockinghit _binitialoverlap _time _distance _location _impactpoint _normal _impactnormal _physmat _hitactor) (`GameplayStatics.BreakHitResult` _hitresult))
      (`/Engine/EditorBlueprintResources/StandardMacros.IsValid` _hitactor
        (:`Is Valid`
          (bind _asphysics_volume (cast `PhysicsVolume` _hitactor)
            (:`then`
              (if (`PhysicsVolume.bWaterVolume` _asphysics_volume)
                (`KismetSystemLibrary.PrintString` (`KismetStringLibrary.Conv_VectorToString` _location) :!label _label)
                (set `self.IsFishing` true)
                (bind _returnvalue (`|SpawnActorFromClass` "/Game/EmPath/Blueprints/Fishing/BP_FishingController.BP_FishingController_C" (`KismetMathLibrary.Conv_VectorToTransform` _location) "Undefined" "MultiplyWithRoot" null null))
                (set `self.FishingController` _returnvalue)))
            (:`CastFailed`
              (if (!= (`KismetArrayLibrary.Array_Find` (`Actor.Tags` _hitactor) "Water") -1)
                (goto _label)))))))))

(fn `UserConstructionScript`
  (`parent.UserConstructionScript`))