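; BP_Telegun is a weapon that teleports the player pawn to where the active camera is aimed.
; Shoot requests a long-range line trace from the player pawn via a message call, then teleports that pawn to the returned location with zero rotation, without checking for a hit.
; The weapon's material changes during the shot and switches back after a short delay.
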(event `/Game/EmPath/Interfaces/BI_Weapon.Shoot`
  (bind _returnvalue (`GameplayStatics.GetPlayerPawn` 0))
  (`PrimitiveComponent.SetMaterial` (`self.Weapon`) 0 "/Game/Sicka_EnvPack2/Sicka_Scifi_Interior2/Materials/MI_Props1_Triangle.MI_Props1_Triangle")
  (bind _hitresult (message `/Game/EmPath/Interfaces/BI_GameActions.LineTraceFromActiveCamera` _returnvalue 99999.0 "None"))
  (`self.K2_TeleportTo` :`self` _returnvalue :`DestLocation` (`.Location` (`GameplayStatics.BreakHitResult` _hitresult)))
  (`KismetSystemLibrary.Delay` 0.5)
  (`PrimitiveComponent.SetMaterial` (`self.Weapon`) 0 "/Game/Sicka_EnvPack2/Sicka_Scifi_Interior2/Materials/MI_Props1_Starbase.MI_Props1_Starbase"))

(fn `UserConstructionScript`
  (`parent.UserConstructionScript`))