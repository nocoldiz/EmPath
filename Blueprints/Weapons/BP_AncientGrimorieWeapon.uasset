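; Ancient grimoire weapon that casts spells and launches the player through messages sent to the player pawn.
; The book plays an opening animation on BeginPlay, and each shot turns a page and tells the pawn to cast the grimoire spell.
; Starting to aim acts as a secondary ability, playing an air spell sound and launching the pawn using camera direction with Z override.
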(event `/Game/EmPath/Interfaces/BI_Weapon.Shoot`
  (`SkeletalMeshComponent.PlayAnimation` (`self.Weapon`) "/Game/OldAnimatedBooks/Animations/Book_Lying_Open_Page_Turn_L_to_R_01.Book_Lying_Open_Page_Turn_L_to_R_01" false)
  (message `/Game/EmPath/Interfaces/BI_GameActions.CastGrimorieSpell` (`GameplayStatics.GetPlayerPawn` 0)))

(event `self.ReceiveBeginPlay`
  (`SkeletalMeshComponent.PlayAnimation` (`self.Weapon`) "/Game/OldAnimatedBooks/Animations/Book_Lying_C_to_Open_01.Book_Lying_C_to_Open_01" false))

(fn `StartAimingEvent`
  (`GameplayStatics.PlaySoundAtLocation` "/Game/UltimateMagicUE/cues/Spell_Shoot/Air_Spell_-_Shoot_9_Cue.Air_Spell_-_Shoot_9_Cue" (`self.K2_GetActorLocation`) (struct) 0.4 1.0 0.0 null "/Game/EmPath/Music/SC_SpellConcurrency.SC_SpellConcurrency" null null)
  (message `/Game/EmPath/Interfaces/BPI_Damagable.Launch` (`GameplayStatics.GetPlayerPawn` 0) (0.0 0.0 1000.0) 10.0 false true true false false))

(fn `UserConstructionScript`
  (`parent.UserConstructionScript`))