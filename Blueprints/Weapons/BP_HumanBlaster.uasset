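; BP_HumanBlaster is a weapon Blueprint that animates a spinning mesh part in response to firing.
; Shoot sets a cooldown flag, then clears it after a retriggerable delay, so repeated shots extend the window.
; Tick rotates StaticMesh1 every frame, faster while the flag is set, without scaling by delta time.
; No projectile or damage logic appears in this graph.
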(event `self.ReceiveTick`
  (params (DeltaSeconds :type "Float (single-precision)"))
  (`parent.ReceiveTick` DeltaSeconds)
  (`SceneComponent.K2_AddLocalRotation` (`self.StaticMesh1`) (`KismetMathLibrary.SelectRotator` (struct :`Yaw` 10.0) (struct :`Yaw` 1.0) (`self.ShootCooldown`)) false false))

(event `/Game/EmPath/Interfaces/BI_Weapon.Shoot`
  (set `self.ShootCooldown` true)
  (`KismetSystemLibrary.RetriggerableDelay` 1.0)
  (set `self.ShootCooldown` false))

(fn `UserConstructionScript`
  (`parent.UserConstructionScript`))