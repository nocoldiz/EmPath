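; Broomstick weapon that gives the player vertical lift and hovering instead of firing a projectile.
; Shoot sends the player pawn an upward launch message, while aiming zeroes its gravity scale and starts a looping one-second timer.
; Stopping aim clears the timer and resets gravity.
; BeginPlay plays a one-shot book-opening animation on the Weapon component.
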(event `self.Shoot`
  (message `/Game/EmPath/Interfaces/BPI_Damagable.Launch` (`GameplayStatics.GetPlayerPawn` 0) (0.0 0.0 100.0) 10.0 false false false false false))

(event `self.ReceiveBeginPlay`
  (`SkeletalMeshComponent.PlayAnimation` (`self.Weapon`) "/Game/OldAnimatedBooks/Animations/Book_Lying_C_to_Open_01.Book_Lying_C_to_Open_01" false))

(fn `BP_Broomstick_AutoGenFunc`
  (message `/Game/EmPath/Interfaces/BI_GameActions.SetGravityScale` (`GameplayStatics.GetPlayerPawn` 0) 0.0))

(fn `StartAimingEvent`
  (bind _returnvalue (`KismetSystemLibrary.K2_SetTimerDelegate` (`|CreateDelegate` :!event `BP_Broomstick_AutoGenFunc`) 1.0 true))
  (set `self.GravityTimerHandle` _returnvalue)
  (message `/Game/EmPath/Interfaces/BI_GameActions.SetGravityScale` (`GameplayStatics.GetPlayerPawn` 0) 0.0))

(event `SetScaleEvent`)

(fn `StopAimingEvent`
  (`KismetSystemLibrary.K2_ClearAndInvalidateTimerHandle` (`self.GravityTimerHandle`))
  (message `/Game/EmPath/Interfaces/BI_GameActions.ResetGravityScale` (`GameplayStatics.GetPlayerPawn` 0) 0.0))

(fn `UserConstructionScript`
  (`parent.UserConstructionScript`))