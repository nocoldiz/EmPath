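; Interaction point attached to a bike actor that lets the player either take the bike or ride it.
; Alternative interact sends the parent pawn to the player through a driving-mode message and clears IsVisible, which ChangeState sets again.
; Normal interact destroys the parent and adds "Bike" to the player's backpack.
; The prompt reads Take/Ride regardless of IsVisible; other interface functions are stubs.
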(event `self.LookingAt`
  (params (HitComponent :type "ActorComponent Object Reference"))
  ;[1 1 1] E key will toggle light
)

(event `self.Interact`
  (params (HitComponent :type "ActorComponent Object Reference") (InteractingActor :type "Actor Object Reference") (AlternativeInteract :type Boolean))
  (bind _returnvalue (`self.GetParentActor`))
  ;[1 1 1] E key will toggle light
  (if AlternativeInteract
    (bind _aspawn (cast `Pawn` _returnvalue))
    (message `/Game/EmPath/Interfaces/BI_GameActions.SetDrivingMode` (`GameplayStatics.GetPlayerPawn` 0) "NewEnumerator6" (struct) _aspawn)
    (set `self.Is Visible` false)
    (else
      (`self.K2_DestroyActor` _returnvalue)
      (message `/Game/EmPath/Interfaces/BI_GameActions.AddItemToBackpack` (`GameplayStatics.GetPlayerPawn` 0) "Bike"))))

(event `self.ChangeState`
  ;[1 1 1] E key will toggle light
  (set `self.Is Visible` true))

(fn `GetID`
  (returns (ID :type String))
  (return ""))

(fn `GetLauncherActor`
  (returns (LauncherActor :type "Actor Object Reference"))
  (return null))

(fn `GetObjectName`
  (returns (NameOut :type String))
  (bind _returnvalue (`KismetStringLibrary.Concat_StrStr` (`self.PrimaryButton`) "" "Take" " / " (`self.SecondaryButton`) " " "Ride"))
  (if (`self.Is Visible`)
    (return _returnvalue)
    (else
      (return _returnvalue))))

(fn `IsProjectile`
  (returns (Result :type Boolean))
  (return false))

(fn `SetVisible`)

(fn `UserConstructionScript`
  (bind _returnvalue (`GameplayStatics.GetCurrentLevelName` true))
  (set `self.LevelName` _returnvalue))