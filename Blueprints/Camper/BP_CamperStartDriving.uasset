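; BP_CamperStartDriving is the camper's interactable for starting driving, offering a "Start driving" prompt everywhere except the TheRoad level.
; Interact sends a driving mode message to the player pawn and clears IsVisible, which blanks the prompt until ChangeState sets it again.
; The construction script caches the level name for the prompt, while Interact re-checks it; the other interface functions are empty stubs.
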(event `self.LookingAt`
  (params (HitComponent :type "ActorComponent Object Reference"))
  ;[1 1 1] E key will toggle light
)

(event `self.Interact`
  (params (HitComponent :type "ActorComponent Object Reference") (InteractingActor :type "Actor Object Reference") (AlternativeInteract :type Boolean))
  ;[1 1 1] E key will toggle light
  (bind _returnvalue (`GameplayStatics.GetCurrentLevelName` true))
  (if (not (`KismetStringLibrary.EqualEqual_StrStr` _returnvalue "TheRoad"))
    (message `/Game/EmPath/Interfaces/BI_GameActions.SetDrivingMode` (`GameplayStatics.GetPlayerPawn` 0) "NewEnumerator6" (struct))
    (set `self.Is Visible` false)))

(event `/Game/MRPGT/Blueprints/Interfaces/Interface_Interactable.ChangeState`
  (set `self.Is Visible` true))

(fn `GetID`
  (returns (ID :type String))
  (return ""))

(fn `GetLauncherActor`
  (returns (LauncherActor :type "Actor Object Reference"))
  (return null))

(fn `GetObjectName`
  (returns (NameOut :type String))
  (if (`self.Is Visible`)
    (return (`KismetMathLibrary.SelectString` "" "Start driving" (`KismetStringLibrary.EqualEqual_StrStr` (`self.LevelName`) "TheRoad")))
    (else
      (return ""))))

(fn `IsProjectile`
  (returns (Result :type Boolean))
  (return false))

(fn `SetVisible`)

(fn `UserConstructionScript`
  (bind _returnvalue (`GameplayStatics.GetCurrentLevelName` true))
  (set `self.LevelName` _returnvalue))