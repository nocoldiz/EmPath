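; Camper passenger seat interactable that seats the player pawn on Use, using its capsule as center and arrow as entrance.
; If the pawn's driving mode is Walking, it advances CamperController to its next state, or prints a warning when no destination is selected.
; Separate Open/Close events drive a button timeline with selectable easing, mesh swaps and 3D sounds, triggering linked actors and horror events immediately or after animation.
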(event `Seat`
  (bind _returnvalue (`GameplayStatics.GetPlayerPawn` 0))
  ;[1 1 1] Seat
  (message `/Game/EmPath/Interfaces/BI_GameActions.StartSeating` _returnvalue (`SceneComponent.K2_GetComponentLocation` (`self.Capsule`)) (`SceneComponent.K2_GetComponentLocation` (`self.Arrow`)) null false (0.0 0.0 0.0) null false)
  (bind _drivingmode (message `/Game/EmPath/Interfaces/BI_GameActions.GetDrivingMode` _returnvalue))
  (switch `/Game/EmPath/Enum/E_DrivingMode` _drivingmode
    (:`NewEnumerator1`
      (bind _destination (message `/Game/EmPath/Interfaces/BI_GameActions.NextDestination` _returnvalue))
      ;[1 1 1] Departure Fx
      (if (`KismetStringLibrary.IsEmpty` _destination)
        (`KismetSystemLibrary.PrintString` "No destination selected")
        (else
          (message `/Game/EmPath/Interfaces/BI_GameActions.NextState` (`self.CamperController`)))))))

(event `TalkEvent`
  (params (HorrorEvent :type Boolean)))

(event `self.Use`
  (params (HorrorEvent :type Boolean))
  ;[1 1 1] Interact Settings
  (`/Game/HorrorEngine/Blueprints/Core/HorrorEngineMacros.HM_CheckInteraction`)
  (`self.Seat`))

(event `self.Open/On`
  (params (HorrorEvent :type Boolean))
  (bind _transformtype (`self.TransformType`))
  (bind _actorstouse (`self.ActorsToUse`))
  (bind _returnvalue (or (`|EnumEquality` _transformtype "NewEnumerator0") (`|EnumEquality` _transformtype "NewEnumerator4")))
  ;[1 1 1] Open / Close Settings
  (`/Game/HorrorEngine/Blueprints/Core/HorrorEngineMacros.HM_CheckInteraction`)
  (if (not (`self.On / Off`))
    (if (not (`self.UseAfterAnimation`))
      (set `self.On / Off` true)
      (`self.Open/On` (`self.ActorsToUse`) false)
      (`self.HorrorEventCheck` "NewEnumerator3"))
    (set `self.InteractionEnabled` false)
    (bind (_direction _direct _direct__easy_ease_ _elastic _elastic__easy_ease_ _flip_flop _flip_flop__easy_ease_) (`Timeline|ButtonTimeline` :!via `PlayFromStart` :!label _label)
      (:`Update`
        (bind _returnvalue_2 (select `/Game/HorrorEngine/Blueprints/Enums/TransfromType` (`self.TransformType`) :`NewEnumerator0` _direct :`NewEnumerator4` _direct__easy_ease_ :`NewEnumerator5` _elastic :`NewEnumerator8` _elastic__easy_ease_ :`NewEnumerator9` _flip_flop :`NewEnumerator13` _flip_flop__easy_ease_ :!type "Float (double-precision)"))
        (`SceneComponent.K2_SetRelativeLocationAndRotation` (`self.ButtonPivot`) (`KismetMathLibrary.VLerp` (`self.OffLocation`) (`self.OnLocation`) _returnvalue_2) (`KismetMathLibrary.RLerp` (`self.OffRotation`) (`self.OnRotation`) _returnvalue_2) false false))
      (:`Finished`
        (switch `ETimelineDirection` _direction
          (:`Forward`
            (`/Game/HorrorEngine/Blueprints/Core/HorrorEngineFunctions.SetMesh` (`self.Button`) (`self.ButtonOnMesh`))
            (if (`self.UseAfterAnimation`)
              (set `self.On / Off` true)
              (`self.Open/On` _actorstouse false)
              (`self.HorrorEventCheck` "NewEnumerator3")))
          (:`Backward`
            (`/Game/HorrorEngine/Blueprints/Core/HorrorEngineFunctions.SetMesh` (`self.Button`) (`self.ButtonOffMesh`))
            (if (`self.UseAfterAnimation`)
              (set `self.On / Off` false)
              (`self.Close/Off` _actorstouse false)
              (`self.HorrorEventCheck` "NewEnumerator4"))))
        (set `self.InteractionEnabled` true)
        (if (`self.StopSoundsAfterAnimation`)
          (`/Game/HorrorEngine/Blueprints/Core/HorrorEngineMacros.HM_StopAll3DSounds`)))
      (:`ButtonStartSound`
        (if _returnvalue
          (switch `ETimelineDirection` _direction
            (:`Forward`
              _)))
        (`/Game/HorrorEngine/Blueprints/Core/HorrorEngineMacros.HM_3DSound` null false (`self.TurnOnSound`) (`self.ButtonPivot`) (`self.SoundAttenuation`)))
      (:`ButtonEndSound`
        (if _returnvalue
          (switch `ETimelineDirection` _direction
            (:`Backward`
              _)))
        (`/Game/HorrorEngine/Blueprints/Core/HorrorEngineMacros.HM_3DSound` null false (`self.TurnOffSound`) (`self.ButtonPivot`) (`self.SoundAttenuation`))))))

(event `self.Close/Off`
  (params (HorrorEvent :type Boolean))
  ;[1 1 1] Open / Close Settings
  (`/Game/HorrorEngine/Blueprints/Core/HorrorEngineMacros.HM_CheckInteraction`)
  (if (`self.On / Off`)
    (if (not (`self.UseAfterAnimation`))
      (set `self.On / Off` false)
      (`self.Close/Off` (`self.ActorsToUse`) false)
      (`self.HorrorEventCheck` "NewEnumerator4"))
    (set `self.InteractionEnabled` false)
    (goto _label :!via `ReverseFromEnd`)))

(event `/Game/HorrorEngine/Blueprints/Core/HorrorEngineInterface.RestoreSaveData`
  (params (AssetSave :type "/Game/HorrorEngine/Blueprints/Structures/SaveStructures/AssetsSave Structure")))

(event `/Game/HorrorEngine/Blueprints/Core/HorrorEngineInterface.CollectSaveData`)

(fn `UserConstructionScript`
  (bind _offrotation (`self.OffRotation`))
  (bind _offlocation (`self.OffLocation`))
  (bind _transformtype (`self.TransformType`))
  (bind _returnvalue (or (`|EnumEquality` _transformtype "NewEnumerator9") (`|EnumEquality` _transformtype "NewEnumerator13")))
  (`/Game/HorrorEngine/Blueprints/Core/HorrorEngineMacros.HM_DefaultConstructions` (`self.CreateNewHorrorEvent`))
  (`/Game/HorrorEngine/Blueprints/Core/HorrorEngineFunctions.SetMesh` (`self.Interact`) (`self.ButtonBaseMesh`))
  (`/Game/HorrorEngine/Blueprints/Core/HorrorEngineFunctions.SetMesh` (`self.Button`) (select `bool` (`self.On / Off`) :`false` (`self.ButtonOffMesh`) :`true` (`self.ButtonOnMesh`)))
  (`/Game/HorrorEngine/Blueprints/Core/HorrorEngineFunctions.PlayRate` (`self.ButtonTimeline`) (`self.Animation Speed (Sec)`))
  (`SceneComponent.K2_SetRelativeLocationAndRotation` (`self.ButtonPivot`) (select `bool` _returnvalue :`false` (select `bool` (`self.On / Off`) :`false` _offlocation :`true` (`self.OnLocation`)) :`true` _offlocation) (select `bool` _returnvalue :`false` (select `bool` (`self.On / Off`) :`false` _offrotation :`true` (`self.OnRotation`)) :`true` _offrotation) false false))