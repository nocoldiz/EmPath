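; Interactable camper pillow that plays a sleep sequence when used.
; Use is guarded by IsSleeping, disables player input, fades the camera out through pawn messages, then branches on driving mode.
; Map mode runs horror interaction and event checks and advances the CamperController state; other modes just wait before fading back in.
; FadeIn clears the guard; Sleep is an unfinished stub, and input is not re-enabled here.
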(event `self.ReceiveBeginPlay`)

(event `self.Use`
  (params (HorrorEvent :type Boolean) (UseFromBackpack :type Boolean))
  (if (not (`self.IsSleeping`))
    ;[1 1 1] Interact Settings
    (set `self.IsSleeping` true)
    (`self.DisableInput` (`GameplayStatics.GetPlayerController` 0) null)
    (bind _drivingmode (message `/Game/EmPath/Interfaces/BI_GameActions.GetDrivingMode` (`GameplayStatics.GetPlayerPawn` 0)))
    (`self.FadeOut`)
    (`KismetSystemLibrary.Delay` 2.0)
    (switch `/Game/EmPath/Enum/E_DrivingMode` _drivingmode
      (:`NewEnumerator0`
        (`/Game/HorrorEngine/Blueprints/Core/HorrorEngineMacros.HM_CheckInteraction`)
        (`/Game/EmPath/Blueprints/Camper/B_CamperController.NextState` (`self.CamperController`))
        (`self.HorrorEventCheck` "NewEnumerator54")
        (`self.FadeIn`))
      (:`NewEnumerator1`
        ;[1 1 1] Go to sleep
        (`KismetSystemLibrary.Delay` 1.0 :!label _label)
        (`self.CameraFadeStop`)
        (`KismetSystemLibrary.PrintString` "fedein")
        (`self.FadeIn`))
      (:`NewEnumerator2`
        (goto _label))
      (:`NewEnumerator3`
        (goto _label))
      (:`NewEnumerator4`
        (goto _label)))))

(fn `AddSin`
  (params (SinName :type String)))

(fn `CameraFadeStop`
  (message `/Game/EmPath/Interfaces/BI_GameActions.Camera Fade Stop` (`GameplayStatics.GetPlayerPawn` 0)))

(fn `CurrentDestination`
  (returns (Destination :type String))
  (return ""))

(fn `FadeIn`
  (message `/Game/EmPath/Interfaces/BI_GameActions.Camera Fade In` (`GameplayStatics.GetPlayerPawn` 0))
  (set `self.IsSleeping` false))

(fn `FadeOut`
  (message `/Game/EmPath/Interfaces/BI_GameActions.Camera Fade Out` (`GameplayStatics.GetPlayerPawn` 0)))

(fn `GetActiveActor`
  (returns (Actor :type "Actor Object Reference"))
  (return null))

(fn `GetActorLocation`
  (returns (Location :type "Vector Structure"))
  (return (0.0 0.0 0.0)))

(fn `GetBackpackIndex`
  (returns (Index :type Integer))
  (return 0))

(fn `GetCurrentMP`
  (returns (Mp :type "Float (double-precision)"))
  (return 0.0))

(fn `GetCurrentSpells`
  (params (Custom :type Boolean))
  (returns (Spells :type "Array of /Game/EmPath/Structures/Spell/S_Spell Structure"))
  (return))

(fn `GetDialogTopicIndex`
  (returns (Index :type Integer))
  (return 0))

(fn `GetDrivingMode`
  (returns (DrivingMode :type "/Game/EmPath/Enum/E_DrivingMode Enum"))
  (return "NewEnumerator0"))

(fn `GetIsSitting`
  (returns (IsSitting :type Boolean))
  (return false))

(fn `GetIsTalking`
  (returns (DialogState :type "/Game/EmPath/Enum/E_DialogState Enum"))
  (return "NewEnumerator0"))

(fn `GetKnownSpells`
  (returns (Spells :type "Array of Name"))
  (return))

(fn `GetLearnedTopics`
  (returns (Topics :type "Array of String"))
  (return))

(fn `GetMapTile`
  (returns (MapTile :type "Vector2D Structure"))
  (return (0.0 0.0)))

(fn `GetMoney`
  (returns (Money :type "Float (double-precision)"))
  (return 0.0))

(fn `GetOpenedChests`
  (returns (NewParam :type "Array of String"))
  (return))

(fn `GetSelectedSpell`
  (params (IsCustomSpell :type Boolean) (IsPistolSpell :type Boolean))
  (returns (SpellInfo :type "/Game/EmPath/Structures/Spell/S_Spell Structure"))
  (return))

(fn `GetSpawnReaction`
  (returns (Spawned :type Boolean))
  (return false))

(fn `GetSpellbookPage`
  (returns (SpellInfo :type "/Game/EmPath/Structures/Spell/S_Spell Structure") (MagicInfo :type "/Game/EmPath/Structures/S_MagicSchools Structure") (GlossaryInfo :type "/Game/EmPath/Structures/S_Glossary Structure") (LastPage :type "/Game/EmPath/Enum/E_PageTypes Enum"))
  (return (struct) (struct) (struct) "NewEnumerator0"))

(fn `GetSpellCollision`
  (returns (IsColliding :type Boolean))
  (return false))

(fn `GetStance`
  (returns (Stance :type "/Game/EmPath/Enum/E_PlayerStances Enum"))
  (return "NewEnumerator0"))

(fn `GetVehicle`
  (returns (Vehicle :type "Actor Object Reference"))
  (return null))

(fn `GetVisibility`
  (returns (Visibility :type "/Game/EmPath/Enum/E_PlayerVisibility Enum"))
  (return "NewEnumerator0"))

(fn `NextDestination`
  (returns (Destination :type String))
  (return ""))

(fn `SetCurrentDestination`
  (returns (Destination :type String))
  (return ""))

(fn `Sleep`
  (`KismetSystemLibrary.PrintString` "Sleep")
  (bind _drivingmode (message `/Game/EmPath/Interfaces/BI_GameActions.GetDrivingMode` (`GameplayStatics.GetPlayerPawn` 0)))
  (switch `/Game/EmPath/Enum/E_DrivingMode` _drivingmode))

(fn `UserConstructionScript`
  (`/Game/HorrorEngine/Blueprints/Core/HorrorEngineMacros.HM_DefaultConstructions` (`self.CreateNewHorrorEvent`)))