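; Interactable NPC with a flipbook sprite that yaws toward the player every tick and toggles on/off like a switch.
; Use drives a timeline that lerps NpcPivot by the selected transform curve, with sounds, triggering linked actors and horror events immediately or after animation.
; Shots jitter the pivot and decrement health; leaving TurnRadius clears subtitles.
; Saved on/off state can be restored, but CollectSaveData is empty.
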(event `self.Use`
  (params (HorrorEvent :type Boolean))
  ;[1 1 1] Interact Settings
  (`/Game/HorrorEngine/Blueprints/Core/HorrorEngineMacros.HM_CheckInteraction`)
  (if (`self.On / Off`)
    (`self.Close/Off` false)
    (else
      (`self.Open/On` false))))

(event `self.Open/On`
  (params (HorrorEvent :type Boolean))
  (bind _transformtype (`self.TransformType`))
  (bind _actorstouse (`self.ActorsToUse`))
  (bind _returnvalue (or (`|EnumEquality` _transformtype "NewEnumerator0") (`|EnumEquality` _transformtype "NewEnumerator4")))
  ;[1 1 1] Open / Close Settings
  (`/Game/HorrorEngine/Blueprints/Core/HorrorEngineMacros.HM_CheckInteraction`)
  (if (not (`self.On / Off`))
    (if (not (`self.UseAfterAnimation`))
      (set `self.On / Off` true)
      (`self.Open/On` (`self.ActorsToUse`) false)
      (`self.HorrorEventCheck` "NewEnumerator3"))
    (set `self.InteractionEnabled` false)
    (bind (_direction _direct _direct__easy_ease_ _elastic _elastic__easy_ease_ _flip_flop _flip_flop__easy_ease_) (`Timeline|ButtonTimeline` :!via `PlayFromStart` :!label _label)
      (:`Update`
        (bind _returnvalue_2 (select `/Game/HorrorEngine/Blueprints/Enums/TransfromType` (`self.TransformType`) :`NewEnumerator0` _direct :`NewEnumerator4` _direct__easy_ease_ :`NewEnumerator5` _elastic :`NewEnumerator8` _elastic__easy_ease_ :`NewEnumerator9` _flip_flop :`NewEnumerator13` _flip_flop__easy_ease_ :!type "Float (double-precision)"))
        (`SceneComponent.K2_SetRelativeLocationAndRotation` (`self.NpcPivot`) (`KismetMathLibrary.VLerp` (`self.OffLocation`) (`self.OnLocation`) _returnvalue_2) (`KismetMathLibrary.RLerp` (`self.OffRotation`) (`self.OnRotation`) _returnvalue_2) false false))
      (:`Finished`
        (switch `ETimelineDirection` _direction
          (:`Forward`
            (`/Game/HorrorEngine/Blueprints/Core/HorrorEngineFunctions.SetMesh` (`self.Npc`) (`self.ButtonOnMesh`))
            (if (`self.UseAfterAnimation`)
              (set `self.On / Off` true)
              (`self.Open/On` _actorstouse false)
              (`self.HorrorEventCheck` "NewEnumerator3")))
          (:`Backward`
            (`/Game/HorrorEngine/Blueprints/Core/HorrorEngineFunctions.SetMesh` (`self.Npc`) (`self.ButtonOffMesh`))
            (if (`self.UseAfterAnimation`)
              (set `self.On / Off` false)
              (`self.Close/Off` _actorstouse false)
              (`self.HorrorEventCheck` "NewEnumerator4"))))
        (set `self.InteractionEnabled` true)
        (if (`self.StopSoundsAfterAnimation`)
          (`/Game/HorrorEngine/Blueprints/Core/HorrorEngineMacros.HM_StopAll3DSounds`)))
      (:`ButtonStartSound`
        (if _returnvalue
          (switch `ETimelineDirection` _direction
            (:`Forward`
              _)))
        (`/Game/HorrorEngine/Blueprints/Core/HorrorEngineMacros.HM_3DSound` null false (`self.TurnOnSound`) (`self.NpcPivot`) (`self.SoundAttenuation`)))
      (:`ButtonEndSound`
        (if _returnvalue
          (switch `ETimelineDirection` _direction
            (:`Backward`
              _)))
        (`/Game/HorrorEngine/Blueprints/Core/HorrorEngineMacros.HM_3DSound` null false (`self.TurnOffSound`) (`self.NpcPivot`) (`self.SoundAttenuation`))))))

(event `self.Close/Off`
  (params (HorrorEvent :type Boolean))
  ;[1 1 1] Open / Close Settings
  (`/Game/HorrorEngine/Blueprints/Core/HorrorEngineMacros.HM_CheckInteraction`)
  (if (`self.On / Off`)
    (if (not (`self.UseAfterAnimation`))
      (set `self.On / Off` false)
      (`self.Close/Off` (`self.ActorsToUse`) false)
      (`self.HorrorEventCheck` "NewEnumerator4"))
    (set `self.InteractionEnabled` false)
    (goto _label :!via `ReverseFromEnd`)))

(event `/Game/HorrorEngine/Blueprints/Core/HorrorEngineInterface.CollectSaveData`
  ;[0 1 0.5572] Save Settings
)

(event `/Game/HorrorEngine/Blueprints/Core/HorrorEngineInterface.RestoreSaveData`
  (params (AssetSave :type "/Game/HorrorEngine/Blueprints/Structures/SaveStructures/AssetsSave Structure"))
  (bind _offrotation (`self.OffRotation`))
  (bind _offlocation (`self.OffLocation`))
  (bind _transformtype (`self.TransformType`))
  (bind _returnvalue (or (`|EnumEquality` _transformtype "NewEnumerator9") (`|EnumEquality` _transformtype "NewEnumerator13")))
  ;[0 1 0.5572] Save Settings
  (set `self.On / Off` (`.BooleanSlot01_63_ED79FB5D49E9ED6768D7AE96EDFDE8DB` (break `/Game/HorrorEngine/Blueprints/Structures/SaveStructures/AssetsSave` AssetSave)))
  (`/Game/HorrorEngine/Blueprints/Core/HorrorEngineFunctions.SetMesh` (`self.Npc`) (select `bool` (`self.On / Off`) :`false` (`self.ButtonOffMesh`) :`true` (`self.ButtonOnMesh`)))
  (`SceneComponent.K2_SetRelativeLocationAndRotation` (`self.NpcPivot`) (select `bool` _returnvalue :`false` (select `bool` (`self.On / Off`) :`false` _offlocation :`true` (`self.OnLocation`)) :`true` _offlocation) (select `bool` _returnvalue :`false` (select `bool` (`self.On / Off`) :`false` _offrotation :`true` (`self.OnRotation`)) :`true` _offrotation) false false))

(event `self.ReceiveTick`
  (params (DeltaSeconds :type "Float (single-precision)"))
  ;[1 1 1] Rotate to player
  (bind _asem_path_player (cast `/Game/EmPath/Blueprints/EmPathPlayer` (`Controller.K2_GetPawn` (`GameplayStatics.GetPlayerController` 0))))
  (`/Engine/EditorBlueprintResources/StandardMacros.IsValid` _asem_path_player
    (:`Is Valid`
      (`self.K2_SetActorRotation` (`KismetMathLibrary.MakeRotator` 0.0 0.0 (.yaw (`KismetMathLibrary.FindLookAtRotation` (`self.K2_GetActorLocation`) (`self.K2_GetActorLocation` _asem_path_player))))))))

(event `self.Shoot`
  (params (HorrorEvent :type Boolean))
  (bind _health (`self.Health`))
  (bind _health_2 (`self.Health`))
  ;[1 1 1] Damage
  (if (not (<= _health 0.0))
    (`SceneComponent.K2_SetRelativeRotation` (`self.NpcPivot`) (`KismetMathLibrary.MakeRotator` (`KismetMathLibrary.RandomFloatInRange` 50.0 20.0) (`KismetMathLibrary.RandomFloatInRange` -20.0 20.0) (`KismetMathLibrary.RandomFloatInRange` -20.0 20.0)) false false)
    (`KismetSystemLibrary.Delay` 0.2)
    (`SceneComponent.K2_SetRelativeRotation` (`self.NpcPivot`) (`KismetMathLibrary.MakeRotator` 0.0) false false)
    (bind _result (`/Engine/EditorBlueprintResources/StandardMacros.DecrementFloat` _health_2)
      (:`  `
        (set `self.Health` _result)
        (`KismetSystemLibrary.PrintString` (`KismetStringLibrary.Conv_DoubleToString` _health))
        (if (== _health_2 0.0)
          (`self.SetActorHiddenInGame` false))))))

(event `self.TurnRadius.OnComponentBeginOverlap`
  (params (OverlappedComponent :type "PrimitiveComponent Object Reference") (OtherActor :type "Actor Object Reference") (OtherComp :type "PrimitiveComponent Object Reference") (OtherBodyIndex :type Integer) (bFromSweep :type Boolean) (SweepResult :type "HitResult Structure (by ref)"))
  ;[1 1 1] Overlap Action
)

(event `self.TurnRadius.OnComponentEndOverlap`
  (params (OverlappedComponent :type "PrimitiveComponent Object Reference") (OtherActor :type "Actor Object Reference") (OtherComp :type "PrimitiveComponent Object Reference") (OtherBodyIndex :type Integer))
  (bind _returnvalue (`GameplayStatics.GetPlayerController` 0))
  (if (!= null _returnvalue)
    (cast `/Game/EmPath/Blueprints/EmPathPlayer` (`Controller.K2_GetPawn` _returnvalue))
    (bind _assubtitle_wb (cast `/Game/HorrorEngine/Blueprints/Widgets/SubtitleWB` (`self.Subtitle WB`)))
    (`/Game/HorrorEngine/Blueprints/Widgets/SubtitleWB.RemoveSubtitle` _assubtitle_wb)))

(fn `UserConstructionScript`
  (bind _offrotation (`self.OffRotation`))
  (bind _offlocation (`self.OffLocation`))
  (bind _transformtype (`self.TransformType`))
  (bind _returnvalue (or (`|EnumEquality` _transformtype "NewEnumerator9") (`|EnumEquality` _transformtype "NewEnumerator13")))
  (`/Game/HorrorEngine/Blueprints/Core/HorrorEngineMacros.HM_DefaultConstructions` (`self.CreateNewHorrorEvent`))
  (`/Game/HorrorEngine/Blueprints/Core/HorrorEngineFunctions.SetMesh` (`self.Interact`) (`self.ButtonBaseMesh`))
  (`/Game/HorrorEngine/Blueprints/Core/HorrorEngineFunctions.SetMesh` (`self.Npc`) (select `bool` (`self.On / Off`) :`false` (`self.ButtonOffMesh`) :`true` (`self.ButtonOnMesh`)))
  (`/Game/HorrorEngine/Blueprints/Core/HorrorEngineFunctions.PlayRate` (`self.ButtonTimeline`) (`self.Animation Speed (Sec)`))
  (`SceneComponent.K2_SetRelativeLocationAndRotation` (`self.NpcPivot`) (select `bool` _returnvalue :`false` (select `bool` (`self.On / Off`) :`false` _offlocation :`true` (`self.OnLocation`)) :`true` _offlocation) (select `bool` _returnvalue :`false` (select `bool` (`self.On / Off`) :`false` _offrotation :`true` (`self.OnRotation`)) :`true` _offrotation) false false)
  (`PaperFlipbookComponent.SetFlipbook` (`self.Sprite`) (`self.NpcSprite`)))