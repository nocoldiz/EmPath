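; Bubba NPC that drives on the TheRoad level, sits idle elsewhere, and talks with the player through topic-based dialogue.
; On the road, BeginPlay fills the dialogue maps from four random DT_BubbaDialogue row picks, then refreshes topics.
; SendDialogues swaps in a supplied line set as a single "Talk" topic and starts it, messaging the player pawn before and after.
; SetPlaceDialogue, used off the road, and the passenger events are empty stubs.
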(event `SetPlaceDialogue`)

(event `RandomizeDrivingDialogue`
  (bind _outrownames (`DataTableFunctionLibrary.GetDataTableRowNames` "/Game/EmPath/DataTables/DT_BubbaDialogue.DT_BubbaDialogue"))
  (for _ (range 4)
    (bind _returnvalue (`|GetDataTableRow` "/Game/EmPath/DataTables/DT_BubbaDialogue.DT_BubbaDialogue" (`KismetArrayLibrary.Array_Random` _outrownames))
      (:`then`
        (bind (_topic _dialogue) (break `/Game/EmPath/Structures/ST_BubbaDialogue` _returnvalue))
        (bind _returnvalue_2 (`KismetTextLibrary.Conv_TextToString` _topic))
        (`BlueprintMapLibrary.Map_Add` (`self.DialogLines`) (`KismetArrayLibrary.Array_Random` (`KismetStringLibrary.ParseIntoArray` _returnvalue_2)) (make `/Game/EmPath/Structures/ST_Dialogue` _dialogue))
        (`BlueprintMapLibrary.Map_Add` (`self.DialogIndexes`) _returnvalue_2))))
  (`self.RefreshTopics`))

(event `self.ReceiveBeginPlay`
  (bind _skeletalmesh_0 (`self.SkeletalMesh_0`))
  (bind _returnvalue (`GameplayStatics.GetCurrentLevelName` true))
  (if (`KismetStringLibrary.EqualEqual_StrStr` _returnvalue "TheRoad")
    (`SkeletalMeshComponent.SetAnimation` _skeletalmesh_0 "/Game/EmPath/Animations/Bubba/Driving.Driving")
    (`self.RandomizeDrivingDialogue`)
    (else
      ;[1 1 1] Comment
      (`SkeletalMeshComponent.SetAnimation` _skeletalmesh_0 "/Game/EmPath/Animations/Bubba/Sitting_Idle.Sitting_Idle")
      (`self.SetPlaceDialogue`))))

(event `EnterPassenger`
  (params (Material :type "Material Object Reference")))

(event `ExitPassenger`)

(event `/Game/EmPath/Interfaces/BI_Bubba.SendDialogues`
  (params (Dialogs :type "Array of Text (by ref)"))
  (bind _returnvalue (`GameplayStatics.GetPlayerPawn` 0))
  (set `self.MaxDialogIndex` (`KismetArrayLibrary.Array_Length` Dialogs))
  (set `self.ActiveOptions` (`|MakeArray` "Talk"))
  (set `self.SelectedTopic` "Talk")
  (set `self.DialogIndexes` (`|MakeMap` "Talk"))
  (set `self.DialogLines` (`|MakeMap` "Talk" (make `/Game/EmPath/Structures/ST_Dialogue` Dialogs)))
  (message `/Game/EmPath/Interfaces/BI_GameActions.StartTalking` _returnvalue "NewEnumerator0")
  (`self.Talk`)
  (message `/Game/EmPath/Interfaces/BI_GameActions.StartTalking` _returnvalue "NewEnumerator1"))

(event `self.PlayDialog`
  (params (NewParam :type String))
  (`self.Talk`))

(fn `UserConstructionScript`
  (`parent.UserConstructionScript`))