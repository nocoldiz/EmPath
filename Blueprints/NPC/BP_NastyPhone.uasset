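; BP_NastyPhone is a talkable NPC Blueprint, named as a phone, that hurts the player when talked to.
; It overrides OnTalkEvent, runs the parent behavior, then sends a small fixed damage message to the first player's pawn, with itself as causer and its own location as the hit point.
; All other logic comes from the parent class, as the event graph and construction script add nothing.
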(fn `OnTalkEvent`
  (`parent.OnTalkEvent`)
  (message `/Game/EmPath/Interfaces/BPI_Damagable.TakeDamage` (`GameplayStatics.GetPlayerPawn` 0) (make `/Game/EmPath/Structures/S_DamageInfo` 5.0 "NewEnumerator1" "NewEnumerator3") self (`self.K2_GetActorLocation`)))

(fn `UserConstructionScript`
  (`parent.UserConstructionScript`))