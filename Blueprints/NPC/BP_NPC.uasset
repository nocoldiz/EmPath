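; BP_NPC is a talkable, shootable NPC with a flipbook sprite that turns to face the player, wobbles when shot and destroys itself at zero health.
; Use runs Talk, which picks lines for the player's selected topic by dialog type: indexed sequence, random, class DataTable or mixed.
; Talk opens WB_DialogBox, speeding it up on repeat use, while a looping SetLetter timer plays a positional sound per letter as a synthetic voice.
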(event `self.ReceiveBeginPlay`
  (bind _dialogindexes (`self.DialogIndexes`))
  ;[1 1 1] BeginPlay
  (bind _keys (`BlueprintMapLibrary.Map_Keys` (`self.DialogLines`)))
  (`KismetArrayLibrary.Array_Set` _keys 0 (`KismetArrayLibrary.Array_Random` (`self.Greetings`)))
  (set `self.ActiveOptions` _keys)
  (for _array_element _keys
    (`BlueprintMapLibrary.Map_Add` _dialogindexes _array_element)
    (set `self.DefaultIndexes` _dialogindexes)))

(event `self.ReceiveTick`
  (params (DeltaSeconds :type "Float (single-precision)"))
  ;[1 1 1] Rotate to player
  (if (not (`self.DisableTurn`))
    (bind _location (message `/Game/EmPath/Interfaces/BI_GameActions.GetActorLocation` (`GameplayStatics.GetPlayerPawn` 0)))
    (`self.K2_SetActorRotation` (`KismetMathLibrary.MakeRotator` 0.0 0.0 (.yaw (`KismetMathLibrary.FindLookAtRotation` (`self.K2_GetActorLocation`) _location))))))

(event `self.Shoot`
  (params (HorrorEvent :type Boolean))
  (bind _health (`self.Health`))
  ;[1 1 1] Damage
  (if (not (<= (`self.Health`) 0.0))
    (`SceneComponent.K2_SetRelativeRotation` (`self.NpcPivot`) (`KismetMathLibrary.MakeRotator` (`KismetMathLibrary.RandomFloatInRange` 50.0 20.0) (`KismetMathLibrary.RandomFloatInRange` -20.0 20.0) (`KismetMathLibrary.RandomFloatInRange` -20.0 20.0)) false false)
    (`KismetSystemLibrary.Delay` 0.2)
    (`SceneComponent.K2_SetRelativeRotation` (`self.NpcPivot`) (`KismetMathLibrary.MakeRotator` 0.0) false false)
    (bind _result (`/Engine/EditorBlueprintResources/StandardMacros.DecrementFloat` _health)
      (:`  `
        (set `self.Health` _result)
        (if (<= _health 0.0)
          (`self.K2_DestroyActor`))))))

(event `/Game/EmPath/Interfaces/BI_NPC.PlayDialog`
  (params (Dialog :type String))
  ;[1 1 1] PlayDialog
  (for _index (range (+ (`KismetStringLibrary.Len` Dialog) 1))
    (`KismetSystemLibrary.Delay` (`self.LetterDelay`))
    (bind _returnvalue (`KismetTextLibrary.Conv_TextToString` (`|GetArrayItem` (`|MakeArray` (`KismetTextLibrary.Conv_StringToText` Dialog)) _index)))
    (if (or (`KismetStringLibrary.EqualEqual_StrStr` _returnvalue ".") (`KismetStringLibrary.EqualEqual_StrStr` _returnvalue ","))
      (`KismetSystemLibrary.Delay` 0.5))
    (`self.PlayletterSound` _returnvalue)))

(event `self.Use`
  (params (HorrorEvent :type Boolean))
  ;[1 1 1] Interact Settings
  (`self.Talk`))

(event `self.Capsule.OnComponentBeginOverlap`
  (params (OverlappedComponent :type "PrimitiveComponent Object Reference") (OtherActor :type "Actor Object Reference") (OtherComp :type "PrimitiveComponent Object Reference") (OtherBodyIndex :type Integer) (bFromSweep :type Boolean) (SweepResult :type "HitResult Structure (by ref)"))
  (if (== OtherActor (`GameplayStatics.GetPlayerPawn` 0))
    (bind _playernear (`self.IsPlayerNear` 200.0))
    (if _playernear
      _)))

(fn `Choose Subtitle`
  (returns (FullText :type Text))
  (locals (BubbaName :type Text :default "NSLOCTEXT(\"\", \"7351920940612346FFD39999B21B466A\", \"Bubba\")"))
  (bind _returnvalue (`KismetStringLibrary.ParseIntoArray` "" ";"))
  (bind (_dialogue _ishidden _dialogtype) (break `/Game/EmPath/Structures/ST_Dialogue` (`BlueprintMapLibrary.Map_Find` (`self.DialogLines`) (`self.SelectedTopic`))))
  (bind _returnvalue_2 (`KismetArrayLibrary.Array_Length` _dialogue))
  (if true
    (if (== (`KismetStringLibrary.Len` (`KismetStringLibrary.Conv_NameToString` "None")) 0)
      (if (> _returnvalue_2 0)
        ;[1 1 1] Choose Next Subtitle
        (if (and (`|EnumEquality` _dialogtype "NewEnumerator1") false) :!label _label
          ;[1 1 1] Choose random line
          (set `self.FullText` (`|GetArrayItem` _dialogue (`KismetMathLibrary.RandomInteger` _returnvalue_2)))
          (elif (or (`|EnumEquality` _dialogtype "NewEnumerator0") (`|EnumEquality` _dialogtype "NewEnumerator4"))
            ;[1 1 1] Get dialogue at index
            (set `self.FullText` (`|GetArrayItem` (`.Dialogue_16_CC43CD494049E0FBDE42708AD7BBF57A` (break `/Game/EmPath/Structures/ST_Dialogue` (`BlueprintMapLibrary.Map_Find` (`self.DialogLines`) (`self.SelectedTopic`)))) (`BlueprintMapLibrary.Map_Find` (`self.DialogIndexes`) (`self.SelectedTopic`))))
            (else
              (set `self.FullText` ""))))
        (`self.PlayDialog` (`KismetTextLibrary.Conv_TextToString` (`self.FullText`)) :!label _label_2)
        (return (`self.FullText`)))
      (else
        (bind _returnvalue_3 (`|GetDataTableRow` "/Game/EmPath/DataTables/DT_ClassDialogue.DT_ClassDialogue" "Driver")
          (:`then`
            (set `self.FullText` (`KismetTextLibrary.Conv_StringToText` (`|GetArrayItem` _returnvalue (`KismetMathLibrary.RandomInteger` (`KismetArrayLibrary.Array_Length` _returnvalue)))))
            (goto _label_2))
          (:`RowNotFound`
            (goto _label)))))
    (else
      ;[1 1 1] Get Bubba Dialogue
      (bind _outrownames (`DataTableFunctionLibrary.GetDataTableRowNames` "/Game/EmPath/DataTables/DT_BubbaDialogue.DT_BubbaDialogue"))
      (bind _returnvalue_4 (`|GetDataTableRow` "/Game/EmPath/DataTables/DT_BubbaDialogue.DT_BubbaDialogue" (`KismetStringLibrary.Conv_StringToName` (`KismetStringLibrary.Conv_IntToString` (`KismetMathLibrary.RandomIntegerInRange` 0 (`KismetArrayLibrary.Array_Length` _outrownames)))))
        (:`then`
          (set `self.FullText` (`.Dialogue_11_CC43CD494049E0FBDE42708AD7BBF57A` (break `/Game/EmPath/Structures/ST_BubbaDialogue` _returnvalue_4)))
          (return (`self.FullText`)))))))

(fn `GetDialogFromNPCClass`
  (returns (Dialog :type Text))
  (bind _returnvalue (`KismetStringLibrary.ParseIntoArray` "" ";"))
  (bind _fulltext (`self.FullText`))
  (bind (_dialogue _ishidden _dialogtype) (break `/Game/EmPath/Structures/ST_Dialogue` (`BlueprintMapLibrary.Map_Find` (`self.DialogLines`) (`self.SelectedTopic`))))
  (bind _returnvalue_2 (`KismetArrayLibrary.Array_Length` _dialogue))
  (if (`KismetTextLibrary.NotEqual_TextText` (`KismetTextLibrary.Conv_StringToText` "Bubba") (`self.Name`))
    (if (== (`KismetStringLibrary.Len` (`KismetStringLibrary.Conv_NameToString` (`self.Npc Class`))) 0)
      (if (> _returnvalue_2 0)
        ;[1 1 1] Choose Next Subtitle
        (if (and (`|EnumEquality` _dialogtype "NewEnumerator6") false) :!label _label
          ;[1 1 1] Choose random line
          (set `self.FullText` (`|GetArrayItem` _dialogue (`KismetMathLibrary.RandomInteger` _returnvalue_2)))
          (elif (or (`|EnumEquality` _dialogtype "NewEnumerator5") (`|EnumEquality` _dialogtype "NewEnumerator4"))
            ;[1 1 1] Get dialogue at index
            (set `self.FullText` (`|GetArrayItem` (`.Dialogue_16_CC43CD494049E0FBDE42708AD7BBF57A` (break `/Game/EmPath/Structures/ST_Dialogue` (`BlueprintMapLibrary.Map_Find` (`self.DialogLines`) (`self.SelectedTopic`)))) (`BlueprintMapLibrary.Map_Find` (`self.DialogIndexes`) (`self.SelectedTopic`))))
            (else
              (set `self.FullText` ""))))
        (`self.PlayDialog` (`KismetTextLibrary.Conv_TextToString` _fulltext) :!label _label_2)
        (return _fulltext))
      (else
        (bind _returnvalue_3 (`|GetDataTableRow` "/Game/EmPath/DataTables/DT_ClassDialogue.DT_ClassDialogue" (`self.Npc Class`))
          (:`then`
            (set `self.FullText` (`KismetTextLibrary.Conv_StringToText` (`|GetArrayItem` _returnvalue (`KismetMathLibrary.RandomInteger` (`KismetArrayLibrary.Array_Length` _returnvalue)))))
            (goto _label_2))
          (:`RowNotFound`
            (goto _label)))))
    (else
      ;[1 1 1] Get Bubba Dialogue
      (bind _outrownames (`DataTableFunctionLibrary.GetDataTableRowNames` "/Game/EmPath/DataTables/DT_BubbaDialogue.DT_BubbaDialogue"))
      (bind _returnvalue_4 (`|GetDataTableRow` "/Game/EmPath/DataTables/DT_BubbaDialogue.DT_BubbaDialogue" (`KismetStringLibrary.Conv_StringToName` (`KismetStringLibrary.Conv_IntToString` (`KismetMathLibrary.RandomIntegerInRange` 0 (`KismetArrayLibrary.Array_Length` _outrownames)))))
        (:`then`
          (return (`.Dialogue_11_CC43CD494049E0FBDE42708AD7BBF57A` (break `/Game/EmPath/Structures/ST_BubbaDialogue` _returnvalue_4))))))))

(fn `IsPlayerNear`
  (params (Radius :type "Float (single-precision)"))
  (returns (PlayerNear :type Boolean))
  (return (<= (`self.GetDistanceTo` (`GameplayStatics.GetPlayerPawn` 0)) Radius)))

(fn `PlayletterSound`
  (params (Selection :type String))
  (`|ExecutionSequence`
    (:`then_0`
      ;[1 1 1] PlayLetter
      (switch `string` Selection
        (:`Default`
          (set `self.NextLetterSound` "/Game/EmPath/Sounds/FX_Silence.FX_Silence" :!label _label))
        (:`a`
          (set `self.NextLetterSound` "/Game/EmPath/Sounds/Dialogue/a.a"))
        (:`b`
          (set `self.NextLetterSound` "/Game/EmPath/Sounds/Dialogue/b.b"))
        (:`c`
          (set `self.NextLetterSound` "/Game/EmPath/Sounds/Dialogue/c.c"))
        (:`d`
          (set `self.NextLetterSound` "/Game/EmPath/Sounds/Dialogue/d.d"))
        (:`e`
          (set `self.NextLetterSound` "/Game/EmPath/Sounds/Dialogue/e.e"))
        (:`f`
          (set `self.NextLetterSound` "/Game/EmPath/Sounds/Dialogue/e.e"))
        (:`g`
          (set `self.NextLetterSound` "/Game/EmPath/Sounds/Dialogue/g.g"))
        (:`h`
          (set `self.NextLetterSound` "/Game/EmPath/Sounds/Dialogue/h.h"))
        (:`i`
          (set `self.NextLetterSound` "/Game/EmPath/Sounds/Dialogue/i.i"))
        (:`l`
          (set `self.NextLetterSound` "/Game/EmPath/Sounds/Dialogue/l.l"))
        (:`m`
          (set `self.NextLetterSound` "/Game/EmPath/Sounds/Dialogue/m.m"))
        (:`n`
          (set `self.NextLetterSound` "/Game/EmPath/Sounds/Dialogue/n.n"))
        (:`o`
          (set `self.NextLetterSound` "/Game/EmPath/Sounds/Dialogue/o.o"))
        (:`p`
          (set `self.NextLetterSound` "/Game/EmPath/Sounds/Dialogue/p.p"))
        (:`q`
          (set `self.NextLetterSound` "/Game/EmPath/Sounds/Dialogue/q.q"))
        (:`r`
          (set `self.NextLetterSound` "/Game/EmPath/Sounds/Dialogue/r.r"))
        (:`s`
          (set `self.NextLetterSound` "/Game/EmPath/Sounds/Dialogue/s.s"))
        (:`t`
          (set `self.NextLetterSound` "/Game/EmPath/Sounds/Dialogue/t.t"))
        (:`u`
          (set `self.NextLetterSound` "/Game/EmPath/Sounds/Dialogue/u.u"))
        (:`v`
          (set `self.NextLetterSound` "/Game/EmPath/Sounds/Dialogue/v.v"))
        (:`w`
          (set `self.NextLetterSound` "/Game/EmPath/Sounds/Dialogue/w.w"))
        (:`z`
          (set `self.NextLetterSound` "/Game/EmPath/Sounds/Dialogue/z.z"))
        (:`x`
          (set `self.NextLetterSound` "/Game/EmPath/Sounds/Dialogue/x.x"))
        (:`y`
          (set `self.NextLetterSound` "/Game/EmPath/Sounds/Dialogue/y.y"))
        (:`.`
          (goto _label))
        (:`,`
          (goto _label))
        (:`!`
          (goto _label))
        (:`?`
          (goto _label))
        (:`:`
          (goto _label))))
    (:`then_1`
      (`GameplayStatics.SpawnSoundAtLocation` (`self.NextLetterSound`) (`self.K2_GetActorLocation`) (struct) 0.4 (`self.Pitch`) 0.0 "/Game/HorrorEngine/Audio/_ATT_Profiles/ATT_Ring.ATT_Ring" null))))

(fn `SetDialogLines`
  (params (Dialog :type "Array of Text")))

(fn `SetLetter`
  (bind _returnvalue (`KismetStringLibrary.GetCharacterArrayFromString` (`KismetTextLibrary.Conv_TextToString` (`self.FullText`))))
  (`self.PlayletterSound` (`|GetArrayItem` _returnvalue (`self.LetterIndex`)))
  (bind _result (`/Engine/EditorBlueprintResources/StandardMacros.IncrementInt` (`self.LetterIndex`))
    (:`  `
      (if (== _result (`KismetArrayLibrary.Array_Length` _returnvalue))
        (`KismetSystemLibrary.K2_ClearTimer` null "SetLetter")
        (set `self.LetterIndex` 0)))))

(fn `Talk`
  (bind _returnvalue (`GameplayStatics.GetPlayerPawn` 0))
  (bind _widget (`self.Widget`))
  (bind _selectedtopic (`self.SelectedTopic`))
  (bind (_dialogue _ishidden _dialogtype) (break `/Game/EmPath/Structures/ST_Dialogue` (`BlueprintMapLibrary.Map_Find` (`self.DialogLines`) (`self.SelectedTopic`))))
  (bind _dialogstate (message `/Game/EmPath/Interfaces/BI_GameActions.GetIsTalking` _returnvalue))
  (`KismetSystemLibrary.PrintString` (`|GetEnumeratorNameAsString` _dialogstate) true true (struct :`G` 0.66 :`B` 1.0 :`A` 1.0) 0.3)
  (bind _index (message `/Game/EmPath/Interfaces/BI_GameActions.GetDialogTopicIndex` _returnvalue))
  ;[1 1 1] Set current selected topic
  (bind _keys (`BlueprintMapLibrary.Map_Keys` (`self.DialogLines`)))
  (bind _output (`|GetArrayItem` _keys _index))
  (if (not (`KismetStringLibrary.EqualEqual_StrStr` _output (`self.SelectedTopic`)))
    (set `self.DialogIndexes` (`self.DefaultIndexes`)))
  (set `self.SelectedTopic` _output)
  (switch `/Game/EmPath/Enum/E_DialogState` _dialogstate
    (:`NewEnumerator0`
      (message `/Game/EmPath/Interfaces/BI_GameActions.StartTalking` (`GameplayStatics.GetPlayerPawn` 0) "NewEnumerator1")
      (switch `/Game/EmPath/Enum/E_DialogTypes` _dialogtype
        (:`NewEnumerator0`
          (bind _max (`self.GetNextDialog` :!label _label))
          (if (not _max)
            ;[1 1 1] Go to next index on topic
            (bind _result (`/Engine/EditorBlueprintResources/StandardMacros.IncrementInt` (`BlueprintMapLibrary.Map_Find` (`self.DialogIndexes`) (`self.SelectedTopic`)))
              (:`  `
                (`BlueprintMapLibrary.Map_Add` (`self.DialogIndexes`) (`self.SelectedTopic`) _result)))))
        (:`NewEnumerator1`
          ;[1 1 1] Random dialog lines
          (set `self.FullText` (`KismetArrayLibrary.Array_Random` _dialogue) :!label _label_2))
        (:`NewEnumerator2`
          (goto _label))
        (:`NewEnumerator3`
          (goto _label))
        (:`NewEnumerator6`
          (bind _dialog (`self.GetDialogFromNPCClass` :!label _label_3))
          (set `self.FullText` _dialog))
        (:`NewEnumerator7`
          (if (> (`KismetMathLibrary.RandomFloatInRange` 0.0 1.0) 0.5)
            (goto _label_2)
            (else
              (goto _label_3)))))
      ;[1 1 1] Check if widget is opened
      (bind _foundwidgets (`WidgetBlueprintLibrary.GetAllWidgetsOfClass` "/Game/EmPath/UI/WB_DialogBox.WB_DialogBox_C"))
      (bind _output_2 (`|GetArrayItem` _foundwidgets))
      (`/Engine/EditorBlueprintResources/StandardMacros.IsValid` _output_2
        (:`Is Valid`
          (`/Game/EmPath/UI/WB_DialogBox.RemoveWidgetNoDelay` _output_2)
          (`KismetSystemLibrary.K2_ClearTimer` null "SetLetter")
          (set `self.LetterIndex` 0)
          (if (not (== (- (`KismetArrayLibrary.Array_Length` (`.Dialogue_16_CC43CD494049E0FBDE42708AD7BBF57A` (break `/Game/EmPath/Structures/ST_Dialogue` (`BlueprintMapLibrary.Map_Find` (`self.DialogLines`) _selectedtopic)))) 0) (`BlueprintMapLibrary.Map_Find` (`self.DialogIndexes`) _selectedtopic)))
            (`self.Talk`)))
        (:`Is Not Valid`
          (bind _returnvalue_2 (`|CreateWidget` "/Game/EmPath/UI/WB_DialogBox.WB_DialogBox_C" null (`self.FullText`) false 0.0 0.0 "NewEnumerator0" (`BlueprintMapLibrary.Map_Find` (`self.DialogIndexes`) (`self.SelectedTopic`)) (`self.Name`)))
          (set `self.Widget` _returnvalue_2)
          (`UserWidget.AddToViewport` _returnvalue_2 0)
          (`KismetSystemLibrary.K2_SetTimer` null "SetLetter" 0.05 true))))
    (:`NewEnumerator1`
      ;[1 1 1] SpeedUp
      (`/Engine/EditorBlueprintResources/StandardMacros.IsValid` _widget
        (:`Is Valid`
          (`/Game/EmPath/UI/WB_DialogBox.SpeedUpDialogue` _widget)
          (`KismetSystemLibrary.K2_ClearTimer` null "SetLetter")
          (set `self.LetterIndex` 0))))
    (:`NewEnumerator2`
      (`KismetSystemLibrary.K2_ClearTimer` null "SetLetter")
      (set `self.LetterIndex` 0)
      (message `/Game/EmPath/Interfaces/BI_GameActions.StartTalking` (`GameplayStatics.GetPlayerPawn` 0) "NewEnumerator0")
      (`self.Talk`))))

(fn `UserConstructionScript`
  (`/Game/HorrorEngine/Blueprints/Core/HorrorEngineMacros.HM_DefaultConstructions` (`self.CreateNewHorrorEvent`))
  (`/Game/HorrorEngine/Blueprints/Core/HorrorEngineFunctions.SetMesh` (`self.Interact`) (`self.ButtonBaseMesh`))
  (`/Game/HorrorEngine/Blueprints/Core/HorrorEngineFunctions.PlayRate` null (`self.Animation Speed (Sec)`))
  (`PaperFlipbookComponent.SetFlipbook` (`self.Sprite`) (`self.NpcSprite`)))