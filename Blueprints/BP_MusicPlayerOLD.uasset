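; Interactable radio prop that plays music channels, toggled by Use and cycled by AlternativeUse with a tuning sound between channels.
; On/off swaps mesh settings, plays switch sounds with interaction briefly locked, and, like channel changes, fires horror event checks.
; Tick tracks playback time so the track resumes mid-song; power state, time and channel are handled through save/restore.
; The track-info notice widget code is disconnected and never runs.
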(event `self.BeginLoad`
  ;[1 1 1] On / Off Settings
  (`self.`)
  (if (`self.On / Off`)
    (`self.PlayRadio`)))

(event `self.Use`
  (params (HorrorEvent :type Boolean) (UseFromBackpack :type Boolean))
  ;[1 1 1] Interact Settings
  (`self.`)
  (if (`self.On / Off`)
    (`self.Close/Off` false)
    (else
      (`self.Open/On` false))))

(event `self.AlternativeUse`
  (params (HorrorEvent :type Boolean))
  ;[1 1 1] Interact Settings
  (`self.SwitchChannel`))

(event `self.Open/On`
  (params (HorrorEvent :type Boolean))
  (bind _on___off (`self.On / Off`))
  (bind _output (`|GetArrayItem` (`self.AddChannels`) (`self.StartChannel`)))
  ;[1 1 1] On / Off Settings
  (`self.`)
  (if (not (`self.On / Off`))
    (set `self.On / Off` true)
    (`self.SetMesh` (`self.Radio`) (select `bool` _on___off :!type " Structure") :!label _label)
    (`self.HorrorEventCheck` (select `bool` _on___off :!type "Byte"))
    (`|ExecutionSequence`
      (:`then_0`
        (set `self.InteractionEnabled` false)
        (bind (_sound _duration) (`self.` null false (select `bool` (`self.On / Off`) :`false` (`self.TurnOffSound`) :`true` (`self.TurnOnSound`)) (`self.Radio`) (`self.SoundAttenuation`)))
        (`KismetSystemLibrary.Delay` _duration)
        (set `self.InteractionEnabled` true))
      (:`then_1`
        (if (`self.On / Off`)
          (bind (_sound_2 _duration_2) (`self.` _output false _output (`self.Radio`) (`self.SoundAttenuation`) (`self.CurrentTime`) :!label _label_2))
          (set `self.CurrentDuration` _duration_2)
          (`self.SetActorTickEnabled` true)
          (`KismetSystemLibrary.Delay` 8.0)
          (bind _returnvalue (`|GetDataTableRow` "/Game/EmPath/DataTables/DT_Music.DT_Music" (`|GetArrayItem` (`self.ChannelsInfo`))))
          (else
            (`self.` _output)
            (`self.` (`self.TuningSound`))
            (`self.SetActorTickEnabled` false)))))))

(event `self.ReceiveTick`
  (params (DeltaSeconds :type "Float (single-precision)"))
  (bind _returnvalue (+ DeltaSeconds (`self.CurrentTime`)))
  ;[1 1 1] Get Playback Time
  (if (not (`self.Switching`))
    (set `self.CurrentTime` (select `bool` (>= _returnvalue (`self.CurrentDuration`)) :`false` _returnvalue))))

(event `self.Close/Off`
  (params (HorrorEvent :type Boolean))
  ;[1 1 1] On / Off Settings
  (`self.`)
  (if (`self.On / Off`)
    (set `self.On / Off` false)
    (goto _label)))

(event `PlayRadio`
  ;[1 1 1] On / Off Settings
  (goto _label_2))

(event `SwitchChannel`
  (bind _tuningsound (`self.TuningSound`))
  (bind _output (`|GetArrayItem` (`self.AddChannels`) (`self.StartChannel`)))
  ;[1 1 1] Channel Settings
  (if (`self.On / Off`)
    (if (> (`KismetArrayLibrary.Array_LastIndex` (`self.AddChannels`)) 0)
      (set `self.InteractionEnabled` false)
      (set `self.Switching` true)
      (set `self.CurrentTime` 0.0)
      (`self.` (`|GetArrayItem` (`self.AddChannels`) (`self.StartChannel`)))
      (if (`KismetSystemLibrary.IsValid` (`self.TuningSound`))
        (bind (_sound _duration) (`self.` _tuningsound false _tuningsound (`self.Radio`) (`self.SoundAttenuation`)))
        (`KismetSystemLibrary.Delay` (- _duration 1.0)))
      (set `self.Switching` false)
      (set `self.InteractionEnabled` true)
      (set `self.StartChannel` (+ (`self.StartChannel`) 1))
      (if (not (`KismetArrayLibrary.Array_IsValidIndex` (`self.AddChannels`) (`self.StartChannel`)))
        (set `self.StartChannel` 0))
      (bind (_sound_2 _duration_2) (`self.` _output false _output (`self.Radio`) (`self.SoundAttenuation`)))
      (set `self.CurrentDuration` _duration_2)
      (`self.HorrorEventCheck` 0))))

(event `self.CollectSaveData`
  ;[0 1 0.5572] Save Settings
  (bind _asmaster (`self.GetPlayer`))
  (`KismetArrayLibrary.Array_Add` (`/Blueprints/BP_MusicPlayerOLD.AssetCache` (`/Blueprints/BP_MusicPlayerOLD.HE_SaveGameComponent` _asmaster)) (make `` (`KismetSystemLibrary.GetObjectName` self) (`self.On / Off`) false false false (`self.CurrentTime`) 0.0 (`self.StartChannel`) "+00000000.00:00:00.000000000" 0 (struct :`Actor` "NewEnumerator0" :`MeshSettings` (struct) :`InspectionSettings` (struct :`InspectionPivotLocation` (0.0 0.0 0.0) :`Takeable` true :`InspectionAnimation` true :`InspectionAnimationSpeedSec` 0.5 :`InspectionBeginRotation` (struct) :`InspectionBeginScale` 1.0 :`MinZoomScale` 1.0 :`MaxZoomScale` 2.0 :`RotationSpeed` 2.5 :`SlideSpeed` 1.0 :`MaxSlideValue` 10.0 :`ItemName` "NSLOCTEXT(\"[E9319CB74B6D000FB1FD816297025122]\", \"B04114684BE13C8CCDB6069E8D44812E\", \"Item Name\")" :`ItemInformation` "NSLOCTEXT(\"[E9319CB74B6D000FB1FD816297025122]\", \"A8A7B76B4C63391D1AC5A7B5D25FB9AE\", \"Item Information\")" :`ReadingText` "NSLOCTEXT(\"[E9319CB74B6D000FB1FD816297025122]\", \"5443C78745510DFFC83277B931F00907\", \"Reading Text\")" :`TakeButton` (struct :`ButtonText` "NSLOCTEXT(\"[E9319CB74B6D000FB1FD816297025122]\", \"9780C15042924951768718B819101440\", \"Take\")") :`ExamineButton` (struct :`ButtonText` "NSLOCTEXT(\"[E9319CB74B6D000FB1FD816297025122]\", \"5175E901487A84D459C6CCAF41D0E6C4\", \"Examine\")") :`ZoomPanButton` (struct :`ButtonText` "NSLOCTEXT(\"[E9319CB74B6D000FB1FD816297025122]\", \"1637EA9C4CEBCB9F6A7CD08E1CBC13F0\", \"Zoom/Slide\")") :`DismissButton` (struct :`ButtonText` "NSLOCTEXT(\"[E9319CB74B6D000FB1FD816297025122]\", \"5A5A20484193E091F4DA148242A59503\", \"Dismiss\")")) :`InventorySettings` (struct :`StorageType` "NewEnumerator3" :`NumberofItemstoAddInventory` 1 :`Interactable` true :`InteractionButton` (struct :`ButtonText` "NSLOCTEXT(\"[E9319CB74B6D000FB1FD816297025122]\", \"97A9B9D546AE5B371A60B2BF356CB282\", \"Use\")") :`SwitchButton` (struct :`ButtonText` "NSLOCTEXT(\"[E9319CB74B6D000FB1FD816297025122]\", \"0D5923514466DE04116E9EA58004B602\", \"Switch\")") :`ZoomSlideButton` (struct :`ButtonText` "NSLOCTEXT(\"[E9319CB74B6D000FB1FD816297025122]\", \"7F750DF3455A9335558F4A9BD1D2A436\", \"Zoom/Slide\")") :`CloseInventoryButton` (struct :`ButtonText` "NSLOCTEXT(\"[E9319CB74B6D000FB1FD816297025122]\", \"2EB73C5B425A32CFA76B8BA90D6BD57D\", \"Close\")")) :`Pistol_MeshSettingsTop` (struct) :`Vhs_CurrentTime` "+00000000.00:00:00.000000000"))))

(event `self.RestoreSaveData`
  (params (AssetSave :type " Structure"))
  (bind ((`BooleanSlot01_63_ED79FB5D49E9ED6768D7AE96EDFDE8DB` _booleanslot01) (`BooleanSlot02_64_3DE3E28A45CAE9F3E913659977556562` _booleanslot02) (`BooleanSlot03_65_04AA048C42686C9D2AF003962AEB7F6C` _booleanslot03) (`BooleanSlot04_66_3CB4510F40F5DDD3D81BCEA77398809A` _booleanslot04) (`FloatSlot01_62_3D225DB249A703592AAD5A8405C67C24` _floatslot01) (`FloatSlot02_72_0C6E79544AA699EC0216E1929F2FE1AC` _floatslot02) (`IntegerSlot01_75_ABA8053D4F033D11B1D4ECB38D77F6AB` _integerslot01)) (break `` AssetSave))
  ;[0 1 0.5572] Save Settings
  (set `self.On / Off` _booleanslot01)
  (set `self.CurrentTime` _floatslot01)
  (set `self.StartChannel` _integerslot01)
  (`self.SetMesh` (`self.Radio`) (select `bool` (`self.On / Off`) :!type " Structure"))
  (if (`self.On / Off`)
    (`self.PlayRadio`)))

(event `/Game/EmPath/Interfaces/BI_MusicPlayer.SetMusic`
  (params (Disable :type Boolean))
  (if Disable
    (`self.Close/Off` false)
    (else
      (`self.Open/On` false))))

(fn `UserConstructionScript`
  (`self.` _)
  (`self.SetMesh` (`self.Radio`) (select `bool` (`self.On / Off`) :!type " Structure")))