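; BP_InfiniteRoad is a road segment that chains copies of itself to form an endless road around the player.
; When the player pawn overlaps SpawnTrigger, it spawns a new segment at its Arrow's world transform and attaches it to the first actor tagged RoadBase, keeping world location and rotation.
; When the player pawn overlaps DeleteTrigger, the segment destroys itself; the SetSpeed event is empty.
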(event `self.SpawnTrigger.OnComponentBeginOverlap`
  (params (OverlappedComponent :type "PrimitiveComponent Object Reference") (OtherActor :type "Actor Object Reference") (OtherComp :type "PrimitiveComponent Object Reference") (OtherBodyIndex :type Integer) (bFromSweep :type Boolean) (SweepResult :type "HitResult Structure (by ref)"))
  (if (== OtherActor (`GameplayStatics.GetPlayerPawn` 0))
    (bind _returnvalue (`|SpawnActorFromClass` "BP_InfiniteRoad_C" (`SceneComponent.K2_GetComponentToWorld` (`self.Arrow`)) "Undefined" "MultiplyWithRoot" null null))
    (bind _outactors (`GameplayStatics.GetAllActorsWithTag` "RoadBase"))
    (`self.K2_AttachToActor` _returnvalue (`|GetArrayItem` _outactors) "None" "KeepWorld" "KeepWorld" "KeepRelative" false)))

(event `self.DeleteTrigger.OnComponentBeginOverlap`
  (params (OverlappedComponent :type "PrimitiveComponent Object Reference") (OtherActor :type "Actor Object Reference") (OtherComp :type "PrimitiveComponent Object Reference") (OtherBodyIndex :type Integer) (bFromSweep :type Boolean) (SweepResult :type "HitResult Structure (by ref)"))
  (if (== OtherActor (`GameplayStatics.GetPlayerPawn` 0))
    (`self.K2_DestroyActor`)))

(event `/Game/EmPath/Interfaces/BI_TerrainSpawner.SetSpeed`
  (params (NewParam :type "Float (double-precision)")))

(fn `UserConstructionScript`)