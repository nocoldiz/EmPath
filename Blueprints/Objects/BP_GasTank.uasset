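; BP_GasTank is a gas tank object that explodes as soon as it takes any damage.
; TakeDamage calls ExplodeTank, which hides the mesh, plays a random 2D sound and swaps in a Niagara explosion, then returns false.
; The area damage, status effects and delayed destroy logic is disconnected, so the explosion is only audiovisual and the actor remains.
; ShootObject is an empty event.
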(event `self.ShootObject`)

(event `ExplodeTank`
  (bind _particle (`self.Particle`))
  (bind _soundarray (`self.SoundArray`))
  (`SceneComponent.SetVisibility` (`self.PhysicsObject`) false false)
  (`GameplayStatics.PlaySound2D` (`|GetArrayItem` _soundarray (`KismetMathLibrary.RandomIntegerInRange` 0 (`KismetArrayLibrary.Array_Length` _soundarray))) 1.0 1.0 0.0 null null)
  (`SceneComponent.K2_SetRelativeRotation` _particle (struct :`Yaw` 3.0) false false)
  (`NiagaraComponent.SetAsset` _particle "/Game/Ultimate_VFX/PyroVFX/Niagara_FX/Explosions/NS_General_M_Ex_03.NS_General_M_Ex_03" true))

(fn `TakeDamage`
  (params (DamageInfo :type "/Game/EmPath/Structures/S_DamageInfo Structure") (`Damage Causer` :type "Actor Object Reference"))
  (returns (WasDamaged :type Boolean))
  (`self.ExplodeTank`)
  (return false))

(fn `UserConstructionScript`
  (`parent.UserConstructionScript`))