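; BP_ProceduralSpellbook is a usable spellbook object that grants the player a procedurally generated custom spell.
; On BeginPlay it draws two random DT_Spells rows and passes them to the player's CreateSpell as dominant and recessive spells, storing the result.
; Use sends that spell to the player pawn to learn and select, then destroys the book.
; The construction script gives each book a random mesh.
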(event `self.ReceiveBeginPlay`
  (bind _outrownames (`DataTableFunctionLibrary.GetDataTableRowNames` "/Game/EmPath/DataTables/DT_Spells.DT_Spells"))
  (bind _returnvalue (`|GetDataTableRow` "/Game/EmPath/DataTables/DT_Spells.DT_Spells" (`KismetArrayLibrary.Array_Random` _outrownames))
    (:`then`
      (bind _returnvalue_2 (`|GetDataTableRow` "/Game/EmPath/DataTables/DT_Spells.DT_Spells" (`KismetArrayLibrary.Array_Random` _outrownames))
        (:`then`
          (bind _asmaster (`/Game/HorrorEngine/Blueprints/Core/HorrorEngineFunctions.GetPlayer`))
          (bind _newspell (`/Game/HorrorEngine/Blueprints/HorrorEngine.CreateSpell` _asmaster (`.Name_6_7F98041B49C9308E9156C2903CAA4431` (break `/Game/EmPath/Structures/Spell/S_SpellData` (`.Data_31_F58FFE3A4CA3B15DEF86A698EF9F7A7B` (break `/Game/EmPath/Structures/Spell/S_Spell` _returnvalue_2)))) (`.Name_6_7F98041B49C9308E9156C2903CAA4431` (break `/Game/EmPath/Structures/Spell/S_SpellData` (`.Data_31_F58FFE3A4CA3B15DEF86A698EF9F7A7B` (break `/Game/EmPath/Structures/Spell/S_Spell` _returnvalue)))) (`self.Random`)))
          (set `self.New Spell` _newspell))))))

(fn `Use`
  (params (HorrorEvent :type Boolean))
  (bind _returnvalue (`GameplayStatics.GetPlayerPawn` 0))
  (bind _new_spell (`self.New Spell`))
  (message `/Game/EmPath/Interfaces/BI_GameActions.LearnSpells` _returnvalue "NewEnumerator0" _new_spell)
  (message `/Game/EmPath/Interfaces/BI_GameActions.SetSelectedSpell` _returnvalue _new_spell true false)
  (`self.K2_DestroyActor`))

(fn `UserConstructionScript`
  (`parent.UserConstructionScript`)
  (`StaticMeshComponent.SetStaticMesh` (`self.PhysicsObject`) (`KismetArrayLibrary.Array_Random` (`self.Meshes`))))