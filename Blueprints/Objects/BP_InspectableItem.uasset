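; Inspectable world item that can be bought or act as a special prop: phone, radio or world map.
; InspectionUse deducts the price from the player pawn's money and plays a cash sound when the item is buyable and affordable.
; Use switches on object type to summon the player to the camper level, cycle a radio frequency via interface, or open the menu.
; The construction script applies mesh, inspection and inventory settings.
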(event `/Game/HorrorEngine/Blueprints/Core/Use.AlternativeUse`
  (params (HorrorEvent :type Boolean))
  ;[1 1 1] Buy item
)

(event `self.InspectionUse`
  (bind _returnvalue (`GameplayStatics.GetPlayerPawn` 0))
  (bind _price (`self.Price`))
  ;[1 1 1] Buy item
  (if (`self.Buyable`)
    (bind _money (message `/Game/EmPath/Interfaces/BI_GameActions.GetMoney` _returnvalue))
    (if (>= _money _price)
      (message `/Game/EmPath/Interfaces/BI_GameActions.SetMoney` _returnvalue (- _money _price))
      (`/Game/HorrorEngine/Blueprints/Core/HorrorEngineMacros.HM_2DSound` "/Game/EmPath/Sounds/Cash.Cash" true))))

(event `/Game/HorrorEngine/Blueprints/Core/Use.Use`
  (params (HorrorEvent :type Boolean))
  (switch `/Game/EmPath/Enum/E_ObjectTypes` (`self.ObjectType`)
    (:`NewEnumerator8`
      (`/Game/HorrorEngine/Blueprints/Core/HorrorEngineFunctions.Notice` "" "Bubba" "is summoning you back to the camper")
      (bind _asmaster (`/Game/HorrorEngine/Blueprints/Core/HorrorEngineFunctions.GetPlayer`))
      (`GameplayStatics.PlaySound2D` "/Game/EmPath/Sounds/Bluezone_-_Interception_-_Radio_Transmission/Bluezone_BC0266_radio_transmission_frequency_selection_002_03.Bluezone_BC0266_radio_transmission_frequency_selection_002_03" 1.0 1.0 0.0 null null)
      (`KismetSystemLibrary.Delay` 3.0)
      (message `/Game/EmPath/Interfaces/BI_GameActions.OpenLevel` (`GameplayStatics.GetPlayerPawn` 0) (`/Game/HorrorEngine/Blueprints/HorrorEngine.CamperLevel` _asmaster) "0" true false))
    (:`NewEnumerator37`
      (bind _outactors (`GameplayStatics.GetAllActorsWithInterface` "/Game/EmPath/Interfaces/BI_Radio.BI_Radio_C"))
      (message `/Game/EmPath/Interfaces/BI_Radio.CycleFrequency` (`|GetArrayItem` _outactors)))
    (:`NewEnumerator41`
      (bind _asmaster_2 (`/Game/HorrorEngine/Blueprints/Core/HorrorEngineFunctions.GetPlayer`))
      (`/Game/HorrorEngine/Blueprints/HorrorEngine.OpenMenu` _asmaster_2))))

(event `self.InventoryUse`)

(event `self.AddToCache`)

(event `self.Retake`
  (params (InventorySave :type "/Game/HorrorEngine/Blueprints/Structures/SaveStructures/InventorySave Structure")))

(fn `UserConstructionScript`
  (`parent.UserConstructionScript`)
  (`/Game/HorrorEngine/Blueprints/Core/HorrorEngineMacros.HM_DefaultConstructions` (`self.CreateNewHorrorEvent`))
  (`/Game/HorrorEngine/Blueprints/Core/HorrorEngineFunctions.SetMesh` (`self.Actor`) (`self.MeshSettings`))
  (`self.SetInspection` (`self.InspectionSettings`))
  (`self.SetInventory` (`self.InventorySettings`))
  (if (`self.Buyable`)
    _))