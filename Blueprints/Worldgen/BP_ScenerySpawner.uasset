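; Scenery spawner for world generation that periodically drops batches of BP_RoadsideScenery actors at randomly picked spawn points.
; A looping timer, started with an immediate first batch on BeginPlay, passes each actor an Urbanization value, randomized initially and overridable through StartGeneration.
; StopGeneration sets a flag that clears the timer after the next batch, and StartGeneration resets it without restarting the timer.
; Speed and Night are stored but unused here.
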(event `self.ReceiveBeginPlay`
  (set `self.Urbanization` (`KismetMathLibrary.RandomFloatInRange` 0.0 1.0))
  (bind _returnvalue (`KismetSystemLibrary.K2_SetTimerDelegate` (delegate `SpawnRandomTerrain`) 7.0 true))
  (set `self.TimerHandle` _returnvalue)
  (`self.SpawnRandomTerrain`))

(event `SpawnRandomTerrain`
  (for _ (range 5)
    (`|SpawnActorFromClass` "/Game/EmPath/Blueprints/Worldgen/BP_RoadsideScenery.BP_RoadsideScenery_C" (select `int` (`KismetMathLibrary.RandomIntegerInRange` 0 9) :`0` (`SceneComponent.K2_GetComponentToWorld` (`self.SpawnL`)) :`1` (`SceneComponent.K2_GetComponentToWorld` (`self.SafeSpawnR`)) :`2` (`SceneComponent.K2_GetComponentToWorld` (`self.Spawn5`)) :`3` (`SceneComponent.K2_GetComponentToWorld` (`self.Spawn4`)) :`4` (`SceneComponent.K2_GetComponentToWorld` (`self.Spawn3`)) :`5` (`SceneComponent.K2_GetComponentToWorld` (`self.Spawn`)) :`6` (`SceneComponent.K2_GetComponentToWorld` (`self.Spawn1`)) :`7` (`SceneComponent.K2_GetComponentToWorld` (`self.Spawn6`)) :`8` (`SceneComponent.K2_GetComponentToWorld` (`self.Spawn8`))) "AdjustIfPossibleButAlwaysSpawn" "MultiplyWithRoot" null (`self.Urbanization`) null))
  (if (`self.StopGen`)
    (`KismetSystemLibrary.K2_ClearAndInvalidateTimerHandle` (`self.TimerHandle`))))

(event `SpawnRoad`)

(event `/Game/EmPath/Interfaces/BI_TerrainSpawner.StartGeneration`
  (params (Speed :type "Float (double-precision)") (Urbanization :type "Float (double-precision)") (Night :type Boolean))
  (set `self.Speed` Speed)
  (set `self.Urbanization` Urbanization)
  (set `self.Night` Night)
  (set `self.StopGen` false))

(event `/Game/EmPath/Interfaces/BI_TerrainSpawner.SetSpeed`
  (params (NewParam :type "Float (double-precision)"))
  (set `self.Speed` NewParam))

(event `/Game/EmPath/Interfaces/BI_TerrainSpawner.StopGeneration`
  (set `self.StopGen` true))

(fn `UserConstructionScript`)