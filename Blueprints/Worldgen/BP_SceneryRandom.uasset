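; BP_SceneryRandom is a worldgen scenery actor that randomly decides at BeginPlay whether to appear and which mesh it shows.
; A SpawnChance roll either reveals the StaticMesh or destroys the actor.
; Surviving actors pick randomly from AlternativeMeshes plus the default mesh when alternatives exist.
; StartGeneration disables collision and StopGeneration restores query-only collision, while a Debug flag makes the mesh visible during construction.
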(event `self.ReceiveBeginPlay`
  (bind _staticmesh (`self.StaticMesh`))
  (bind _alternativemeshes (`self.AlternativeMeshes`))
  (if (<= (`KismetMathLibrary.RandomFloatInRange` 0.0 1.0) (`self.SpawnChance`))
    (`SceneComponent.SetVisibility` _staticmesh true false)
    (if (> (`KismetArrayLibrary.Array_Length` _alternativemeshes) 0)
      (`KismetArrayLibrary.Array_Add` _alternativemeshes (`StaticMeshComponent.StaticMesh` _staticmesh))
      (`StaticMeshComponent.SetStaticMesh` _staticmesh (`KismetArrayLibrary.Array_Random` _alternativemeshes)))
    (else
      (`self.K2_DestroyActor`))))

(event `/Game/EmPath/Interfaces/BI_TerrainSpawner.StartGeneration`
  (params (Speed :type "Float (double-precision)") (Urbanization :type "Float (double-precision)") (Night :type Boolean))
  (`PrimitiveComponent.SetCollisionEnabled` (`self.StaticMesh`) "NoCollision"))

(event `/Game/EmPath/Interfaces/BI_TerrainSpawner.StopGeneration`
  (`PrimitiveComponent.SetCollisionEnabled` (`self.StaticMesh`) "QueryOnly"))

(fn `UserConstructionScript`
  (if (`self.Debug`)
    (`SceneComponent.SetVisibility` (`self.StaticMesh`) true false)))