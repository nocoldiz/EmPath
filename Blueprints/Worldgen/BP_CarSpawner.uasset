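; BP_CarSpawner is a worldgen actor that keeps spawning random vehicles at its Spawn transform, mostly with AutoDrive enabled.
; BeginPlay calls SpawnCar immediately and on a looping timer, and each call picks one class from a switch on a random integer.
; After each spawn, a short random delay and chance roll can re-trigger SpawnCar, producing occasional bursts of traffic.
; StartGeneration and StopGeneration are empty stubs.
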(event `self.ReceiveBeginPlay`
  (`KismetSystemLibrary.K2_SetTimerDelegate` (delegate `SpawnCar`) 30.0 true)
  (`self.SpawnCar`))

(event `SpawnCar`
  (bind _returnvalue (`SceneComponent.K2_GetComponentToWorld` (`self.Spawn`)))
  (`|ExecutionSequence`
    (:`then_0`
      (switch `int` (`KismetMathLibrary.RandomInteger` 13)
        (:`Default`
          (`|SpawnActorFromClass` "/Game/CitySampleVehicles/vehicle06_Car/BP_vehicle06_Car.BP_vehicle06_Car_C" _returnvalue "Undefined" "MultiplyWithRoot" null false null :!label _label))
        (:`2`
          (`|SpawnActorFromClass` "/Game/CitySampleVehicles/vehicle01_Van/BP_vehicle01_Van.BP_vehicle01_Van_C" _returnvalue "Undefined" "MultiplyWithRoot" null true null))
        (:`3`
          (`|SpawnActorFromClass` "/Game/CitySampleVehicles/vehicle02_Car/BP_vehicle02_Car.BP_vehicle02_Car_C" _returnvalue "Undefined" "MultiplyWithRoot" null true null))
        (:`4`
          (`|SpawnActorFromClass` "/Game/CitySampleVehicles/vehicle04_Truck/BP_vehicle04_Truck.BP_vehicle04_Truck_C" _returnvalue "Undefined" "MultiplyWithRoot" null true null))
        (:`5`
          (`|SpawnActorFromClass` "/Game/CitySampleVehicles/vehicle05_Car/BP_vehicle05_Car.BP_vehicle05_Car_C" _returnvalue "Undefined" "MultiplyWithRoot" null true null))
        (:`6`
          (goto _label))
        (:`7`
          (`|SpawnActorFromClass` "/Game/CitySampleVehicles/vehicle08_Truck/BP_vehicle08_Truck.BP_vehicle08_Truck_C" _returnvalue "Undefined" "MultiplyWithRoot" null true null :!label _label_2))
        (:`8`
          (goto _label_2))
        (:`9`
          (`|SpawnActorFromClass` "/Game/CitySampleVehicles/vehicle09_Van/BP_vehicle09_Van.BP_vehicle09_Van_C" _returnvalue "Undefined" "MultiplyWithRoot" null true null))
        (:`10`
          (`|SpawnActorFromClass` "/Game/CitySampleVehicles/vehicle10_Bus/BP_vehicle10_Bus.BP_vehicle10_Bus_C" _returnvalue "Undefined" "MultiplyWithRoot" null true null))
        (:`11`
          (`|SpawnActorFromClass` "/Game/CitySampleVehicles/vehicle11_Truck/BP_vehicle11_Truck.BP_vehicle11_Truck_C" _returnvalue "Undefined" "MultiplyWithRoot" null true null))
        (:`12`
          (`|SpawnActorFromClass` "/Game/CitySampleVehicles/vehicle12_Car/BP_vehicle12_Car.BP_vehicle12_Car_C" _returnvalue "Undefined" "MultiplyWithRoot" null true null))
        (:`13`
          (`|SpawnActorFromClass` "/Game/CitySampleVehicles/vehicle13_Car/BP_vehicle13_Car.BP_vehicle13_Car_C" _returnvalue "Undefined" "MultiplyWithRoot" null true null))))
    (:`then_1`
      (`KismetSystemLibrary.Delay` (`KismetMathLibrary.RandomFloatInRange` 1.0 3.0))
      (if (<= (`KismetMathLibrary.RandomFloatInRange` 0.0 1.0) 0.3)
        (`self.SpawnCar`)))))

(event `/Game/EmPath/Interfaces/BI_TerrainSpawner.StartGeneration`
  (params (Speed :type "Float (double-precision)") (Urbanization :type "Float (double-precision)") (Night :type Boolean)))

(event `/Game/EmPath/Interfaces/BI_TerrainSpawner.StopGeneration`)

(fn `UserConstructionScript`)