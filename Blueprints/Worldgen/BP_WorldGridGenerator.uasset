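; Streams a chunk grid along X around the player, with a road down the Y=0 row and random terrain scenery beside it.
; BeginPlay sorts DT_Chunks into scenery, road and large pools, then builds the starting area.
; A timer checks player travel, then pauses the game while destroying and loading chunks and offsets the car spawner.
; BP_Chunk actors gain random level instances or soft-class actors; large chunks reserve surrounding cells.
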(event Custom|LoadRoad
  (bind _verticalrenderdistance (Variables|Default|GetVerticalRenderDistance))
  ;[0.15 0.15 0.15 0.5] LoadRoad
  (for _index (range (- -2 _verticalrenderdistance) (+ _verticalrenderdistance 7))
    (CallFunction|LoadChunk (Math|Vector2D|MakeVector2D (Math|Conversions|ToFloat(Integer) _index) 0.0))))

(event Custom|CheckNewRoad
  (CallFunction|UpdateRoadChunks))

(event Custom|UnloadLevel
  (params (InVec :type Vector%202D%20Structure))
  (bind _returnvalue (Utilities|String|ToString(Vector2d) InVec))
  (bind _returnvalue_2 (Utilities|String|StringToName _returnvalue))
  (Game|UnloadStreamLevel(byName) _returnvalue_2 false)
  (Development|PrintString (Utilities|String|ToString(Name) _returnvalue_2) true true "(R=1.000000,G=0.195801,B=0.000000,A=1.000000)"))

(event Custom|DebugCoordinates
  (bind _playerreference (Variables|Default|GetPlayerReference))
  (Development|PrintString (Utilities|String|ToString(Vector2d) (Utilities|GetPlayerCoordinates _playerreference)) true true "(R=0.000000,G=0.660000,B=1.000000,A=1.000000)" 0.3)
  (Development|PrintString (Utilities|String|ToString(Transform) (Transformation|GetActorTransform _playerreference)) true true "(R=0.000000,G=0.660000,B=1.000000,A=1.000000)" 0.3))

(event Custom|LoadStartingArea
  (bind _horizontalrenderdistance (Variables|Default|GetHorizontalRenderDistance))
  ;[0.15 0.15 0.15 0.5] LoadStartingArea
  (CallFunction|LoadLargeChunk "(X=10.000000,Y=0.000000)")
  (for _index (range -3 9)
    (for _index_2 (range (- 0 _horizontalrenderdistance) _horizontalrenderdistance)
      (CallFunction|LoadChunk (Math|Vector2D|MakeVector2D (Math|Conversions|ToFloat(Integer) _index) (Math|Conversions|ToFloat(Integer) _index_2))))))

(event EventBeginPlay
  (Utilities|Time|SetTimerbyEvent (delegate Custom|DebugCoordinates) 0.3 true)
  (Utilities|Time|SetTimerbyEvent (delegate Custom|CheckNewRoad) 3.0 true)
  (bind _output_get (Variables|Default|SetPlayerReference (Game|Player|GetPlayerPawn 0)))
  (Variables|Default|SetLastUpdatePosition (Transformation|GetActorLocation _output_get))
  (bind _enumvalue (|ForEachE_WorldTerrainType)
    (:LoopBody
      (Utilities|Array|Add (Variables|Default|GetTerrains) _enumvalue))
    (:then
      (Variables|Default|SetSelectedTerrain "NewEnumerator1")
      (bind _outactors (Actor|GetAllActorsOfClass "/Game/EmPath/Blueprints/Worldgen/BP_CarSpawner.BP_CarSpawner_C"))
      (Variables|Default|SetCarSpawnerReference (Utilities|Array|Get(acopy) _outactors))
      (bind _outrownames (DataTable|GetDataTableRowNames "/Game/EmPath/DataTables/DT_Chunks.DT_Chunks"))
      (for _array_element _outrownames
        (bind _returnvalue (Utilities|GetDataTableRow "/Game/EmPath/DataTables/DT_Chunks.DT_Chunks" _array_element)
          (:then
            (if (Utilities|Enum|Equal(Enum) (.Roadtype (Utilities|Struct|BreakS_Chunk _returnvalue)) "NewEnumerator0") ; Check if is a terrain
              (Utilities|Array|Add (Variables|Default|GetSceneryChunksTable) _returnvalue)
              (elif (.LargeChunk (Utilities|Struct|BreakS_Chunk _returnvalue))
                (Utilities|Array|Add (Variables|Default|GetLargeChunksTable) _returnvalue)
                (else
                  (Utilities|Array|Add (Variables|Default|GetRoadChunksTable) _returnvalue)))))))
      (Class|LevelStreamingDynamic|LoadLevelInstance "ck_base" "0, 0, 0" "0, 0, 0" "" 0 false)
      (CallFunction|LoadStartingArea))))

(event Collision|EventActorBeginOverlap
  (params (OtherActor :type Actor%20Object%20Reference)))

(event EventTick
  (params (DeltaSeconds :type Float%20%28single-precision%29)))

(fn ConstructionScript)

(fn LoadChunk
  (params (Coordinates :type Vector%202D%20Structure))
  (bind _y (Math|Vector2D|BreakVector2D Coordinates))
  (bind _returnvalue (Utilities|CalculateChunkSize Coordinates))
  (bind _scenerychunkstable (Variables|Default|GetSceneryChunksTable))
  (bind _outitem (Utilities|Array|Random _scenerychunkstable))
  (bind _returnvalue_2 (Math|Conversions|ToTransform(Vector) _returnvalue))
  (bind _returnvalue_3 (== _y 0.0))
  (bind (_name _levelactor) (Utilities|Struct|BreakS_Chunk _outitem))
  (if (not (.Value (Utilities|Map|Find (Variables|Default|GetChunkMap) Coordinates)))
    (if _returnvalue_3
      (bind _returnvalue_4 (Game|SpawnActorfromClass "/Game/EmPath/Blueprints/Worldgen/BP_Chunk.BP_Chunk_C" (Math|Conversions|ToTransform(Vector) _returnvalue) "Undefined" "MultiplyWithRoot" 0 true false (Variables|Default|GetSelectedTerrain) 0))
      (Utilities|Map|Add (Variables|Default|GetSpawnedChunks) Coordinates _returnvalue_4)
      (Utilities|Map|Add (Variables|Default|GetChunkMap) Coordinates true)
      (elif (< (Math|Random|RandomFloatinRange 0.0 1.0) (Variables|Default|GetSpawnSpecialChunkChance))
        (bind _returnvalue_5 (Game|SpawnActorfromClass "/Game/EmPath/Blueprints/Worldgen/BP_Chunk.BP_Chunk_C" _returnvalue_2 "Undefined" "MultiplyWithRoot" 0 false false (Variables|Default|GetSelectedTerrain) 0))
        (Utilities|Map|Add (Variables|Default|GetSpawnedChunks) Coordinates _returnvalue_5)
        (Utilities|Map|Add (Variables|Default|GetChunkMap) Coordinates true)
        (LocalVariables|SetLevelName _name)
        (CallFunction|LoadLevel Coordinates (select (or false _returnvalue_3) "0, 0, 0" (Math|Rotator|MakeRotator 0.0 0.0 (Utilities|Select :Index (Math|Random|RandomIntegerinRange 0 6) :Option%200 0.0 :Option%201 9e+01 :Option%202 -9e+01 :Option%203 1.8e+02 :Option%204 -1.8e+02))) _returnvalue (LocalVariables|GetLevelName) _levelactor)
        (else
          (bind _returnvalue_6 (Game|SpawnActorfromClass "/Game/EmPath/Blueprints/Worldgen/BP_Chunk.BP_Chunk_C" _returnvalue_2 "Undefined" "MultiplyWithRoot" 0 false false (Variables|Default|GetSelectedTerrain) 0))
          (Utilities|Map|Add (Variables|Default|GetSpawnedChunks) Coordinates _returnvalue_6)
          (Utilities|Map|Add (Variables|Default|GetChunkMap) Coordinates true))))))

(fn DestroyChunk
  (params (Key :type Vector%202D%20Structure%20%28by%20ref%29))
  (bind _spawnedchunks (Variables|Default|GetSpawnedChunks))
  (bind _debugthisblueprint (Variables|Default|GetDebugThisBlueprint))
  (bind _chunkmap (Variables|Default|GetChunkMap))
  (bind (_value _returnvalue) (Utilities|Map|Find _spawnedchunks Key))
  (if (.ReturnValue (Utilities|Map|Find (Variables|Default|GetChunkMap) Key))
    (Utilities|Map|Remove _chunkmap Key))
  (if _returnvalue
    (Actor|DestroyActor _value))
  (if (.ReturnValue (Utilities|Map|Find _chunkmap Key))
    (Development|PrintString (Utilities|String|Append "Unload " (Utilities|String|ToString(Vector2d) Key)) _debugthisblueprint true "(R=0.348958,G=0.015275,B=0.000000,A=1.000000)")
    (Utilities|Map|Remove (Variables|Default|GetChunkMap) Key)
    (CallFunction|UnloadLevel Key)
    (else
      (Development|PrintString "NotLoad" _debugthisblueprint))))

(fn UnloadFarChunks
  (bind _verticalrenderdistance (Variables|Default|GetVerticalRenderDistance))
  (bind _horizontalrenderdistance (Variables|Default|GetHorizontalRenderDistance))
  (for _index (range (+ (Math|Float|Truncate (.X (Math|Vector2D|BreakVector2D (Variables|Default|GetPlayerCoordinates)))) _verticalrenderdistance) (+ 10 _verticalrenderdistance))
    (for _index_2 (range (- 0 _horizontalrenderdistance) _horizontalrenderdistance)
      (CallFunction|DestroyChunk (Math|Vector2D|MakeVector2D (Math|Conversions|ToFloat(Integer) (- 0 _index)) (Math|Conversions|ToFloat(Integer) _index_2))))))

(fn LoadLargeChunk
  (params (Coordinates :type Vector%202D%20Structure))
  (bind _returnvalue (Utilities|CalculateLargeChunkSize Coordinates))
  (bind _largechunkstable (Variables|Default|GetLargeChunksTable))
  (bind _outitem (Utilities|Array|Random _largechunkstable))
  (bind (_name _levelactor _chunktype _roadtype _largechunk _fixedrotation) (Utilities|Struct|BreakS_Chunk _outitem))
  (Development|PrintString (Utilities|String|Append "Spawn At" (Utilities|String|ToString(Vector) _returnvalue) (Utilities|String|ToString(Vector2d) Coordinates)) true true "(R=1.000000,G=0.000000,B=0.181645,A=1.000000)" 1e+01)
  (CallFunction|LoadLevel Coordinates (Math|Rotator|SelectRotator "0, 0, 0" (Math|Rotator|SelectRotator "0, 0, 0" "0.000000,-180.000000,0.000000" (Math|Random|RandomBool)) _fixedrotation) _returnvalue _name)
  (CallFunction|ReserveChunkAroundCoordinate Coordinates)
  (Utilities|Map|Add (Variables|Default|GetChunkMap) Coordinates true)
  (Development|PrintString (Utilities|String|Append "Spawned large chunk at " (Utilities|String|ToString(Vector2d) Coordinates))))

(fn UpdateRoadChunks
  (bind _playerreference (Variables|Default|GetPlayerReference))
  (bind _returnvalue (Transformation|GetActorLocation _playerreference))
  ;[0.15 0.15 0.15 0.5] IF flying load chunk faster
  (if (> (Math|Float|Absolute(Float) (/ (.X (Math|Vector|BreakVector (- _returnvalue (Variables|Default|GetLastUpdatePosition)))) (Variables|Default|GetChunkSize))) (/ (Variables|Default|GetVerticalRenderDistance) 2))
    (Game|SetGamePaused true)
    (bind _output_get (Variables|Default|SetLastUpdatePosition _returnvalue))
    (if (Utilities|Operators|NotEqual(!=) (Math|Vector2D|MakeVector2D (Math|Conversions|ToFloat(Integer) (Math|Float|Floor (.X (Math|Vector|BreakVector (/ _output_get (Variables|Default|GetChunkSize)))))) (Math|Conversions|ToFloat(Integer) (Math|Float|Floor (.Y (Math|Vector|BreakVector (/ _output_get (Variables|Default|GetChunkSize))))))) (Variables|Default|GetPlayerCoordinates) 0.6)
      (bind _output_get_2 (Variables|Default|SetPlayerCoordinates (Math|Vector2D|MakeVector2D (Math|Conversions|ToFloat(Integer) (Math|Float|Floor (.X (Math|Vector|BreakVector (/ _output_get (Variables|Default|GetChunkSize)))))) (Math|Conversions|ToFloat(Integer) (Math|Float|Floor (.Y (Math|Vector|BreakVector (/ _output_get (Variables|Default|GetChunkSize)))))))))
      (CallFunction|UnloadFarChunks)
      (if (< (Math|Random|RandomFloatinRange 0.0 1.0) (Variables|Default|GetLargeChunkSpanceChance))
        (Variables|Default|SetShouldSpawnLargeChunk true)
        (else
          (Variables|Default|SetShouldSpawnLargeChunk false)))
      (Utilities|FlowControl|Sequence
        (:then_0
          (for _index (range (Math|Float|Truncate (.X (Math|Vector2D|BreakVector2D _output_get_2))) (+ (Math|Float|Truncate (.X (Math|Vector2D|BreakVector2D _output_get_2))) (Variables|Default|GetVerticalRenderDistance)))
            (for _index_2 (range (- 0 (Variables|Default|GetHorizontalRenderDistance)) (Variables|Default|GetHorizontalRenderDistance))
              (if (Math|Boolean|ANDBoolean (== _index_2 0) (== (Math|Integer|%(Integer) _index (Variables|Default|GetSpecialChunksInterval)) 0) (!= _index 0))
                (if (Variables|Default|GetShouldSpawnLargeChunk)
                  (CallFunction|LoadLargeChunk (Math|Vector2D|MakeVector2D (Math|Conversions|ToFloat(Integer) _index) (Math|Conversions|ToFloat(Integer) _index_2)))
                  (else
                    (CallFunction|LoadChunk (Math|Vector2D|MakeVector2D (Math|Conversions|ToFloat(Integer) _index) (Math|Conversions|ToFloat(Integer) _index_2)) :!label _label)))
                (else
                  (goto _label)))))
          (Game|SetGamePaused false))
        (:then_1
          (Transformation|AddActorWorldOffset (Variables|Default|GetCarSpawnerReference) (Math|Vector|MakeVector (+ (.X (Math|Vector|BreakVector (Variables|Default|GetLastUpdatePosition))) 3e+03) 0.0 0.0)))))))

(fn ReserveChunkAroundCoordinate
  (params (InVec :type Vector%202D%20Structure))
  (bind (_x _y) (Math|Vector2D|BreakVector2D InVec))
  (for _index (range (Math|Float|Truncate (- _x 2.0)) (Math|Float|Truncate (+ _x 2.0)))
    (for _index_2 (range (Math|Float|Truncate (- _y 2.0)) (Math|Float|Truncate (+ _y 2.0)))
      (if (not (.ReturnValue (Utilities|Map|Find (Variables|Default|GetChunkMap) (Math|Vector2D|MakeVector2D (Math|Conversions|ToFloat(Integer) _index) (Math|Conversions|ToFloat(Integer) _index_2)))))
        (Utilities|Map|Add (Variables|Default|GetSpawnedChunks) (Math|Vector2D|MakeVector2D (Math|Conversions|ToFloat(Integer) _index) (Math|Conversions|ToFloat(Integer) _index_2)) (stale _returnvalue))
        (Utilities|Map|Add (Variables|Default|GetChunkMap) (Math|Vector2D|MakeVector2D (Math|Conversions|ToFloat(Integer) _index) (Math|Conversions|ToFloat(Integer) _index_2)) true)))))

(fn LoadLevel
  (params (Key :type Vector%202D%20Structure%20%28by%20ref%29) (Rotation :type Rotator) (Location :type Vector) (LevelName :type String) (LevelActor :type Packed%20Level%20Actor%20Soft%20Class%20Reference))
  (if (Utilities|IsValidSoftClassReference LevelActor)
    (Utilities|LoadClassAssetBlocking LevelActor)
    (bind _returnvalue (Game|SpawnActorfromClass (Utilities|ResolveSoftReference LevelActor) (Math|Transform|MakeTransform (.Location (Math|Transform|BreakTransform (Math|Conversions|ToTransform(Vector) Location))) (Math|Rotator|MakeRotator 0.0 0.0 (Math|Random|RandomFloatinRange 0.0 0.0))) "Undefined" "MultiplyWithRoot" 0 0))
    (Utilities|Map|Add (Variables|Default|GetSpawnedChunks) Key _returnvalue)
    (else
      (bind _boutsuccess (Class|LevelStreamingDynamic|LoadLevelInstance LevelName Location Rotation (Utilities|String|ToString(Vector2d) Key) 0 false))
      (if _boutsuccess
        (Utilities|Map|Add (Variables|Default|GetChunkMap) Key true)))))

(fn LoadTerrainChunk
  (params (A :type Float%20%28double-precision%29) (A2 :type Float%20%28double-precision%29))
  (bind _returnvalue (Math|Float|Floor A))
  (bind _verticalrenderdistance (Variables|Default|GetVerticalRenderDistance))
  (for _index (range (- _returnvalue _verticalrenderdistance) (+ _returnvalue _verticalrenderdistance))
    (for _index_2 (range (- 0 (Variables|Default|GetHorizontalRenderDistance)) (Variables|Default|GetHorizontalRenderDistance))
      (CallFunction|LoadChunk (Math|Vector2D|MakeVector2D (Math|Conversions|ToFloat(Integer) _index) (Math|Conversions|ToFloat(Integer) _index_2))))))