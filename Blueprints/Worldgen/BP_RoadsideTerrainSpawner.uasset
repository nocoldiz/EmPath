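; Roadside terrain piece that leapfrogs forward along world X to keep scenery ahead of the player.
; On BeginPlay, if alternative meshes exist, it picks randomly among them and its original, then applies a fixed footprint with random height scale.
; When the player pawn enters its Box, it offsets itself, its Companion and any valid BasePlane by one fixed distance.
; StartGeneration disables mesh collision; StopGeneration restores it as query-only.
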(event `self.ReceiveBeginPlay`
  (bind _staticmesh (`self.StaticMesh`))
  (bind _alternativemeshes (`self.AlternativeMeshes`))
  (`SceneComponent.SetVisibility` _staticmesh true false)
  (if (> (`KismetArrayLibrary.Array_Length` _alternativemeshes) 0)
    (`KismetArrayLibrary.Array_Add` _alternativemeshes (`StaticMeshComponent.StaticMesh` _staticmesh))
    (`StaticMeshComponent.SetStaticMesh` _staticmesh (`KismetArrayLibrary.Array_Random` _alternativemeshes))
    (`SceneComponent.SetWorldScale3D` (`self.StaticMesh`) (`KismetMathLibrary.MakeVector` 6.0 6.0 (`KismetMathLibrary.RandomFloatInRange` 6.0 12.0)))))

(event `self.StartGeneration`
  (params (Speed :type "Float (double-precision)") (Urbanization :type "Float (double-precision)") (Night :type Boolean))
  (`PrimitiveComponent.SetCollisionEnabled` (`self.StaticMesh`) "NoCollision"))

(event `self.StopGeneration`
  (`PrimitiveComponent.SetCollisionEnabled` (`self.StaticMesh`) "QueryOnly"))

(event `self.Box.OnComponentBeginOverlap`
  (params (OverlappedComponent :type "PrimitiveComponent Object Reference") (OtherActor :type "Actor Object Reference") (OtherComp :type "PrimitiveComponent Object Reference") (OtherBodyIndex :type Integer) (bFromSweep :type Boolean) (SweepResult :type "HitResult Structure (by ref)"))
  (bind _baseplane (`self.BasePlane`))
  (if (== OtherActor (`GameplayStatics.GetPlayerPawn` 0))
    (`self.K2_AddActorWorldOffset` (`self.Companion`) (113500.0 0.0 0.0) false false)
    (`self.K2_AddActorWorldOffset` self (113500.0 0.0 0.0) false false)
    (`/Engine/EditorBlueprintResources/StandardMacros.IsValid` _baseplane
      (:`Is Valid`
        (`self.K2_AddActorWorldOffset` _baseplane (113500.0 0.0 0.0) false false)))))

(fn `UserConstructionScript`
  (`SceneComponent.SetVisibility` (`self.StaticMesh`) true false))