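; BP_RoadsideScenery is a moving roadside prop for worldgen that shows a random City or Wilderness mesh, weighted by Urbanization.
; After a short spawn delay it picks the mesh, or clears it in Debug mode.
; Tick offsets it along X by Speed per frame, and outside Debug a repeating 60-second check destroys it once Speed is non-zero.
; StartGeneration and StopGeneration switch mesh collision between none and query-only.
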(event `self.ReceiveBeginPlay`
  (bind _staticmesh (`self.StaticMesh`))
  (`KismetSystemLibrary.Delay` 0.6)
  (if (`self.Debug`)
    (`StaticMeshComponent.SetStaticMesh` _staticmesh null)
    (else
      (`StaticMeshComponent.SetStaticMesh` _staticmesh (select `bool` (<= (`KismetMathLibrary.RandomFloatInRange` 0.0 1.0) (`self.Urbanization`)) :`false` (`KismetArrayLibrary.Array_Random` (`self.Wilderness`)) :`true` (`KismetArrayLibrary.Array_Random` (`self.City`))))
      (`KismetSystemLibrary.Delay` 60.0 :!label _label)
      (if (!= (`self.Speed`) 0.0)
        (`self.K2_DestroyActor`)
        (else
          (`self.WaitForDelete`))))))

(event `WaitForDelete`
  (goto _label))

(event `self.ReceiveTick`
  (params (DeltaSeconds :type "Float (single-precision)"))
  (`self.K2_AddActorWorldOffset` (`KismetMathLibrary.MakeVector` (`self.Speed`))))

(event `/Game/EmPath/Interfaces/BI_TerrainSpawner.SetSpeed`
  (params (NewParam :type "Float (double-precision)"))
  (set `self.Speed` NewParam))

(event `/Game/EmPath/Interfaces/BI_TerrainSpawner.StartGeneration`
  (params (Speed :type "Float (double-precision)") (Urbanization :type "Float (double-precision)") (Night :type Boolean))
  (`PrimitiveComponent.SetCollisionEnabled` (`self.StaticMesh`) "NoCollision"))

(event `/Game/EmPath/Interfaces/BI_TerrainSpawner.StopGeneration`
  (`PrimitiveComponent.SetCollisionEnabled` (`self.StaticMesh`) "QueryOnly"))

(fn `UserConstructionScript`)