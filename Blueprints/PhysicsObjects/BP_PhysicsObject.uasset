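; BP_PhysicsObject is a physics prop with a configurable mesh and optional gravity, labeled as grabbable and able to take damage.
; Unless indestructible, hits play particle, Niagara and sound effects and reduce health; below zero it destroys itself, or only swaps its hit sound if living.
; A Clone status spawns a copy in place.
; Destruction effects and most combat, team and activity functions are stubs returning defaults.
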(event `self.ReceiveBeginPlay`
  (set `self.Health` (`self.MaxHealth`))
  (if (`self.DisableGravity`)
    (`PrimitiveComponent.SetEnableGravity` (`self.StaticMesh`) false)))

(event `/Game/EmPath/Interfaces/BPI_Damagable.ApplyStatus`
  (params (Status :type "/Game/EmPath/Enum/E_SpellEffect Enum" :default "NewEnumerator12") (Duration :type "Float (double-precision)") (Magnitude :type "Float (double-precision)") (Enable :type Boolean) (SuccessRate :type "Float (double-precision)") (HitBoneName :type Name))
  (switch `/Game/EmPath/Enum/E_SpellEffect` Status
    (:`NewEnumerator39`
      (`|SpawnActorFromClass` (`GameplayStatics.GetObjectClass` self) (`self.GetTransform`) "AdjustIfPossibleButAlwaysSpawn" "MultiplyWithRoot" null (`self.Mesh`) null))))

(event `/Game/EmPath/Interfaces/BPI_Damagable.ClearStatus`
  (params (SpellEffect :type "/Game/EmPath/Enum/E_SpellEffect Enum" :default "NewEnumerator12") (ClearAll :type Boolean)))

(fn `ActivityTimeUpdate`
  (params (Time :type Integer))
  (returns (Activity :type "/Game/EmPath/Enum/E_NPCActivities Enum"))
  (return "NewEnumerator0"))

(fn `GetCurrentHealth`
  (returns (Health :type "Float (double-precision)"))
  (return (`self.Health`)))

(fn `GetID`
  (returns (ID :type String))
  (return ""))

(fn `GetLauncherActor`
  (returns (LauncherActor :type "Actor Object Reference"))
  (return null))

(fn `GetMaxHealth`
  (returns (MaxHealth :type "Float (double-precision)"))
  (return (`self.MaxHealth`)))

(fn `GetNextActivity`
  (returns (Activity :type "/Game/EmPath/Enum/E_NPCActivities Enum") (Time :type Integer))
  (return "NewEnumerator0" 0))

(fn `GetObjectName`
  (returns (NameOut :type String))
  (return (`KismetStringLibrary.Concat_StrStr` (`KismetStringLibrary.Concat_StrStr` " [ E ] Grab " (`self.Name`)) " \n" (`self.Class`))))

(fn `GetTeamNumber`
  (returns (TeamNumber :type Integer))
  (return 0))

(fn `Heal`
  (params (Amount :type "Float (double-precision)"))
  (returns (NewHealth :type "Float (double-precision)"))
  (return 0.0))

(fn `IsAttacking`
  (returns (Attacking :type Boolean))
  (return false))

(fn `IsDead`
  (returns (Dead :type Boolean))
  (return false))

(fn `IsProjectile`
  (returns (Result :type Boolean))
  (return false))

(fn `PlayDamageFx`
  (bind _returnvalue (`self.K2_GetActorLocation`))
  (bind _hitsystem_template (`self.HitSystem Template`))
  (bind _hitemittertemplate (`self.HitEmitterTemplate`))
  (`|ExecutionSequence`
    (:`then_0`
      (`/Engine/EditorBlueprintResources/StandardMacros.IsValid` _hitemittertemplate
        (:`Is Valid`
          (`GameplayStatics.SpawnEmitterAtLocation` _hitemittertemplate _returnvalue))))
    (:`then_1`
      (`/Engine/EditorBlueprintResources/StandardMacros.IsValid` _hitsystem_template
        (:`Is Valid`
          (`NiagaraFunctionLibrary.SpawnSystemAtLocation` _hitsystem_template _returnvalue))))
    (:`then_2`
      (`GameplayStatics.PlaySoundAtLocation` (`self.HitSound`) _returnvalue (struct) 1.0 1.0 0.0 "/Game/HorrorEngine/Audio/_ATT_Profiles/ATT_General.ATT_General" null null null))))

(fn `PlayDestructionFx`)

(fn `ReserveAttackToken`
  (params (Amount :type Integer))
  (returns (Success :type Boolean))
  (return false))

(fn `TakeDamage`
  (params (DamageInfo :type "/Game/EmPath/Structures/S_DamageInfo Structure") (`Damage Causer` :type "Actor Object Reference") (HitLocation :type "Vector Structure"))
  (returns (WasDamaged :type Boolean))
  (if (`self.Indestructible`)
    (return false)
    (else
      (`self.PlayDamageFx`)
      (bind _output_get (set `self.Health` (- (`self.Health`) (`.Amount_2_64864A0D4320D27C3EA14D8019B5EC9D` (break `/Game/EmPath/Structures/S_DamageInfo` DamageInfo)))))
      (if (< _output_get 0.0)
        (`self.PlayDestructionFx`)
        (if (`self.IsLiving`)
          (set `self.HitSound` "/Game/EmPath/Cues/SC_PlayerDamage.SC_PlayerDamage")
          (else
            (`self.K2_DestroyActor`)))
        (else
          (return true))))))

(fn `UserConstructionScript`
  (`StaticMeshComponent.SetStaticMesh` (`self.StaticMesh`) (`self.Mesh`)))