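; Time manager actor that runs the day/night cycle from the time and day stored in BP_EmPathGameInstance.
; Advance steps the clock ten minutes, rolls over days at midnight, saves back to the GameInstance, then refreshes the world.
; The refresh rotates the first DirectionalLight, lerps temperature and switches BI_Light actors between day and night.
; RealTimeMode starts a looping timer, and debug variables can offset the start time or skip lighting.
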(event `Advance`
  (`KismetSystemLibrary.PrintString` "Passed")
  (bind (_time _day) (`/Game/MRPGT/Blueprints/GameInstance/BP_EmPathGameInstance.GetTimeDay` (`self.GameInstance`)))
  (set `self.DaysPassed` _day)
  (set `self.TimePassed` (`KismetMathLibrary.Conv_IntToDouble` _time))
  (`self.UpdateClock`)
  (`self.AdvanceTime`))

(event `self.ReceiveBeginPlay`
  (bind _debugtime (`self.DebugTime`))
  (bind _asbp_em_path_game_instance (cast `/Game/MRPGT/Blueprints/GameInstance/BP_EmPathGameInstance` (`GameplayStatics.GetGameInstance`)))
  (set `self.GameInstance` _asbp_em_path_game_instance)
  (bind (_time _day) (`/Game/MRPGT/Blueprints/GameInstance/BP_EmPathGameInstance.GetTimeDay` (`self.GameInstance`) :!label _label))
  (set `self.TimePassed` (`KismetMathLibrary.Conv_IntToDouble` _time))
  (set `self.DaysPassed` _day)
  (`|ExecutionSequence`
    (:`then_0`
      (`/Engine/EditorBlueprintResources/StandardMacros.DoOnce` false
        (:`Completed`
          ;[1 1 1] Debug Light
          (if (> _debugtime 0)
            (set `self.TimePassed` _debugtime)
            (`self.UpdateClock`)))))
    (:`then_1`
      (if (not (`self.DebugLight`))
        (bind _outactors (`GameplayStatics.GetAllActorsOfClass` "/Script/Engine.DirectionalLight"))
        (set `self.DirectionalLight` (`|GetArrayItem` _outactors))
        (`self.UpdateLightBasedONTime`)
        (if (or (<= _time 360) (> _time 1080))
          (`self.UpdateLevelLights` true)
          (else
            (`self.UpdateLevelLights` false)))
        (if (`self.RealTimeMode`)
          (`KismetSystemLibrary.K2_SetTimerDelegate` (`|CreateDelegate` :!event `Advance`) (`self.RealTimeTick`) true))))))

(event `AdvanceTime`
  (goto _label))

(event `UpdateLightBasedONTime`
  (bind _timepassed (`self.TimePassed`))
  (bind _returnvalue (/ _timepassed 1440.0))
  (bind _returnvalue_2 (- (mod (* _returnvalue 360.0) 360.0) -90.0))
  (`KismetSystemLibrary.PrintString` (`KismetStringLibrary.Conv_DoubleToString` _timepassed) true true (struct :`G` 0.66 :`B` 1.0 :`A` 1.0) 6.0)
  (`KismetSystemLibrary.PrintString` (`KismetStringLibrary.Conv_DoubleToString` _returnvalue_2) true true (struct :`G` 0.66 :`B` 1.0 :`A` 1.0) 6.0)
  (`self.K2_SetActorRotation` (`self.DirectionalLight`) (`KismetMathLibrary.MakeRotator` 0.0 _returnvalue_2) false)
  (`/Game/MRPGT/Blueprints/GameInstance/BP_EmPathGameInstance.SetTemperature` (`self.GameInstance`) (`KismetMathLibrary.Lerp` (`KismetMathLibrary.Conv_IntToDouble` (`self.NightTemperature`)) (`KismetMathLibrary.Conv_IntToDouble` (`self.DayTemperature`)) _returnvalue)))

(event `UpdateLevelLights`
  (params (SetNight :type Boolean))
  (bind _outactors (`GameplayStatics.GetAllActorsWithInterface` "/Game/EmPath/Interfaces/BI_Light.BI_Light_C"))
  (for _array_element _outactors
    (if SetNight
      (message `/Game/EmPath/Interfaces/BI_Light.SetNight` _array_element)
      (else
        (message `/Game/EmPath/Interfaces/BI_Light.SetDay` _array_element)))))

(fn `UpdateClock`
  ;[1 1 1] Pass 15 minutes in normal speed
  (set `self.TimePassed` (+ (`self.TimePassed`) 10.0))
  (if (>= (`self.TimePassed`) 1440.0)
    ;[1 1 1] Reset clock and advance 1 day
    (set `self.TimePassed` 0.0)
    (`/Engine/EditorBlueprintResources/StandardMacros.IncrementInt` (`self.DaysPassed`)
      (:`  `
        _)))
  (`/Game/MRPGT/Blueprints/GameInstance/BP_EmPathGameInstance.SetTimeDay` (`self.GameInstance`) (`KismetMathLibrary.FTrunc` (`self.TimePassed`)) (`self.DaysPassed`)))

(fn `UserConstructionScript`)