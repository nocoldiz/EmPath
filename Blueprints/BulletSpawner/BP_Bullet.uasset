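; BP_Bullet is a projectile that damages and force-mutilates any BPI_Damagable actor it overlaps, fading its travel sound on impact.
; Construction copies speed and gravity variables into ProjectileMovement; BeginPlay aligns ImpactRadius to the camera and makes enemy-cast bullets home on the player.
; SetHomingProjectile can also target the player's last living enemy, though only the player branch is called here.
; Spell-collision, reaction and destroy logic is disconnected, and the Play*Sequence functions are empty.
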(event `self.ReceiveBeginPlay`
  ;[1 1 1 1 28] Begin Play
  ;[0 1 0.3242] Spell Flowchart
  (`SceneComponent.K2_SetRelativeRotation` (`self.ImpactRadius`) (`KismetMathLibrary.Conv_VectorToRotator` (`self.GetActorForwardVector` (`GameplayStatics.GetPlayerCameraManager` 0))) false false)
  (if (`self.IsCastedByEnemy`)
    (`self.Set Homing Projectile` false))
  (set `self.BounceTimes` 0)
  ;;[1 1 1] Projectile travel
  (`/Engine/EditorBlueprintResources/StandardMacros.IsValid` null))

(event `self.ImpactRadius.OnComponentBeginOverlap`
  (params (OverlappedComponent :type "PrimitiveComponent Object Reference") (OtherActor :type "Actor Object Reference") (OtherComp :type "PrimitiveComponent Object Reference") (OtherBodyIndex :type Integer) (bFromSweep :type Boolean) (SweepResult :type "HitResult Structure (by ref)"))
  (bind _travelsound (`self.TravelSound`))
  ;[1 0.5177 0.03873 1 24] Spell impact
  (`/Engine/EditorBlueprintResources/StandardMacros.IsValid` _travelsound
    (:`Is Valid`
      (`AudioComponent.FadeOut` _travelsound 0.6 0.0 "Linear"))
    (:`Is Not Valid`
      _))
  (if (`KismetSystemLibrary.DoesImplementInterface` OtherActor "/Game/EmPath/Interfaces/BPI_Damagable.BPI_Damagable_C")
    (message `/Game/EmPath/Interfaces/BPI_Damagable.TakeDamage` OtherActor (make `/Game/EmPath/Structures/S_DamageInfo` 1.0 "NewEnumerator1") null)
    (message `/Game/EmPath/Interfaces/BPI_Damagable.Mutilate` OtherActor "None" true)))

(event `self.ImpactRadius.OnComponentHit`
  (params (HitComponent :type "PrimitiveComponent Object Reference") (OtherActor :type "Actor Object Reference") (OtherComp :type "PrimitiveComponent Object Reference") (NormalImpulse :type "Vector Structure") (Hit :type "HitResult Structure (by ref)"))
  (bind _travelsound (`self.TravelSound`))
  ;[1 0.5177 0.03873 1 24] Spell impact
  (`/Engine/EditorBlueprintResources/StandardMacros.IsValid` _travelsound
    (:`Is Valid`
      (`AudioComponent.FadeOut` _travelsound 1.0 0.0 "Linear"))))

(event `self.ProjectileMovement.OnProjectileBounce`
  (params (ImpactResult :type "HitResult Structure (by ref)") (ImpactVelocity :type "Vector Structure (by ref)"))
  ;[1 0.5177 0.03873 1 24] Spell impact
)

(event `Trigger`
  ;[1 0.5177 0.03873 1 24] Spell impact
)

(fn `PlayCastSequence`)

(fn `PlayDestroySequence`)

(fn `PlayHitSequence`)

(fn `PlaySpawnSequence`)

(fn `PlayTravelSequence`)

(fn `Set Homing Projectile`
  (params (TargetEnemy :type Boolean))
  (bind _projectilemovement (`self.ProjectileMovement`))
  ;[1 1 1] SetHomingProjectile
  (if TargetEnemy
    (bind _asmaster (`/Game/HorrorEngine/Blueprints/Core/HorrorEngineFunctions.GetPlayer`))
    (bind _lasttarget (`/Game/HorrorEngine/Blueprints/HorrorEngine.LastTarget` _asmaster))
    (bind _returnvalue (`KismetSystemLibrary.LoadAsset_Blocking` _lasttarget))
    (`/Engine/EditorBlueprintResources/StandardMacros.IsValid` (`|ConvertAsset` _lasttarget)
      (:`Is Valid`
        (bind _asbp_enemy_base (cast `/Game/EmPath/Enemies/BP_EnemyBase` _returnvalue))
        (bind _health (`/Game/EmPath/Enemies/BP_EnemyBase.GetCurrentHealth` _asbp_enemy_base))
        (if (> _health 0.0)
          (bind _returnvalue_2 (`AddComponent|NODE_AddSceneComponent-3` :`self` _asbp_enemy_base))
          (set `self.Homing Target Component` _returnvalue_2)
          (set `ProjectileMovementComponent.HomingTargetComponent` (`self.Homing Target Component`) _projectilemovement :!label _label)
          (set `ProjectileMovementComponent.bIsHomingProjectile` true _projectilemovement)
          (set `ProjectileMovementComponent.HomingAccelerationMagnitude` 15000.0 _projectilemovement))))
    (else
      (bind _asem_path_player (cast `/Game/EmPath/Blueprints/EmPathPlayer` (`GameplayStatics.GetPlayerCharacter` 0)))
      (bind _returnvalue_3 (`AddComponent|NODE_AddSceneComponent-1` :`self` _asem_path_player))
      (set `self.Homing Target Component` _returnvalue_3)
      (goto _label))))

(fn `SpawnEffect`
  (params (SchoolB :type "/Game/EmPath/Enum/E_MagicSchools Enum" :default "NewEnumerator0"))
  (bind _spawned (message `/Game/EmPath/Interfaces/BI_GameActions.GetSpawnReaction` (`GameplayStatics.GetPlayerPawn` 0)))
  (if (not _spawned)
    (`|SpawnActorFromClass` "/Game/EmPath/Blueprints/Spells/BP_ElementalReaction.BP_ElementalReaction_C" (`KismetMathLibrary.Conv_VectorToTransform` (`self.K2_GetActorLocation` self)) "Undefined" "MultiplyWithRoot" null "NewEnumerator0" "NewEnumerator0" SchoolB null)
    (message `/Game/EmPath/Interfaces/BI_GameActions.SetSpawnReaction` (`GameplayStatics.GetPlayerPawn` 0) true)))

(fn `UserConstructionScript`
  (bind _projectilemovement (`self.ProjectileMovement`))
  ;[1 1 1] Set projectile movement
  (set `ProjectileMovementComponent.InitialSpeed` (`self.Initial Speed`) _projectilemovement)
  (set `ProjectileMovementComponent.MaxSpeed` (`self.Max Speed`) _projectilemovement)
  (set `ProjectileMovementComponent.ProjectileGravityScale` (`self.Projectile Gravity Scale`) _projectilemovement))