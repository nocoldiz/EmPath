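; Level bounds trigger that sends the player to another level when they enter its box.
; An overlapping player pawn gets a random level from Destinations, the BP_CamperSmall gets TheRoad, and any other actor is destroyed.
; For a transfer it shows a loading widget, then after a short delay the game instance saves the level, transform and coordinates and auto-loads that save at the Entrance.
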(event `self.ReceiveBeginPlay`
  (bind _asbp_em_path_game_instance (cast `/Game/MRPGT/Blueprints/GameInstance/BP_EmPathGameInstance` (`GameplayStatics.GetGameInstance`)))
  (set `self.GameInstance` _asbp_em_path_game_instance))

(event `self.Box.OnComponentBeginOverlap`
  (params (OverlappedComponent :type "PrimitiveComponent Object Reference") (OtherActor :type "Actor Object Reference") (OtherComp :type "PrimitiveComponent Object Reference") (OtherBodyIndex :type Integer) (bFromSweep :type Boolean) (SweepResult :type "HitResult Structure (by ref)"))
  (bind _gameinstance (`self.GameInstance`))
  (bind _levelname (`self.LevelName`))
  (if (== OtherActor (`GameplayStatics.GetPlayerPawn` 0))
    (bind _drivingmode (message `/Game/EmPath/Interfaces/BI_GameActions.GetDrivingMode` (`GameplayStatics.GetPlayerPawn` 0)))
    (if (or (`|EnumEquality` _drivingmode "NewEnumerator6") (`|EnumEquality` _drivingmode "NewEnumerator2"))
      _
      (else
        _))
    (set `self.LevelName` (`KismetArrayLibrary.Array_Random` (`self.Destinations`)))
    (bind _mapcoordinates (`/Game/MRPGT/Blueprints/GameInstance/BP_EmPathGameInstance.Get Coordinates` (`self.GameInstance`) :!label _label))
    (bind _returnvalue (`|CreateWidget` "/Game/EmPath/UI/W_Loading.W_Loading_C"))
    (`UserWidget.AddToViewport` _returnvalue 0)
    (`KismetSystemLibrary.Delay` 0.4)
    (`/Game/MRPGT/Blueprints/GameInstance/BP_EmPathGameInstance.SaveNewGame` _gameinstance "NewEnumerator0" _levelname "None" (`self.Transform`) _mapcoordinates)
    (`/Game/MRPGT/Blueprints/GameInstance/BP_EmPathGameInstance.LoadSavedGame` _gameinstance "0" true (`self.Entrance`) (`KismetStringLibrary.Conv_NameToString` _levelname))
    (elif (== OtherActor "/Game/EmPath/Blueprints/Camper/BP_CamperSmall.BP_CamperSmall")
      (set `self.LevelName` "TheRoad")
      (goto _label)
      (else
        (`self.K2_DestroyActor` OtherActor)))))

(fn `UserConstructionScript`)