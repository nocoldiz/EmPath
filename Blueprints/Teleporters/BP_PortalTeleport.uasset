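; BP_PortalTeleport is a portal that teleports the player when they enter its sphere trigger.
; The overlap event responds only to the pawn of player 0, plays a 2D teleport sound, then moves that pawn to the Arrow component's world location and rotation.
; It also sets the player controller's control rotation to the Arrow's, so the view faces the exit direction.
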(event `self.Sphere.OnComponentBeginOverlap`
  (params (OverlappedComponent :type "PrimitiveComponent Object Reference") (OtherActor :type "Actor Object Reference") (OtherComp :type "PrimitiveComponent Object Reference") (OtherBodyIndex :type Integer) (bFromSweep :type Boolean) (SweepResult :type "HitResult Structure (by ref)"))
  (bind _arrow (`self.Arrow`))
  (bind _returnvalue (`SceneComponent.K2_GetComponentRotation` _arrow))
  (if (== OtherActor (`GameplayStatics.GetPlayerPawn` 0))
    (`GameplayStatics.PlaySound2D` (`self.TeleportSound`) 1.0 1.0 0.0 null null)
    (`self.K2_TeleportTo` (`GameplayStatics.GetPlayerPawn` 0) (`SceneComponent.K2_GetComponentLocation` _arrow) _returnvalue)
    (`Controller.SetControlRotation` (`GameplayStatics.GetPlayerController` 0) _returnvalue)))

(fn `UserConstructionScript`)